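; Two-panel sliding door that parts vertically when something overlaps its Intersect component and CanOpen is true, and closes when the overlap ends.
; Begin overlap passes CanOpen through a client-named event to OpenDoor; timelines lerp Top and Bottom in opposite directions, with a sound at each move.
; Short Delay loops poll Top's position so opening waits until fully closed, and closing waits until fully open plus a pause.
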(event `self.ReceiveBeginPlay`
  (set `self.Start_T` (`SceneComponent.K2_GetComponentLocation` (`self.Top`)))
  (set `self.Start_B` (`SceneComponent.K2_GetComponentLocation` (`self.Bottom`))))

(event `Client_SetCanOpen`
  (params (`CanOpen?` :type Boolean))
  ;[0.3 0.3 0.3] Set Condition to Open Door
  (bind _output_get (set `self.CanOpen?` `CanOpen?`))
  (if _output_get
    (`self.OpenDoor`)))

(event `OpenDoor`
  (bind _start_t (`self.Start_T`))
  (bind _start_b (`self.Start_B`))
  (bind _start_t_2 (`self.Start_T`))
  (bind _returnvalue (- _start_b (0.0 0.0 150.0)))
  (bind _returnvalue_2 (+ _start_t (0.0 0.0 150.0)))
  ;[0.3 0.3 0.3] Open Door
  (`KismetSystemLibrary.Delay` 0.1 :!label _label)
  (if (`KismetMathLibrary.EqualExactly_VectorVector` _start_t_2 (`SceneComponent.K2_GetComponentLocation` (`self.Top`)))
    (`GameplayStatics.PlaySoundAtLocation` null _start_t_2 (struct) 4.0 1.0 0.0 null null null)
    (bind (_direction _opendoor) (`Timeline|Open` :!via `PlayFromStart`)
      (:`Update`
        (`SceneComponent.K2_SetWorldLocation` (`self.Top`) (`KismetMathLibrary.VLerp` _start_t _returnvalue_2 _opendoor) false false)
        (set `self.End_T` _returnvalue_2)
        (`SceneComponent.K2_SetWorldLocation` (`self.Bottom`) (`KismetMathLibrary.VLerp` _start_b _returnvalue _opendoor) false false)
        (set `self.End_B` _returnvalue)))
    (else
      (goto _label))))

(event `self.Intersect.OnComponentBeginOverlap`
  (params (OverlappedComponent :type "PrimitiveComponent Object Reference") (OtherActor :type "Actor Object Reference") (OtherComp :type "PrimitiveComponent Object Reference") (OtherBodyIndex :type Integer) (bFromSweep :type Boolean) (SweepResult :type "HitResult Structure (by ref)"))
  (`self.Client_SetCanOpen` (`self.CanOpen?`)))

(event `self.Intersect.OnComponentEndOverlap`
  (params (OverlappedComponent :type "PrimitiveComponent Object Reference") (OtherActor :type "Actor Object Reference") (OtherComp :type "PrimitiveComponent Object Reference") (OtherBodyIndex :type Integer))
  (bind _top (`self.Top`))
  (bind _end_t (`self.End_T`))
  (bind _end_b (`self.End_B`))
  (bind _end_t_2 (`self.End_T`))
  (bind _returnvalue (- _end_t (0.0 0.0 150.0)))
  ;[0.3 0.3 0.3] Close Door
  (`KismetSystemLibrary.Delay` 0.1 :!label _label_2)
  (if (`KismetMathLibrary.EqualExactly_VectorVector` (`SceneComponent.K2_GetComponentLocation` (`self.Top`)) _end_t_2)
    (`KismetSystemLibrary.Delay` 1.0)
    (`GameplayStatics.PlaySoundAtLocation` null _end_t_2 (struct) 4.0 1.0 0.0 null null null)
    (set `self.End_T` (`SceneComponent.K2_GetComponentLocation` _top))
    (bind (_direction _closedoor) (`Timeline|Close` :!via `PlayFromStart`)
      (:`Update`
        (`SceneComponent.K2_SetWorldLocation` _top (`KismetMathLibrary.VLerp` _end_t _returnvalue _closedoor) false false)
        (set `self.Start_T` _returnvalue)
        (bind _returnvalue_2 (`KismetMathLibrary.VLerp` _end_b (+ _end_b (0.0 0.0 150.0)) _closedoor))
        (`SceneComponent.K2_SetWorldLocation` (`self.Bottom`) _returnvalue_2 false false)
        (set `self.Start_B` _returnvalue_2)))
    (else
      (goto _label_2))))

(fn `UserConstructionScript`)