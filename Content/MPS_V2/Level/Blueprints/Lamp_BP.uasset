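; Lamp_BP is a damageable, cable-hung lamp that breaks and goes dark when its health runs out.
; Any damage is passed to a server health event and briefly enables physics on the lamp through a multicast, using a retriggerable delay.
; On death, with a DoOnce gate for one weapon slot, a multicast breaks the constraint and cables, spawns sparks, removes the lights and later destroys the actor.
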(event `MC_Physics`
  ;[0.3 0.3 0.3] Simulate Physics
  (`PrimitiveComponent.SetSimulatePhysics` (`self.Lamp`) true)
  (`KismetSystemLibrary.RetriggerableDelay` 8.0)
  (`PrimitiveComponent.SetSimulatePhysics` (`self.Lamp`) false))

(event `self.ReceiveAnyDamage`
  (params (Damage :type "Float (single-precision)") (DamageType :type "DamageType Object Reference") (InstigatedBy :type "Controller Object Reference") (DamageCauser :type "Actor Object Reference"))
  (`self.Svr_Damaging` Damage InstigatedBy DamageCauser)
  (`self.MC_Physics`))

(event `Svr_Damaging`
  (params (Damage :type "Float (double-precision)") (Instigator :type "Controller Object Reference") (Causer :type "Object Object Reference"))
  ;[0.3 0.3 0.3] Server Handles Damage
  (bind _output_get (set `self.Health` (- (`self.Health`) Damage)))
  (if (<= _output_get 0.0)
    (if (`self.IsActive`)
      (bind _asmps_master_bp (cast `/Game/MPS_V2/Game/Blueprints/MPS_MasterBP` (`Controller.K2_GetPawn` Instigator)))
      (if (== Causer (`|GetArrayItem` (`/Game/MPS_V2/Game/Blueprints/MPS_MasterBP.Weapons` _asmps_master_bp) 3))
        (`|ExecutionSequence`
          (:`then_0`
            (`/Engine/EditorBlueprintResources/StandardMacros.DoOnce` false :!label _label
              (:`Completed`
                _)))
          (:`then_1`
            (`KismetSystemLibrary.Delay` 0.6)
            (goto _label :!via `Reset`))))
      (set `self.IsActive` false)
      (`/Engine/EditorBlueprintResources/ActorMacros.Switch Has Authority`
        (:`Authority`
          (`self.MC_Destroyed`))))))

(event `MC_Destroyed`
  (bind _cable1 (`self.Cable1`))
  (bind _cable (`self.Cable`))
  ;[0.3 0.3 0.3] Replicated Destruction of Target
  (`/Engine/EditorBlueprintResources/StandardMacros.IsValid` self
    (:`Is Valid`
      (`PhysicsConstraintComponent.BreakConstraint` (`self.PhysicsConstraint`))
      (set `CableComponent.bAttachEnd` false _cable)
      (set `CableComponent.CableLength` 100.0 _cable)
      (set `CableComponent.bAttachEnd` false _cable1)
      (set `CableComponent.CableLength` 100.0 _cable1)
      (bind _returnvalue (`GameplayStatics.SpawnEmitterAtLocation` "/Game/MPS_V2/Game/Commons/Particles/P_Sparks.P_Sparks" (`SceneComponent.K2_GetComponentLocation` (`self.SpotLight`))))
      (`PrimitiveComponent.SetMaterial` (`self.Lamp`) 1 "/Game/MPS_V2/Level/Materials/ShootingRange/MI_NoGlow.MI_NoGlow")
      (`|ExecutionSequence`
        (:`then_0`
          (`ActorComponent.K2_DestroyComponent` (`self.SpotLight`))
          (`ActorComponent.K2_DestroyComponent` (`self.Beam`))
          (`ActorComponent.K2_DestroyComponent` (`self.PointLight`))
          (`KismetSystemLibrary.Delay` 20.0)
          (`self.K2_DestroyActor`))
        (:`then_1`
          (`KismetSystemLibrary.Delay` 0.3)
          (`ActorComponent.K2_DestroyComponent` _returnvalue))))))

(fn `UserConstructionScript`
  (`parent.UserConstructionScript`))