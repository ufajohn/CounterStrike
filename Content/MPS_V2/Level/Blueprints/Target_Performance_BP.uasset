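; Shootable performance target that takes damage on the server, credits hits to the shooter, and opens a door when destroyed.
; Hits from the shooter's fourth weapon slot are throttled by a resetting DoOnce, while other weapons always register.
; At zero health it calls the game controller's door event, deactivates, then multicasts destruction: ropes break, the target falls with sparks, and parts are removed.
; A multicast plays a random-pitch hit sound, and the construction script toggles the optional frame.
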(event `self.ReceiveAnyDamage`
  (params (Damage :type "Float (single-precision)") (DamageType :type "DamageType Object Reference") (InstigatedBy :type "Controller Object Reference") (DamageCauser :type "Actor Object Reference"))
  (`self.Svr_Damaging` Damage InstigatedBy DamageCauser)
  (`self.MC_Sound`))

(event `Svr_Damaging`
  (params (Damage :type "Float (double-precision)") (Instigator :type "Controller Object Reference") (Causer :type "Object Object Reference"))
  ;[0.3 0.3 0.3] Server Handles Damage
  (if (`self.IsActive`)
    (bind _asmps_master_bp (cast `/Game/MPS_V2/Game/Blueprints/MPS_MasterBP` (`Controller.K2_GetPawn` Instigator)))
    (if (== Causer (`|GetArrayItem` (`/Game/MPS_V2/Game/Blueprints/MPS_MasterBP.Weapons` _asmps_master_bp) 3))
      (`|ExecutionSequence`
        (:`then_0`
          (`/Engine/EditorBlueprintResources/StandardMacros.DoOnce` false :!label _label
            (:`Completed`
              _)))
        (:`then_1`
          (`KismetSystemLibrary.Delay` 0.6)
          (goto _label :!via `Reset`))))
    (`/Game/MPS_V2/Game/Blueprints/MPS_MasterBP.HitCounter` _asmps_master_bp 1)
    (bind _output_get (set `self.Health` (- (`self.Health`) Damage)))
    (if (<= _output_get 0.0)
      (bind _asgame_controller_bp (castclass `/Game/MPS_V2/Game/Blueprints/Data/GameController_BP` "/Game/MPS_V2/Game/Blueprints/Data/GameController_BP.GameController_BP_C"))
      (bind _outactors (`GameplayStatics.GetAllActorsOfClass` _asgame_controller_bp))
      (`/Engine/EditorBlueprintResources/StandardMacros.IsValid` (`|GetArrayItem` _outactors)
        (:`Is Valid`
          (`/Game/MPS_V2/Game/Blueprints/Data/GameController_BP.Svr_OpenDoor` _outactors)
          (set `self.IsActive` false)
          (`/Engine/EditorBlueprintResources/ActorMacros.Switch Has Authority`
            (:`Authority`
              (`self.MC_Destroyed`))))))))

(event `MC_Destroyed`
  ;[0.3 0.3 0.3] Replicated Destruction of Target
  (`/Engine/EditorBlueprintResources/StandardMacros.IsValid` self
    (:`Is Valid`
      (`ActorComponent.K2_DestroyComponent` (`self.Rope2`))
      (`ActorComponent.K2_DestroyComponent` (`self.Rope1`))
      (`PrimitiveComponent.SetSimulatePhysics` (`self.Target`) true)
      (bind _returnvalue (`GameplayStatics.SpawnEmitterAtLocation` "/Game/MPS_V2/Game/Commons/Particles/P_Sparks.P_Sparks" (`SceneComponent.K2_GetComponentLocation` (`self.SpotLight`))))
      (`|ExecutionSequence`
        (:`then_0`
          (`ActorComponent.K2_DestroyComponent` (`self.SpotLight`))
          (`ActorComponent.K2_DestroyComponent` (`self.Beam`))
          (`KismetSystemLibrary.Delay` 20.0)
          (`ActorComponent.K2_DestroyComponent` (`self.Frame`)))
        (:`then_1`
          (`KismetSystemLibrary.Delay` 0.3)
          (`ActorComponent.K2_DestroyComponent` _returnvalue))))))

(event `MC_Sound`
  ;[0.3 0.3 0.3] Sound
  (`GameplayStatics.PlaySoundAtLocation` "/Game/MPS_V2/Game/Sounds/Cue/TargetHit_Cue.TargetHit_Cue" (`self.K2_GetActorLocation`) (struct) 0.5 (`KismetMathLibrary.RandomFloatInRange` 1.0 1.5) 0.0 null null null))

(fn `UserConstructionScript`
  (`parent.UserConstructionScript`)
  (`SceneComponent.SetVisibility` (`self.Frame`) (`self.HasFrame`) true))