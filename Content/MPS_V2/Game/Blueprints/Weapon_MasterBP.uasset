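; Base weapon Blueprint for MPS_V2 that configures itself from the Weapons_DT row matching its name and runs the player's shooting.
; StartShooting branches by type and firemode (semi, auto, burst, melee, explosive), gated by dry-fire checks and delays, triggering effects, controller-spawned projectiles and random recoil.
; Attachments snap to mesh sockets, with per-weapon loadouts persisted through SaveGame slots.
; It also handles dropping, magazine refills and customization preview movement.
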(event `self.ReceiveBeginPlay`
  ;[0.3 0.3 0.3] Event Begin Play
  (`parent.ReceiveBeginPlay`)
  (set `self.SaveName` (`KismetStringLibrary.Conv_NameToString` (`self.Name`)))
  (`self.Load`)
  (bind _asmps_master_bp (cast `/Game/MPS_V2/Game/Blueprints/MPS_MasterBP` (`GameplayStatics.GetPlayerCharacter` 0)))
  (set `self.MPS` _asmps_master_bp))

(event `StartShooting`
  (bind _returnvalue (select `/Game/MPS_V2/Game/Blueprints/Data/WeaponType_Enum` (`self.DT_Type`) :`NewEnumerator3` 1 :`NewEnumerator4` 2 :`NewEnumerator5` 3 :`NewEnumerator6` 4 :`NewEnumerator7` 5 :`NewEnumerator8` 6))
  ;[0.3 0.3 0.3] Logic
  (`self.DryCheck`
    (:`OutputPin`
      (if (`self.FireDelayComplete`)
        (`|ExecutionSequence`
          (:`then_0`
            (goto _label :!via `Reset`))
          (:`then_1`
            _)))
      (`/Engine/EditorBlueprintResources/StandardMacros.DoOnce` false :!label _label
        (:`Completed`
          (set `self.IsShooting?` true)
          (if (!= _returnvalue 6)
            (if (> _returnvalue 0)
              (switch `/Game/MPS_V2/Game/Blueprints/Data/Firemode_Enum` (`self.DT_Firemode`)
                (:`NewEnumerator0`
                  (set `self.DT_AmmoMag` (- (`self.DT_AmmoMag`) 1))
                  (`self.Anims&Effects`)
                  (`self.SpawnProjectile`)
                  (`self.Recoil`)
                  (`self.DryCheck`
                    (:`OutputPin`
                      (if (`self.DT_Rechamber?`)
                        (`self.RechamberDelay`)
                        (else
                          (`self.ShootingDelay`))))))
                (:`NewEnumerator3`
                  (if (`self.IsShooting?`) :!label _label_2
                    (`self.Anims&Effects`)
                    (`self.SpawnProjectile`)
                    (`self.Recoil`)
                    (set `self.DT_AmmoMag` (- (`self.DT_AmmoMag`) 1))
                    (`self.DryCheck`
                      (:`OutputPin`
                        (`self.ShootingDelay`)
                        (goto _label_2)))))
                (:`NewEnumerator4`
                  (if (`self.BurstComplete`)
                    (bind _counter (`/Engine/EditorBlueprintResources/StandardMacros.Do N` (+ (`self.DT_Bullet_Count`) 1) :!label _label_3)
                      (:`Exit`
                        (`KismetSystemLibrary.Delay` (/ (`self.DT_ShootingDelay`) 4.0))
                        (if (!= _counter (+ (`self.DT_Bullet_Count`) 1))
                          (set `self.DT_AmmoMag` (- (`self.DT_AmmoMag`) 1))
                          (`|ExecutionSequence`
                            (:`then_0`
                              (`self.Anims&Effects`)
                              (`self.SpawnProjectile`)
                              (`self.Recoil`)
                              (`self.DryCheck`
                                (:`OutputPin`
                                  (`self.ShootingDelay`)
                                  (goto _label_3))))
                            (:`then_1`
                              (`self.BurstDelay`)))
                          (else
                            (`KismetSystemLibrary.Delay` (`self.DT_BurstDelay`))
                            (goto _label_3 :!via `Reset`))))))))
              (else
                (`self.Anims&Effects`)
                (set `self.FireDelayComplete` false :!label _label_4)
                (`KismetSystemLibrary.Delay` 0.21)
                (bind _counter_2 (`/Engine/EditorBlueprintResources/StandardMacros.Do N` 10 :!label _label_5)
                  (:`Exit`
                    (if (!= _counter_2 10)
                      (`KismetSystemLibrary.Delay` 0.01)
                      (`/Game/MPS_V2/Game/Blueprints/MPS_MasterBP.Client_MeleeDamage` (`self.MPS`))
                      (goto _label_5)
                      (else
                        (`KismetSystemLibrary.Delay` (`self.DT_ShootingDelay`))
                        (set `self.FireDelayComplete` true)
                        (goto _label_5 :!via `Reset`)))))))
            (else
              (`/Game/MPS_V2/Game/Blueprints/MPS_MasterBP.ExplosiveAnims` (`self.MPS`))
              (`self.ShootingDelay`))))))))

(event `StopShooting`
  ;[0.3 0.3 0.3] Logic
  (set `self.IsShooting?` false)
  (if (`/Game/MPS_V2/Game/Blueprints/MPS_MasterBP.ToggleRecoilRecovery` (`self.MPS`))
    (bind (_direction _recoilrecovery) (`Timeline|RecoilRecovery` :!via `PlayFromStart`)
      (:`Update`
        (`Pawn.AddControllerPitchInput` (`GameplayStatics.GetPlayerCharacter` 0) (* _recoilrecovery (/ (`KismetMathLibrary.Abs` (`self.StorePitch`)) 100.0) (`self.Number`))))
      (:`Finished`
        (set `self.Number` 1.0 :!label _label_6)))
    (else
      (goto _label_6))))

(event `SwitchFiremode`
  ;[0.3 0.3 0.3] Logic
  (switch `/Game/MPS_V2/Game/Blueprints/Data/Firemode_Enum` (`self.DT_Firemode`)
    (:`NewEnumerator0`
      (set `self.DT_Firemode` "NewEnumerator4"))
    (:`NewEnumerator3`
      (set `self.DT_Firemode` "NewEnumerator0"))
    (:`NewEnumerator4`
      (set `self.DT_Firemode` "NewEnumerator3"))))

(event `QuickMelee`
  ;[0.3 0.3 0.3] Logic
  (goto _label_4))

(event `Save`
  (params (Material :type "MaterialInstance Object Reference") (Optics :type "StaticMesh Object Reference") (Siderail :type "StaticMesh Object Reference") (Underbarrel :type "StaticMesh Object Reference") (Barrel :type "StaticMesh Object Reference") (OpticsOffset :type "Float (double-precision)") (HasSilencer :type Boolean))
  ;[0.3 0.3 0.3] Customization
  (`self.SaveLoadout` Material Optics Siderail Underbarrel Barrel OpticsOffset HasSilencer))

(event `Load`
  ;[0.3 0.3 0.3] Customization
  (bind (_material _optics _siderail _underbarrel _barrel _opticsoffset _hassilencer_) (`self.LoadLoadout`))
  (`PrimitiveComponent.SetMaterial` (`self.Item`) 0 _material)
  (`StaticMeshComponent.SetStaticMesh` (`self.Optics_Mesh`) _optics)
  (bind _returnvalue (`StaticMeshComponent.SetStaticMesh` (`self.Siderail_Mesh`) _siderail))
  (set `self.HasLaser?` _returnvalue)
  (bind _returnvalue_2 (`StaticMeshComponent.SetStaticMesh` (`self.Underbarrel_Mesh`) _underbarrel))
  (set `self.MoveLeftHand?` _returnvalue_2)
  (`StaticMeshComponent.SetStaticMesh` (`self.Barrel_Mesh`) _barrel)
  (set `self.Optics_Offset` _opticsoffset)
  (bind _output_get (set `self.HasSilencer?` _hassilencer_))
  (if _output_get
    (set `self.IsSilenced?` (`self.HasSilencer?`))
    (set `self.MuzzleOffset` (20.0 0.0 0.0))
    (else
      (set `self.IsSilenced?` false)
      (set `self.MuzzleOffset` (0.0 0.0 0.0)))))

(event `MoveOutView`
  ;[0.3 0.3 0.3] Customization
  (bind (_direction _moveout) (`Timeline|MoveOut` :!via `PlayFromStart`)
    (:`Update`
      (`self.K2_SetActorLocation` (`KismetMathLibrary.VLerp` (175.0 90.0 105.0) (200.0 200.0 85.0) _moveout)))))

(event `MoveInView`
  (params (A :type "Vector Structure") (B :type "Vector Structure"))
  ;[0.3 0.3 0.3] Customization
  (bind (_direction _movein) (`Timeline|MoveIn` :!via `PlayFromStart`)
    (:`Update`
      (`self.K2_SetActorLocation` (`KismetMathLibrary.VLerp` A B _movein)))))

(event `Client_DroppedFromPlayer`
  (params (MagDropped :type Integer) (AddCarriedAmmo :type Integer))
  ;[0.3 0.3 0.3] Event Dropped
  (`self.MC_DroppedFromPlayer` (== MagDropped 0))
  (set `self.MagSize` (`self.DT_AmmoMag`))
  (set `self.DT_AmmoMag` MagDropped)
  (set `self.DT_Ammo_Bag` AddCarriedAmmo))

(event `MC_DroppedFromPlayer`
  (params (NoMag :type Boolean))
  ;[0.3 0.3 0.3] Event Dropped
  (`PrimitiveComponent.SetSimulatePhysics` (`self.Item`) true)
  (`self.RemoveMag` NoMag)
  (`KismetSystemLibrary.Delay` 5.0)
  (`PrimitiveComponent.SetSimulatePhysics` (`self.Item`) false))

(fn `Ammunition`
  (params (Condition :type Boolean))
  (bind _difference (`self.Difference`))
  ;[0.3 0.3 0.3] Clip Filled?
  (if Condition
    (set `self.Difference` (- (`self.MagSize`) (- (`self.DT_AmmoMag`) 1)))
    (if (>= (`self.DT_Ammo_Bag`) (`self.Difference`))
      ;[0.3 0.3 0.3] Fill up Mag Completly
      (set `self.DT_AmmoMag` (+ (`self.DT_AmmoMag`) _difference) :!label _label)
      (set `self.DT_Ammo_Bag` (- (`self.DT_Ammo_Bag`) _difference))
      (else
        ;[0.3 0.3 0.3] Fill up Mag with what's left in Bag
        (set `self.DT_AmmoMag` (+ (`self.DT_AmmoMag`) (`self.DT_Ammo_Bag`)) :!label _label_2)
        (set `self.DT_Ammo_Bag` 0)))
    (else
      (set `self.Difference` (- (`self.MagSize`) (`self.DT_AmmoMag`)))
      (if (>= (`self.DT_Ammo_Bag`) (`self.Difference`))
        (goto _label)
        (else
          (goto _label_2))))))

(fn `Anims&Effects`
  (bind _mps (`self.MPS`))
  (`/Game/MPS_V2/Game/Blueprints/MPS_MasterBP.MPS_ShootingAnims` _mps)
  (`/Game/MPS_V2/Game/Blueprints/MPS_MasterBP.Muzzle` _mps))

(fn `DataTable`
  (bind _item (`self.Item`))
  (bind _returnvalue (`|GetDataTableRow` "/Game/MPS_V2/Game/Weapons/Weapons_DT.Weapons_DT" (`self.Name`))
    (:`then`
      (bind (_parameters _features _attachments _animations) (break `/Game/MPS_V2/Game/Blueprints/Data/Weapons_Struct` _returnvalue))
      (set `self.DT_HolsterName` (`KismetStringLibrary.Conv_StringToName` (`|GetEnumeratorNameAsString` (break `/Game/MPS_V2/Game/Blueprints/Data/WeaponParameters_Struct` _parameters))))
      (set `self.DT_Slot` (`KismetMathLibrary.Conv_ByteToInt` (`.Slot_59_D63B79844837C996A69958A48BFD5C24` (break `/Game/MPS_V2/Game/Blueprints/Data/WeaponParameters_Struct` _parameters))))
      (set `self.DT_Type` (`.Type_60_123272EA4DA642ADB23E598C62325188` (break `/Game/MPS_V2/Game/Blueprints/Data/WeaponParameters_Struct` _parameters)))
      (set `self.DT_Firemode` (`.Firemode_61_97B0630D4472B7660FF9559DE70A8D08` (break `/Game/MPS_V2/Game/Blueprints/Data/WeaponParameters_Struct` _parameters)))
      (set `self.DT_Firemodes?` (`.Firemodes_19_62B754AA488C19DEC0D095812838B1B4` (break `/Game/MPS_V2/Game/Blueprints/Data/WeaponParameters_Struct` _parameters)))
      (set `self.DT_Rechamber?` (`.Rechamber_18_10DC87EB43896797D0BFD89BA433FA88` (break `/Game/MPS_V2/Game/Blueprints/Data/WeaponParameters_Struct` _parameters)))
      (set `self.DT_AmmoMag` (`.AmmoMag_22_2FDF3348431CCB5B8813F79FB2C0C971` (break `/Game/MPS_V2/Game/Blueprints/Data/WeaponParameters_Struct` _parameters)))
      (set `self.DT_Ammo_Bag` (`.AmmoBag_24_AAE6D1FA4337D0C7BF841FA12727109D` (break `/Game/MPS_V2/Game/Blueprints/Data/WeaponParameters_Struct` _parameters)))
      (set `self.DT_Bullet_Count` (`.BulletCount_26_711C6EF244F834F3D72CE2BB335BCDDC` (break `/Game/MPS_V2/Game/Blueprints/Data/WeaponParameters_Struct` _parameters)))
      (set `self.DT_ShootingDelay` (`.ShootingDelay_29_D583DA1641A50C2817211B80C3800265` (break `/Game/MPS_V2/Game/Blueprints/Data/WeaponParameters_Struct` _parameters)))
      (set `self.DT_BurstDelay` (`.BurstDelay_32_4B75D0B643DCFA4DA191E499D7F7CDD2` (break `/Game/MPS_V2/Game/Blueprints/Data/WeaponParameters_Struct` _parameters)))
      (set `self.DT_RechamberTime` (`.RechamberDelay_33_B1FFF610430F04B5ECBE57A66BDBEFD5` (break `/Game/MPS_V2/Game/Blueprints/Data/WeaponParameters_Struct` _parameters)))
      (set `self.DT_CameraShakeIntensity` (`.CameraShakeIntensity_35_A61C4A62402B59E378EFFD948C7E558D` (break `/Game/MPS_V2/Game/Blueprints/Data/WeaponParameters_Struct` _parameters)))
      (set `self.DT_Velocity` (`.Velocity_37_FC1B0AEE42CB0812702BD69A1FEFC845` (break `/Game/MPS_V2/Game/Blueprints/Data/WeaponParameters_Struct` _parameters)))
      (set `self.DT_Spread_Up` (`.Spread_Up_46_0BF490824722A4BAEDC4E4972BD4A93A` (break `/Game/MPS_V2/Game/Blueprints/Data/WeaponParameters_Struct` _parameters)))
      (set `self.DT_Spread_Right` (`.Spread_Right_44_86D61823425DF5595CCA6AA6FB026DB9` (break `/Game/MPS_V2/Game/Blueprints/Data/WeaponParameters_Struct` _parameters)))
      (set `self.DT_MaxDamage` (`.MaxDamage_47_B3EE07E74444115278E4B399E0D19323` (break `/Game/MPS_V2/Game/Blueprints/Data/WeaponParameters_Struct` _parameters)))
      (set `self.DT_MinDamage` (`.MinDamage_48_4F1168104AFC4A186CBAE09B28089F21` (break `/Game/MPS_V2/Game/Blueprints/Data/WeaponParameters_Struct` _parameters)))
      (set `self.DT_MaxRange` (`.MaxRange_49_E5AF2E514E9ED39BDEDBDE8E146298F4` (break `/Game/MPS_V2/Game/Blueprints/Data/WeaponParameters_Struct` _parameters)))
      (set `self.DT_MinRange` (`.MinRange_51_5AB4A60144C5288F3D4480B98573C30D` (break `/Game/MPS_V2/Game/Blueprints/Data/WeaponParameters_Struct` _parameters)))
      (set `self.DT_AnimBP` (break `/Game/MPS_V2/Game/Blueprints/Data/Features_Struct` _features))
      (set `self.DT_WeaponMesh` (`.WeaponMesh_5_C1A5A51A49231FE32BECD9AC41966301` (break `/Game/MPS_V2/Game/Blueprints/Data/Features_Struct` _features)))
      (set `self.DT_Material` (`.Material_42_EA2A67C14B8661D6550817A136295AB5` (break `/Game/MPS_V2/Game/Blueprints/Data/Features_Struct` _features)))
      (set `self.DT_Weapon_TF` (`.Weapon_TF_15_8FA2D4DF4F2A00C397F9F59DCF44C3D8` (break `/Game/MPS_V2/Game/Blueprints/Data/Features_Struct` _features)))
      (set `self.DT_RightHand_TF` (`.RightHand_TF_44_8B70452B4C7C016D24F0C8AEF6290FE3` (break `/Game/MPS_V2/Game/Blueprints/Data/Features_Struct` _features)))
      (set `self.DT_LeftHand_TF` (`.LeftHand_TF_13_6EB5E72D407B90799F0058963319F05E` (break `/Game/MPS_V2/Game/Blueprints/Data/Features_Struct` _features)))
      (set `self.DT_ShootSound` (`.Shoot_Sound_18_75EB1ABF44FD8A062A846D992792CD88` (break `/Game/MPS_V2/Game/Blueprints/Data/Features_Struct` _features)))
      (set `self.DT_SilencedSound` (`.Silenced_Sound_20_BBC1E81449ED8575044048885D9003B5` (break `/Game/MPS_V2/Game/Blueprints/Data/Features_Struct` _features)))
      (set `self.DT_EmptySound` (`.Empty_Sound_27_C835544744E9D3D78122F495CE372348` (break `/Game/MPS_V2/Game/Blueprints/Data/Features_Struct` _features)))
      (set `self.DT_ShellSound` (`.Shells_Sound_28_9CF8EED74AC52F1F80BD68B31F9FDFC9` (break `/Game/MPS_V2/Game/Blueprints/Data/Features_Struct` _features)))
      (set `self.DT_Shells` (`.Shells_30_F355ADAC401CDF3D9F31B9A21E15DACE` (break `/Game/MPS_V2/Game/Blueprints/Data/Features_Struct` _features)))
      (set `self.DT_Muzzle` (`.Muzzle_32_3904752645C7EF22E83BFD84B1519388` (break `/Game/MPS_V2/Game/Blueprints/Data/Features_Struct` _features)))
      (set `self.DT_ShellDelay` (`.ShellDelay_47_8CC6C86E4622774E4073F1B988947750` (break `/Game/MPS_V2/Game/Blueprints/Data/Features_Struct` _features)))
      (set `self.DT_Customize` (`.CanCustomize_35_44E56D3347F4EEE616E764BF24DACF56` (break `/Game/MPS_V2/Game/Blueprints/Data/Features_Struct` _features)))
      (set `self.DT_CustomMaterials` (`.CanCustomizeMaterials_41_A873DFDF40F818F5FC6300B0DE0B0390` (break `/Game/MPS_V2/Game/Blueprints/Data/Features_Struct` _features)))
      (set `self.DT_Optics` (break `/Game/MPS_V2/Game/Blueprints/Data/Attachment_Struct` _attachments))
      (set `self.DT_Siderail` (`.SideRail_5_CC1173574644F176B94762976B643331` (break `/Game/MPS_V2/Game/Blueprints/Data/Attachment_Struct` _attachments)))
      (set `self.DT_Underbarrel` (`.Underbarrel_20_939C6D31414576AF6FDEF99F237CE4B3` (break `/Game/MPS_V2/Game/Blueprints/Data/Attachment_Struct` _attachments)))
      (set `self.DT_Barrel` (`.Barrel_7_B30DE97B714131EE2E1B1095333DD0B1` (break `/Game/MPS_V2/Game/Blueprints/Data/Attachment_Struct` _attachments)))
      (set `self.DT_OpticsOffset` (`.OpticsOffset_23_502BBF1CB04D88AF81F72488DCC37847` (break `/Game/MPS_V2/Game/Blueprints/Data/Attachment_Struct` _attachments)))
      (set `self.DT_FirstDraw` (break `/Game/MPS_V2/Game/Blueprints/Data/Weapon_Anims_Struct` _animations))
      (set `self.DT_Draw` (`.DT_Draw_4_DDC62F58440E3D7F3A0478813CDDED06` (break `/Game/MPS_V2/Game/Blueprints/Data/Weapon_Anims_Struct` _animations)))
      (set `self.DT_Holster` (`.DT_Holster_6_80D9E65541A1A5F8A0564BB3C899223F` (break `/Game/MPS_V2/Game/Blueprints/Data/Weapon_Anims_Struct` _animations)))
      (set `self.DT_Shoot` (`.DT_Shoot_8_EA975BE247D27CB08EB2AF93728F95CE` (break `/Game/MPS_V2/Game/Blueprints/Data/Weapon_Anims_Struct` _animations)))
      (set `self.DT_Reload_Short` (`.DT_Reload_Short_11_075293ED44061C44879977A7666F9962` (break `/Game/MPS_V2/Game/Blueprints/Data/Weapon_Anims_Struct` _animations)))
      (set `self.DT_Reload_Long` (`.DT_Reload_Long_12_AE1C78D94D86F212CE6FF483B6229A04` (break `/Game/MPS_V2/Game/Blueprints/Data/Weapon_Anims_Struct` _animations)))
      ;[0.3 0.3 0.3] Apply
      (`SkeletalMeshComponent.SetAnimInstanceClass` _item (`self.DT_AnimBP`))
      (`SkinnedMeshComponent.SetSkinnedAssetAndUpdate` _item (`self.DT_WeaponMesh`) true)
      (`PrimitiveComponent.SetMaterial` _item 0 (`self.DT_Material`)))))

(fn `InteractWeapon`
  (returns (WeaponPick :type "/Game/MPS_V2/Game/Blueprints/Weapon_MasterBP Object Reference"))
  (return self))

(fn `LoadLoadout`
  (returns (Material :type "MaterialInstance Object Reference") (Optics :type "StaticMesh Object Reference") (Siderail :type "StaticMesh Object Reference") (Underbarrel :type "StaticMesh Object Reference") (Barrel :type "StaticMesh Object Reference") (OpticsOffset :type "Float (double-precision)") (`HasSilencer?` :type Boolean))
  (bind _savename (`self.SaveName`))
  (bind _returnvalue (`GameplayStatics.DoesSaveGameExist` _savename))
  (if _returnvalue
    (bind _returnvalue_2 (`GameplayStatics.LoadGameFromSlot` _savename))
    (bind _output_get (set `self.SavedLoadout` _returnvalue_2))
    (bind _assave_loadout (cast `/Game/MPS_V2/Game/Blueprints/Data/SaveLoadout` _output_get)
      (:`then`
        (return (`/Game/MPS_V2/Game/Blueprints/Data/SaveLoadout.Material` _assave_loadout) (`/Game/MPS_V2/Game/Blueprints/Data/SaveLoadout.Optics` _assave_loadout) (`/Game/MPS_V2/Game/Blueprints/Data/SaveLoadout.Siderail` _assave_loadout) (`/Game/MPS_V2/Game/Blueprints/Data/SaveLoadout.Underbarrel` _assave_loadout) (`/Game/MPS_V2/Game/Blueprints/Data/SaveLoadout.Barrel` _assave_loadout) (`/Game/MPS_V2/Game/Blueprints/Data/SaveLoadout.OpticsOffset` _assave_loadout) (`/Game/MPS_V2/Game/Blueprints/Data/SaveLoadout.HasSilencer?` _assave_loadout)))
      (:`CastFailed`
        _)))
  (return null null null null null 0.0 false))

(fn `Recoil`
  (bind _returnvalue (`KismetMathLibrary.RandomFloatInRange` -0.3 0.3))
  (bind _returnvalue_2 (`GameplayStatics.GetPlayerCharacter` 0))
  (bind _returnvalue_3 (* (`KismetMathLibrary.RandomFloatInRange` -0.5 -0.8) (/ (`self.DT_Spread_Up`) 3.0)))
  (set `self.Number` (+ (`self.Number`) 1.0))
  (`Pawn.AddControllerPitchInput` _returnvalue_2 _returnvalue_3)
  (set `self.StorePitch` _returnvalue_3)
  (`Pawn.AddControllerYawInput` _returnvalue_2 _returnvalue)
  (set `self.StoreYaw` _returnvalue))

(fn `RemoveMag`
  (params (Condition :type Boolean))
  (if Condition
    (`SkinnedMeshComponent.HideBoneByName` (`self.Item`) "Magazine" "PBO_None")
    (else
      (`SkinnedMeshComponent.HideBoneByName` (`self.Item`) "None" "PBO_None"))))

(fn `SaveLoadout`
  (params (Material :type "MaterialInstance Object Reference") (Optics :type "StaticMesh Object Reference") (Siderail :type "StaticMesh Object Reference") (Underbarrel :type "StaticMesh Object Reference") (Barrel :type "StaticMesh Object Reference") (OpticsOffset :type "Float (double-precision)") (HasSilencer :type Boolean))
  (bind _returnvalue (`GameplayStatics.CreateSaveGameObject` "/Game/MPS_V2/Game/Blueprints/Data/SaveLoadout.SaveLoadout_C"))
  (bind _output_get (set `self.SavedLoadout` _returnvalue))
  (bind _assave_loadout (cast `/Game/MPS_V2/Game/Blueprints/Data/SaveLoadout` _output_get))
  (set `/Game/MPS_V2/Game/Blueprints/Data/SaveLoadout.Material` Material _assave_loadout)
  (set `/Game/MPS_V2/Game/Blueprints/Data/SaveLoadout.Optics` Optics _assave_loadout)
  (set `/Game/MPS_V2/Game/Blueprints/Data/SaveLoadout.Siderail` Siderail _assave_loadout)
  (set `/Game/MPS_V2/Game/Blueprints/Data/SaveLoadout.Underbarrel` Underbarrel _assave_loadout)
  (set `/Game/MPS_V2/Game/Blueprints/Data/SaveLoadout.Barrel` Barrel _assave_loadout)
  (set `/Game/MPS_V2/Game/Blueprints/Data/SaveLoadout.OpticsOffset` OpticsOffset _assave_loadout)
  (set `/Game/MPS_V2/Game/Blueprints/Data/SaveLoadout.HasSilencer?` HasSilencer _assave_loadout)
  (bind _returnvalue_2 (`GameplayStatics.SaveGameToSlot` _output_get (`self.SaveName`)))
  (if _returnvalue_2
    (`KismetSystemLibrary.PrintString` "GameSaved" true true (struct :`R` 0.3 :`G` 0.3 :`B` 0.3 :`A` 0.33))
    (else
      (`KismetSystemLibrary.PrintString` "Error" true true (struct :`R` 1.0 :`G` 0.049243 :`A` 1.0)))))

(fn `SpawnAttachments`
  (bind _item (`self.Item`))
  (bind _item_2 (`self.Item`))
  (bind _barrel_mesh (`self.Barrel_Mesh`))
  (bind _item_3 (`self.Item`))
  (bind _optics_mesh (`self.Optics_Mesh`))
  (bind _underbarrel_mesh (`self.Underbarrel_Mesh`))
  (bind _item_4 (`self.Item`))
  (bind _siderail_mesh (`self.Siderail_Mesh`))
  (`|ExecutionSequence`
    (:`then_0`
      ;[0.3 0.3 0.3] Optics
      (`StaticMeshComponent.SetStaticMesh` _optics_mesh (`self.Optics`))
      (`SceneComponent.K2_SetWorldLocation` _optics_mesh (`SceneComponent.GetSocketLocation` _item_3 "Optics") false false)
      (`SceneComponent.K2_AttachToComponent` _optics_mesh _item_3 "Optics" "SnapToTarget" "SnapToTarget" "KeepRelative" true))
    (:`then_1`
      ;[0.3 0.3 0.3] Siderail
      (`StaticMeshComponent.SetStaticMesh` _siderail_mesh (`self.Siderail`))
      (`SceneComponent.K2_SetWorldLocation` _siderail_mesh (`SceneComponent.GetSocketLocation` _item "Siderail") false false)
      (`SceneComponent.K2_SetWorldRotation` _siderail_mesh (`SceneComponent.GetSocketRotation` _item "Siderail") false false)
      (`SceneComponent.K2_AttachToComponent` _siderail_mesh _item "Siderail" "SnapToTarget" "SnapToTarget" "KeepRelative" true))
    (:`then_2`
      ;[0.3 0.3 0.3] Barrel
      (`StaticMeshComponent.SetStaticMesh` _barrel_mesh (`self.Barrel`))
      (`SceneComponent.K2_SetWorldLocation` _barrel_mesh (`SceneComponent.GetSocketLocation` _item_2 "Barrel") false false)
      (`SceneComponent.K2_AttachToComponent` _barrel_mesh _item_2 "Barrel" "SnapToTarget" "SnapToTarget" "KeepRelative" true))
    (:`then_3`
      ;[0.3 0.3 0.3] Underbarrel
      (`StaticMeshComponent.SetStaticMesh` _underbarrel_mesh (`self.Underbarrel`))
      (`SceneComponent.K2_SetWorldLocation` _underbarrel_mesh (`SceneComponent.GetSocketLocation` _item_4 "Underbarrel") false false)
      (`SceneComponent.K2_AttachToComponent` _underbarrel_mesh _item_4 "Underbarrel" "SnapToTarget" "SnapToTarget" "KeepRelative" true))))

(fn `SpawnProjectile`
  (bind _mps (`self.MPS`))
  (if (`|EnumInequality` (`self.DT_Type`) "NewEnumerator7")
    (`/Game/MPS_V2/Game/Blueprints/Data/MPS_Controller.SpawnProjectile` (cast `/Game/MPS_V2/Game/Blueprints/Data/MPS_Controller` (`GameplayStatics.GetPlayerController` 0) :!pure true) _mps (`/Game/MPS_V2/Game/Blueprints/MPS_MasterBP.FP_Camera` _mps) self (`self.DT_Spread_Right`) (`self.DT_Spread_Up`) :!label _label)
    (else
      (for _ (range (+ (`self.DT_Bullet_Count`) 1))
        (goto _label)))))

(fn `UserConstructionScript`
  (bind _dt_righthand_tf (`self.DT_RightHand_TF`))
  (`parent.UserConstructionScript`)
  (set `self.Type` "NewEnumerator0")
  (set `self.PickupName` (`KismetTextLibrary.Conv_NameToText` (`self.Name`)))
  (`self.DataTable`)
  (set `self.MagSize` (`self.DT_AmmoMag`))
  (`self.SpawnAttachments`)
  (set `self.DT_RightHand_TF` (`KismetMathLibrary.MakeTransform` (`KismetMathLibrary.MakeVector` (.x (.location _dt_righthand_tf)) (.y (.location _dt_righthand_tf)) (+ (.z (.location _dt_righthand_tf)) (`self.Optics_Offset`))) (.rotation _dt_righthand_tf) (.scale _dt_righthand_tf))))