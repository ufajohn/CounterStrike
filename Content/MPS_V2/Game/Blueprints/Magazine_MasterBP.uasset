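; Magazine_MasterBP is the master Blueprint for weapon ammo magazine pickup items, extending a parent interactable item.
; Its Construction Script sets the item type, builds the "{Mag} Ammo" pickup name from Name and applies the item mesh.
; It also looks up the Name row in Weapons_DT to cache slot, type and magazine ammo.
; InteractItem runs the parent logic and returns the magazine itself.
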(fn `DataTable`
  (bind _returnvalue (`|GetDataTableRow` "/Game/MPS_V2/Game/Weapons/Weapons_DT.Weapons_DT" (`self.Name`))
    (:`then`
      (bind ((`Slot_59_D63B79844837C996A69958A48BFD5C24` _slot) (`Type_60_123272EA4DA642ADB23E598C62325188` _type) (`AmmoMag_22_2FDF3348431CCB5B8813F79FB2C0C971` _ammomag)) (break `/Game/MPS_V2/Game/Blueprints/Data/WeaponParameters_Struct` (`.Parameters_19_F721682042B1599A30916CA94C9E68E1` (break `/Game/MPS_V2/Game/Blueprints/Data/Weapons_Struct` _returnvalue))))
      (set `self.DT_Slot` (`KismetMathLibrary.Conv_ByteToInt` _slot))
      (set `self.DT_Type` _type)
      (set `self.DT_Ammo_Mag` _ammomag))))

(fn `InteractItem`
  (returns (MagazinePick :type "/Game/MPS_V2/Game/Blueprints/Magazine_MasterBP Object Reference"))
  (`parent.InteractItem`)
  (return self))

(fn `UserConstructionScript`
  (`parent.UserConstructionScript`)
  (set `self.Type` "NewEnumerator1")
  (set `self.PickupName` (`|FormatText` "{Mag} Ammo" (`KismetTextLibrary.Conv_NameToText` (`self.Name`))))
  (`self.DataTable`)
  (`StaticMeshComponent.SetStaticMesh` (`self.Item_Static`) (`self.Item_Mesh`)))