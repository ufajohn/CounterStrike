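; Base interactable pickup actor with empty InteractItem and InteractWeapon functions, presumably for children to override.
; While unowned, its Overlap volume enables CanPickup on an MPS_MasterBP and shows the name and "F" prompt in the Pickup widget.
; The Spot volume toggles a dot marker on the same widget.
; Construction applies the physics flag to unowned items, and BeginPlay stops Item's simulation after a short delay.
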(event `self.ReceiveBeginPlay`
  (`KismetSystemLibrary.Delay` 5.0)
  (`PrimitiveComponent.SetSimulatePhysics` (`self.Item`) false))

(event `self.Overlap.OnComponentBeginOverlap`
  (params (OverlappedComponent :type "PrimitiveComponent Object Reference") (OtherActor :type "Actor Object Reference") (OtherComp :type "PrimitiveComponent Object Reference") (OtherBodyIndex :type Integer) (bFromSweep :type Boolean) (SweepResult :type "HitResult Structure (by ref)"))
  (bind _returnvalue (`WidgetComponent.GetUserWidgetObject` (`self.Widget`)))
  (bind _returnvalue_2 (`WidgetComponent.GetUserWidgetObject` (`self.Widget`)))
  (bind _aspickup (cast `/Game/MPS_V2/Game/Blueprints/Widgets/Pickup` _returnvalue :!pure true))
  (bind _aspickup_2 (cast `/Game/MPS_V2/Game/Blueprints/Widgets/Pickup` _returnvalue_2 :!pure true))
  (bind _asmps_master_bp (cast `/Game/MPS_V2/Game/Blueprints/MPS_MasterBP` OtherActor)
    (:`then`
      (`/Engine/EditorBlueprintResources/StandardMacros.IsValid` _asmps_master_bp
        (:`Is Valid`
          (if (not (`self.IsOwned?`))
            (set `/Game/MPS_V2/Game/Blueprints/MPS_MasterBP.CanPickup?` true _asmps_master_bp)
            (`/Engine/EditorBlueprintResources/StandardMacros.IsValid` _returnvalue_2
              (:`Is Valid`
                (set `/Game/MPS_V2/Game/Blueprints/Widgets/Pickup.PickupName` (`self.PickupName`) _aspickup_2)
                (set `/Game/MPS_V2/Game/Blueprints/Widgets/Pickup.Press` "Press \"F\" to Pickup" _aspickup_2)))
            (else
              (set `/Game/MPS_V2/Game/Blueprints/MPS_MasterBP.CanPickup?` false _asmps_master_bp :!label _label)
              (`/Engine/EditorBlueprintResources/StandardMacros.IsValid` _returnvalue :!label _label_2
                (:`Is Valid`
                  (set `/Game/MPS_V2/Game/Blueprints/Widgets/Pickup.PickupName` "" _aspickup)
                  (set `/Game/MPS_V2/Game/Blueprints/Widgets/Pickup.Press` "" _aspickup))))))
        (:`Is Not Valid`
          (goto _label))))
    (:`CastFailed`
      (goto _label))))

(event `self.Overlap.OnComponentEndOverlap`
  (params (OverlappedComponent :type "PrimitiveComponent Object Reference") (OtherActor :type "Actor Object Reference") (OtherComp :type "PrimitiveComponent Object Reference") (OtherBodyIndex :type Integer))
  (bind _asmps_master_bp (cast `/Game/MPS_V2/Game/Blueprints/MPS_MasterBP` OtherActor))
  (`/Engine/EditorBlueprintResources/StandardMacros.IsValid` _asmps_master_bp
    (:`Is Valid`
      (set `/Game/MPS_V2/Game/Blueprints/MPS_MasterBP.CanPickup?` false _asmps_master_bp)
      (goto _label_2))))

(event `self.Spot.OnComponentBeginOverlap`
  (params (OverlappedComponent :type "PrimitiveComponent Object Reference") (OtherActor :type "Actor Object Reference") (OtherComp :type "PrimitiveComponent Object Reference") (OtherBodyIndex :type Integer) (bFromSweep :type Boolean) (SweepResult :type "HitResult Structure (by ref)"))
  (bind _returnvalue (`WidgetComponent.GetUserWidgetObject` (`self.Widget`)))
  (bind _asmps_master_bp (cast `/Game/MPS_V2/Game/Blueprints/MPS_MasterBP` OtherActor))
  (`/Engine/EditorBlueprintResources/StandardMacros.IsValid` _asmps_master_bp
    (:`Is Valid`
      (if (not (`self.IsOwned?`))
        (`/Engine/EditorBlueprintResources/StandardMacros.IsValid` _returnvalue
          (:`Is Valid`
            (set `/Game/MPS_V2/Game/Blueprints/Widgets/Pickup.Marker` "." (cast `/Game/MPS_V2/Game/Blueprints/Widgets/Pickup` _returnvalue :!pure true))))))))

(event `self.Spot.OnComponentEndOverlap`
  (params (OverlappedComponent :type "PrimitiveComponent Object Reference") (OtherActor :type "Actor Object Reference") (OtherComp :type "PrimitiveComponent Object Reference") (OtherBodyIndex :type Integer))
  (bind _returnvalue (`WidgetComponent.GetUserWidgetObject` (`self.Widget`)))
  (bind _asmps_master_bp (cast `/Game/MPS_V2/Game/Blueprints/MPS_MasterBP` OtherActor))
  (`/Engine/EditorBlueprintResources/StandardMacros.IsValid` _asmps_master_bp
    (:`Is Valid`
      (`/Engine/EditorBlueprintResources/StandardMacros.IsValid` _returnvalue
        (:`Is Valid`
          (set `/Game/MPS_V2/Game/Blueprints/Widgets/Pickup.Marker` "" (cast `/Game/MPS_V2/Game/Blueprints/Widgets/Pickup` _returnvalue :!pure true)))))))

(fn `InteractItem`
  (returns (MagazinePick :type "/Game/MPS_V2/Game/Blueprints/Magazine_MasterBP Object Reference"))
  (return null))

(fn `InteractWeapon`
  (returns (WeaponPick :type "/Game/MPS_V2/Game/Blueprints/Weapon_MasterBP Object Reference"))
  (return null))

(fn `UserConstructionScript`
  (if (not (`self.IsOwned?`))
    (`PrimitiveComponent.SetSimulatePhysics` (`self.Item_Static`) (`self.IsSimulatingPhysics?`))
    (`PrimitiveComponent.SetSimulatePhysics` (`self.Item`) (`self.IsSimulatingPhysics?`))))