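; Game controller that counts destroyed targets and unlocks doors as the count reaches set milestones.
; Svr_OpenDoor increments ActorsNo and, at the first two milestones, sets CanOpen on the first and second Door_BP found by GetAllActorsOfClass, so door choice depends on array order.
; At those and a final third milestone, it calls MC_Widget, which copies the count to TargetsDestroyed on player 0's MPS_MasterBP character.
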(event `MC_Widget`
  (bind _asmps_master_bp (cast `/Game/MPS_V2/Game/Blueprints/MPS_MasterBP` (`GameplayStatics.GetPlayerCharacter` 0)))
  (set `/Game/MPS_V2/Game/Blueprints/MPS_MasterBP.TargetsDestroyed` (`self.ActorsNo`) _asmps_master_bp))

(event `Svr_OpenDoor`
  (bind _actorsno (`self.ActorsNo`))
  (bind _result (`/Engine/EditorBlueprintResources/StandardMacros.IncrementInt` _actorsno)
    (:`  `
      (set `self.ActorsNo` _result)
      (if (== _actorsno 9)
        (bind _asdoor_bp (castclass `/Game/MPS_V2/Level/Blueprints/Door_BP` "/Game/MPS_V2/Level/Blueprints/Door_BP.Door_BP_C"))
        (bind _outactors (`GameplayStatics.GetAllActorsOfClass` _asdoor_bp))
        (set `/Game/MPS_V2/Level/Blueprints/Door_BP.CanOpen?` true (`|GetArrayItem` _outactors))
        (`self.MC_Widget`)
        (elif (== _actorsno 15)
          (bind _asdoor_bp_2 (castclass `/Game/MPS_V2/Level/Blueprints/Door_BP` "/Game/MPS_V2/Level/Blueprints/Door_BP.Door_BP_C"))
          (bind _outactors_2 (`GameplayStatics.GetAllActorsOfClass` _asdoor_bp_2))
          (set `/Game/MPS_V2/Level/Blueprints/Door_BP.CanOpen?` true (`|GetArrayItem` _outactors_2 1))
          (`self.MC_Widget`)
          (elif (== _actorsno 24)
            (`self.MC_Widget`)))))))

(fn `UserConstructionScript`)