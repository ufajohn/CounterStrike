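; SoundNotify_BP is an animation notify state that plays a sound for the duration of its window in an animation.
; On begin, it sets its Sound on the AudioNotify component of the player-0 MPS_MasterBP character, plays it, then applies its Pitch multiplier.
; On end, it stops that component.
; It always targets the first player's character, whichever mesh triggers the notify.
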(fn `Received_NotifyBegin`
  (params (MeshComp :type "SkeletalMeshComponent Object Reference") (Animation :type "AnimSequenceBase Object Reference") (TotalDuration :type "Float (double-precision)"))
  (returns (ReturnValue :type Boolean))
  (bind _asmps_master_bp (cast `/Game/MPS_V2/Game/Blueprints/MPS_MasterBP` (`GameplayStatics.GetPlayerCharacter` MeshComp)))
  (bind _audionotify (`/Game/MPS_V2/Game/Blueprints/MPS_MasterBP.AudioNotify` _asmps_master_bp))
  (`AudioComponent.SetSound` _audionotify (`self.Sound`))
  (`AudioComponent.Play` _audionotify 0.0)
  (`AudioComponent.SetPitchMultiplier` _audionotify (`self.Pitch`))
  (return false))

(fn `Received_NotifyEnd`
  (params (MeshComp :type "SkeletalMeshComponent Object Reference") (Animation :type "AnimSequenceBase Object Reference"))
  (returns (ReturnValue :type Boolean))
  (bind _asmps_master_bp (cast `/Game/MPS_V2/Game/Blueprints/MPS_MasterBP` (`GameplayStatics.GetPlayerCharacter` MeshComp)))
  (`AudioComponent.Stop` (`/Game/MPS_V2/Game/Blueprints/MPS_MasterBP.AudioNotify` _asmps_master_bp))
  (return false))