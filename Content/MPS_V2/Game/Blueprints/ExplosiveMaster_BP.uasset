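; Master explosive actor that detonates when its HitBox registers a hit, or five seconds after BeginPlay if none has.
; Both triggers share one detonation chain: radial damage with falloff, a RadialForce impulse, explosion sound, scaled-up particle effect and temporary decal.
; The actor destroys itself after a short delay.
; The Hit flag only gates the timed path, so hit events are not guarded against repeats.
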(event `self.ReceiveBeginPlay`
  (bind _returnvalue (`self.K2_GetActorLocation`))
  (`KismetSystemLibrary.Delay` 5.0)
  (if (not (`self.Hit`))
    (`GameplayStatics.ApplyRadialDamageWithFalloff` :`BaseDamage` 1000.0 :`Origin` (`self.K2_GetActorLocation`) :`DamageInnerRadius` 200.0 :`DamageOuterRadius` 500.0 :`DamageFalloff` 2.0 :`DamageTypeClass` "/Script/Engine.DamageType" :`DamageCauser` (`self.GetOwner`) :`InstigatedByController` (`self.GetInstigatorController`) :!label _label)
    (`RadialForceComponent.FireImpulse` (`self.RadialForce`))
    (`GameplayStatics.PlaySoundAtLocation` "/Game/MPS_V2/Game/Sounds/Cue/Explosion_Cue.Explosion_Cue" _returnvalue (struct) 1.0 1.0 0.0 null null null)
    (`GameplayStatics.SpawnEmitterAtLocation` "/Game/MPS_V2/Game/Commons/Particles/P_Explosion.P_Explosion" _returnvalue (struct) (5.0 5.0 5.0))
    (`GameplayStatics.SpawnDecalAtLocation` "/Game/MPS_V2/Game/Commons/Particles/Materials/Decals/Bullet_Decals_M.Bullet_Decals_M" (200.0 200.0 200.0) _returnvalue (struct :`Pitch` -90.0) 20.0)
    (`KismetSystemLibrary.Delay` 0.1)
    (`self.K2_DestroyActor`)))

(event `self.HitBox.OnComponentHit`
  (params (HitComponent :type "PrimitiveComponent Object Reference") (OtherActor :type "Actor Object Reference") (OtherComp :type "PrimitiveComponent Object Reference") (NormalImpulse :type "Vector Structure") (Hit :type "HitResult Structure (by ref)"))
  (set `self.Hit` true)
  (goto _label))

(fn `UserConstructionScript`)