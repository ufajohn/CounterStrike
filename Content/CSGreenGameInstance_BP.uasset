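; Game instance Blueprint that provides a ShowMainMenu event for opening the main menu.
; The event creates a W_MainMenu widget for the first player controller when no valid one is stored, then adds it to the viewport.
; It shows the mouse cursor, switches input to UI-only focused on the menu with fullscreen mouse lock, and stores the widget's Messages in its own variable.
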(event `ShowMainMenu`
  (bind _returnvalue (`GameplayStatics.GetPlayerController` 0))
  (bind _w_mainmenu (`self.W_MainMenu`))
  ;[1 1 1] ShowMainMenu
  (`/Engine/EditorBlueprintResources/StandardMacros.IsValid` (`self.W_MainMenu`)
    (:`Is Valid`
      _)
    (:`Is Not Valid`
      (bind _returnvalue_2 (`|CreateWidget` "/Game/Widgets/W_MainMenu.W_MainMenu_C" _returnvalue))))
  (bind _output_get (set `self.W_MainMenu` _returnvalue_2))
  (`UserWidget.AddToViewport` _output_get 0)
  (set `PlayerController.bShowMouseCursor` true _returnvalue)
  (`WidgetBlueprintLibrary.SetInputMode_UIOnlyEx` _returnvalue _w_mainmenu "LockInFullscreen")
  (set `self.Messages` (`/Game/Widgets/W_MainMenu.messages` _w_mainmenu)))