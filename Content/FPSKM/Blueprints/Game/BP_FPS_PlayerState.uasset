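; Player state for the FPS game, holding weapon slots, carried ammo by type and shop weapon upgrade levels.
; Query functions find the in-use slot and its inventory ammo through the weapon database's ammo type.
; Shop functions rebuild the upgrade list from weapon slots, add missing weapons at level zero and increment levels.
; Each stored level indexes that weapon's database upgrade array to fetch its current upgrade data.
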(event `self.ReceiveBeginPlay`
  ;[1 1 1] Event - BeginPlay
  (bind _asbp_fps_game_inst (cast `/Game/FPSKM/Blueprints/Game/BP_FPS_GameInst` (`GameplayStatics.GetGameInstance`)))
  (set `self.GameInstRef` _asbp_fps_game_inst))

(fn `AddShopWeaponInvenInfo`
  (params (IpWeaponNo :type Integer))
  (if (and (> IpWeaponNo 0) (not (`self.FindShopWeaponInvenInfo` IpWeaponNo)))
    (`KismetArrayLibrary.Array_Add` (`self.ShopWeaponInvenInfoAry`) (make `/Game/FPSKM/Blueprints/Structures/S_ShopWeaponInvenInfo` (`local.IpWeaponNo`)))))

(fn `CollectShopWeaponInvenInfos`
  (`KismetArrayLibrary.Array_Clear` (`self.ShopWeaponInvenInfoAry`))
  (for _array_element (`self.WeaponSlotAry`)
    (`self.AddShopWeaponInvenInfo` (`.WeaponDBNo_15_84B5AB884944E9D099ECCC9DEE41CD33` (break `/Game/FPSKM/Blueprints/Structures/EquipSlots/S_WeaponEquipSlotInfo` _array_element)))))

(fn `FindShopWeaponInvenInfo`
  (params (IpWeaponNo :type Integer))
  (returns (IsFind :type Boolean) (Result :type "/Game/FPSKM/Blueprints/Structures/S_ShopWeaponInvenInfo Structure"))
  (for _array_element (`self.ShopWeaponInvenInfoAry`)
    (if (== (`.WeaponNo_2_DD2EFEA04F5C60B43F42F0AB69134233` (break `/Game/FPSKM/Blueprints/Structures/S_ShopWeaponInvenInfo` _array_element)) (`local.IpWeaponNo`))
      (return true _array_element)))
  (return false (make `/Game/FPSKM/Blueprints/Structures/S_ShopWeaponInvenInfo` 0)))

(fn `FindWeaponUpgradeData`
  (params (IpWeaponNo :type Integer))
  (returns (IsFind :type Boolean) (Result :type "/Game/FPSKM/Blueprints/Structures/S_WeaponUpgradeData Structure"))
  (locals (LocalShopWeaponInvenInfo :type "/Game/FPSKM/Blueprints/Structures/S_ShopWeaponInvenInfo Structure") (LocalGameInst :type "/Game/FPSKM/Blueprints/Game/BP_FPS_GameInst Object Reference"))
  (bind (_isfind _result) (`self.FindShopWeaponInvenInfo` (`local.IpWeaponNo`)))
  (bind (_isfind_2 _weapondata) (`/Game/FPSKM/Blueprints/Game/BPFL_FPS.FindWeaponDBData` (`local.IpWeaponNo`)))
  (bind ((`UpgradeAry_147_13D23180428AC3EB5D4D4DBD9BD4A56A` _upgradeary)) (break `/Game/FPSKM/Blueprints/Structures/ItemData/S_WeaponItemData` _weapondata))
  (`|ExecutionSequence`
    (:`then_0`
      ;[1 1 1] Set Game Instance
      (bind _asbp_fps_game_inst (cast `/Game/FPSKM/Blueprints/Game/BP_FPS_GameInst` (`GameplayStatics.GetGameInstance`)))
      (set `local.LocalGameInst` _asbp_fps_game_inst)
      ;[1 1 1] Check if weapon has upgrade info
      (if _isfind
        (set `local.LocalShopWeaponInvenInfo` _result)
        ;[1 1 1] Get Upgrade Info
        (if _isfind_2
          (if (> (`KismetArrayLibrary.Array_Length` _upgradeary) 0)
            (return true (`|GetArrayItem` _upgradeary (`.UpgradeLevel_4_BFA12D28400D245ECEA7A0B517D2F29D` (break `/Game/FPSKM/Blueprints/Structures/S_ShopWeaponInvenInfo` (`local.LocalShopWeaponInvenInfo`)))))))))
    (:`then_2`
      (return false))))

(fn `GetCharInvenAmmo`
  (params (IpAmmoType :type "/Game/FPSKM/Blueprints/Enums/E_A_AmmoType Enum" :default "NewEnumerator0"))
  (returns (Result :type Integer))
  (bind (_lightammo _mediumammo _heavyammo) (break `/Game/FPSKM/Blueprints/Structures/S_CharInvenInfo` (`self.CharInvenInfo`)))
  (switch `/Game/FPSKM/Blueprints/Enums/E_A_AmmoType` IpAmmoType
    (:`NewEnumerator0`
      (return _lightammo))
    (:`NewEnumerator1`
      (return _mediumammo))
    (:`NewEnumerator2`
      (return _heavyammo))))

(fn `GetCurWeaponInvenAmmo`
  (returns (Result :type Integer))
  (bind (_isfind _result) (`self.GetCurWeaponSlot`))
  (if _isfind
    (bind (_isfind_2 _weapondata) (`/Game/FPSKM/Blueprints/Game/BPFL_FPS.FindWeaponDBData` (`.WeaponDBNo_15_84B5AB884944E9D099ECCC9DEE41CD33` (break `/Game/FPSKM/Blueprints/Structures/EquipSlots/S_WeaponEquipSlotInfo` _result))))
    (if _isfind_2
      (return (`self.GetCharInvenAmmo` (`.AmmoType_111_A99AFC6F49F4437EA31C79B709FCBFE4` (break `/Game/FPSKM/Blueprints/Structures/ItemData/S_WeaponItemData` _weapondata))))
      (else
        (return 0)))
    (else
      (return 0))))

(fn `GetCurWeaponSlot`
  (returns (IsFind :type Boolean) (Result :type "/Game/FPSKM/Blueprints/Structures/EquipSlots/S_WeaponEquipSlotInfo Structure"))
  (for _array_element (`self.WeaponSlotAry`)
    (if (`.IsUsingWeapon_19_7FB370B84CE5CB0B434F4E904BB4B080` (break `/Game/FPSKM/Blueprints/Structures/EquipSlots/S_WeaponEquipSlotInfo` _array_element))
      (return true _array_element)))
  (return false))

(fn `LevelUpShopWeaponInvenInfo`
  (params (IpWeaponNo :type Integer))
  (returns (Result :type Boolean))
  (locals (LocalFindIndex :type Integer :default -1))
  (if (not (`self.FindShopWeaponInvenInfo` (`local.IpWeaponNo`)))
    (`self.AddShopWeaponInvenInfo` (`local.IpWeaponNo`)))
  (`|ExecutionSequence`
    (:`then_0`
      (for (_array_element _array_index) (`self.ShopWeaponInvenInfoAry`)
        (if (== (`.WeaponNo_2_DD2EFEA04F5C60B43F42F0AB69134233` (break `/Game/FPSKM/Blueprints/Structures/S_ShopWeaponInvenInfo` _array_element)) (`local.IpWeaponNo`))
          (set `local.LocalFindIndex` _array_index)))
      (if (> (`local.LocalFindIndex`) -1)
        (`/Engine/EditorBlueprintResources/StandardMacros.IncrementInt` (`.UpgradeLevel_4_BFA12D28400D245ECEA7A0B517D2F29D` (break `/Game/FPSKM/Blueprints/Structures/S_ShopWeaponInvenInfo` (`|GetArrayItem` (`self.ShopWeaponInvenInfoAry`) (`local.LocalFindIndex`))))
          (:`  `
            (return true)))))
    (:`then_1`
      (return false))))

(fn `UserConstructionScript`)