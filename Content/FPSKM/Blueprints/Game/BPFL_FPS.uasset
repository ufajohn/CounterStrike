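; Blueprint function library of shared helpers for the FPS game.
; Looks up weapon and grenade data table rows by converting numeric IDs to row names, returning a found flag with the data.
; A separate search returns a grenade's index within the table's row names.
; Other helpers copy hit info into an SCHitInfo struct and compute screen size as viewport size divided by viewport scale.
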(fn `FindGrenadeDBData`
  (params (No :type Integer))
  (returns (IsFind :type Boolean) (GrenadeData :type "/Game/FPSKM/Blueprints/Structures/ItemData/S_GrenadeItemData Structure"))
  (bind _returnvalue (`|GetDataTableRow` "/Game/FPSKM/Blueprints/DBTables/GrenadeDataTable_FPS.GrenadeDataTable_FPS" (`KismetStringLibrary.Conv_StringToName` (`KismetStringLibrary.Conv_IntToString` No)))
    (:`then`
      (return true _returnvalue))
    (:`RowNotFound`
      (return false))))

(fn `FindGrenadeDBDataIndex`
  (params (InNo :type Integer))
  (returns (IsFind :type Boolean) (ResultIndex :type Integer))
  (locals (LocalIsFind :type Boolean) (LocalIndex :type Integer))
  (bind _outrownames (`DataTableFunctionLibrary.GetDataTableRowNames` "/Game/FPSKM/Blueprints/DBTables/GrenadeDataTable_FPS.GrenadeDataTable_FPS"))
  (for (_array_element _array_index) _outrownames
    (if (`KismetStringLibrary.EqualEqual_StrStr` (`KismetStringLibrary.Conv_NameToString` _array_element) (`KismetStringLibrary.Conv_IntToString` InNo))
      (set `local.LocalIsFind` true)
      (set `local.LocalIndex` _array_index)
      (break)))
  (return (`local.LocalIsFind`) (`local.LocalIndex`)))

(fn `FindWeaponDBData`
  (params (WeaponDBNo :type Integer))
  (returns (IsFind :type Boolean) (WeaponData :type "/Game/FPSKM/Blueprints/Structures/ItemData/S_WeaponItemData Structure"))
  (bind _returnvalue (`|GetDataTableRow` "/Game/FPSKM/Blueprints/DBTables/WeaponDataTable_FPS.WeaponDataTable_FPS" (`KismetStringLibrary.Conv_StringToName` (`KismetStringLibrary.Conv_IntToString` WeaponDBNo)))
    (:`then`
      (return true _returnvalue))
    (:`RowNotFound`
      (return false))))

(fn `GetScreenSize`
  (returns (ReturnValue :type "Vector2D Structure"))
  (bind _returnvalue (`WidgetLayoutLibrary.GetViewportScale` null))
  (bind (_x _y) (`KismetMathLibrary.BreakVector2D` (`WidgetLayoutLibrary.GetViewportSize` null)))
  (return (`KismetMathLibrary.MakeVector2D` (/ _x _returnvalue) (/ _y _returnvalue))))

(fn `ToCHitInfo`
  (params (IpHitInfo :type "HitResult Structure"))
  (returns (S_C_HitInfo :type "/Game/FPSKM/Blueprints/Structures/S_C_HitInfo Structure"))
  (bind (_bblockinghit _binitialoverlap _time _distance _location _impactpoint _normal _impactnormal _physmat _hitactor _hitcomponent _hitbonename) (`GameplayStatics.BreakHitResult` IpHitInfo))
  (return (make `/Game/FPSKM/Blueprints/Structures/S_C_HitInfo` _bblockinghit _location _impactpoint _normal _impactnormal _hitactor _hitcomponent _hitbonename)))