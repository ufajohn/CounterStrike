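; Player controller for the FPS character that routes mobile touch and keyboard/mouse input to movement, combat, stance, weapon and grenade actions.
; Touch events pass through the mobile shooter input component, whose callbacks drive the cached controlled character.
; Tick polls that character to refresh the mobile HUD, re-caching the pawn if invalid.
; OwningClient events run defense-wave UI, toggling shops and waypoints between waves and showing the victory screen.
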(event `InputTouch`
  (params (Location :type "Vector Structure") (FingerIndex :type "ETouchIndex Enum"))
  (bind _bpc_mobiletouchinput_shooter (`self.BPC_MobileTouchInput_Shooter`))
  ;[1 1 1] Input Graph
  (:`Pressed`
    (`/Game/FPSKM/Blueprints/TouchInputCore/Widgets/Widget_MobileShootingMain.OnPressed_InputTouch` _bpc_mobiletouchinput_shooter Location FingerIndex))
  (:`Released`
    (`/Game/FPSKM/Blueprints/TouchInputCore/Widgets/Widget_MobileShootingMain.OnReleased_InputTouch` _bpc_mobiletouchinput_shooter Location FingerIndex))
  (:`Moved`
    (`/Game/FPSKM/Blueprints/TouchInputCore/Widgets/Widget_MobileShootingMain.OnMoved_InputTouch` _bpc_mobiletouchinput_shooter Location FingerIndex)))

(event `self.BPC_MobileTouchInput_Shooter.InputTouch Axis MoveForward`
  (params (AxisValue :type "Float (single-precision)") (JoystickAngle :type "Float (single-precision)") (JoystickMoveLength :type "Float (single-precision)"))
  ;[1 1 1] Input Graph
  (bind _output_get (set `/Game/FPSKM/Blueprints/Characters/Player/BP_FPS_PlayerChar.InputTouchForward` AxisValue (`self.ControlledChar`)))
  (`/Game/FPSKM/Blueprints/Characters/Player/BP_FPS_PlayerChar.MoveForward` (`self.ControlledChar`) _output_get))

(event `self.BPC_MobileTouchInput_Shooter.InputTouch Axis MoveRight`
  (params (AxisValue :type "Float (single-precision)"))
  ;[1 1 1] Input Graph
  (bind _output_get (set `/Game/FPSKM/Blueprints/Characters/Player/BP_FPS_PlayerChar.InputTouchRight` AxisValue (`self.ControlledChar`)))
  (`/Game/FPSKM/Blueprints/Characters/Player/BP_FPS_PlayerChar.MoveRight` (`self.ControlledChar`) _output_get))

(event `self.BPC_MobileTouchInput_Shooter.InputTouch Axis LookUp`
  (params (`Axis Value` :type "Float (single-precision)"))
  ;[1 1 1] Input Graph
  (`self.AddPitchInput` `Axis Value`))

(event `self.BPC_MobileTouchInput_Shooter.InputTouch Axis Turn`
  (params (AxisValue :type "Float (single-precision)"))
  ;[1 1 1] Input Graph
  (`self.AddYawInput` AxisValue))

(event `self.BPC_MobileTouchInput_Shooter.OnPressed Button Fire`
  ;[1 1 1] Input Graph
  (`/Game/FPSKM/Blueprints/Characters/Player/BP_FPS_PlayerChar.Pressed_FireInput` (`self.ControlledChar`)))

(event `self.BPC_MobileTouchInput_Shooter.OnReleased Button Fire`
  ;[1 1 1] Input Graph
  (`/Game/FPSKM/Blueprints/Characters/Player/BP_FPS_PlayerChar.Released_FireInput` (`self.ControlledChar`)))

(event `self.BPC_MobileTouchInput_Shooter.OnPressed Button Reload`
  ;[1 1 1] Input Graph
  (`/Game/FPSKM/Blueprints/Components/WeaponControllers/BPC_BaseWeaponCtrl.ReqReloadStart` (`/Game/FPSKM/Blueprints/Characters/Player/BP_FPS_PlayerChar.CurWeaponCtrl` (`self.ControlledChar`))))

(event `self.BPC_MobileTouchInput_Shooter.OnPressed Button Jump`
  ;[1 1 1] Input Graph
  (if (`/Game/FPSKM/Blueprints/Characters/BP_BaseChar.CanJump_State` (`self.ControlledChar`))
    (`Character.Jump` (`self.ControlledChar`))))

(event `self.BPC_MobileTouchInput_Shooter.OnPressed Button Crouch`
  ;[1 1 1] Input Graph
  (if (not (`/Game/FPSKM/Blueprints/Characters/BP_BaseChar.IsCustomCrouch` (`self.ControlledChar`)))
    (if (`/Game/FPSKM/Blueprints/Characters/BP_BaseChar.CanCrouch_State` (`self.ControlledChar`))
      (`/Game/FPSKM/Blueprints/Characters/Player/BP_FPS_PlayerChar.Released_SprintInput` (`self.ControlledChar`))
      (`/Game/FPSKM/Blueprints/Characters/Player/BP_FPS_PlayerChar.CustomCrouch` (`self.ControlledChar`) true))
    (else
      (`/Game/FPSKM/Blueprints/Characters/Player/BP_FPS_PlayerChar.CustomCrouch` (`self.ControlledChar`) false))))

(event `self.BPC_MobileTouchInput_Shooter.OnPressed Button Aim`
  ;[1 1 1] Input Graph
  (if (not (`/Game/FPSKM/Blueprints/Characters/BP_BaseChar.IsAiming` (`self.ControlledChar`)))
    (if (`/Game/FPSKM/Blueprints/Characters/Player/BP_FPS_PlayerChar.IsCurState` (`self.ControlledChar`) "NewEnumerator0")
      (`/Game/FPSKM/Blueprints/Characters/Player/BP_FPS_PlayerChar.SetAim` (`self.ControlledChar`) true))
    (else
      (`/Game/FPSKM/Blueprints/Characters/Player/BP_FPS_PlayerChar.SetAim` (`self.ControlledChar`) false))))

(event `self.BPC_MobileTouchInput_Shooter.OnReleased Button Jump`
  ;[1 1 1] Input Graph
  (`Character.StopJumping` (`self.ControlledChar`)))

(event `self.BPC_MobileTouchInput_Shooter.OnStart Sprint Input`
  ;[1 1 1] Input Graph
  (`/Game/FPSKM/Blueprints/Characters/Player/BP_FPS_PlayerChar.Pressed_SprintInput` (`self.ControlledChar`)))

(event `self.BPC_MobileTouchInput_Shooter.OnEnd Sprint Input`
  ;[1 1 1] Input Graph
  (`/Game/FPSKM/Blueprints/Characters/Player/BP_FPS_PlayerChar.Released_SprintInput` (`self.ControlledChar`)))

(event `self.BPC_MobileTouchInput_Shooter.OnPressed Button Pickup`
  ;[1 1 1] Input Graph
  (`/Game/FPSKM/Blueprints/Characters/Player/BP_FPS_PlayerChar.ReqInteract` (`self.ControlledChar`)))

(event `self.BPC_MobileTouchInput_Shooter.OnPressed Button WeaponSlot1`
  ;[1 1 1] Input Graph
  (`/Game/FPSKM/Blueprints/Characters/Player/BP_FPS_PlayerChar.StartChangeWeapon` (`self.ControlledChar`) 0))

(event `self.BPC_MobileTouchInput_Shooter.OnPressed Button WeaponSlot2`
  ;[1 1 1] Input Graph
  (`/Game/FPSKM/Blueprints/Characters/Player/BP_FPS_PlayerChar.StartChangeWeapon` (`self.ControlledChar`) 1))

(event `self.BPC_MobileTouchInput_Shooter.OnPressed_Button_GrenadeSlot`
  (params (IpSlotIndex :type Integer))
  ;[1 1 1] Input Graph
  (`/Game/FPSKM/Blueprints/Characters/Player/BP_FPS_PlayerChar.StartChangeGrenade` (`self.ControlledChar`) IpSlotIndex))

(event `InputAxis|Turn`
  (params (AxisValue :type "Float (single-precision)"))
  ;[1 1 1] Input Graph
  (`self.AddYawInput` AxisValue))

(event `InputAxis|LookUp`
  (params (AxisValue :type "Float (single-precision)"))
  ;[1 1 1] Input Graph
  (`self.AddPitchInput` AxisValue))

(event `InputAxis|MoveForward`
  (params (AxisValue :type "Float (single-precision)"))
  ;[1 1 1] Input Graph
  (`/Engine/EditorBlueprintResources/StandardMacros.IsValid` (`self.ControlledChar`)
    (:`Is Valid`
      (`/Game/FPSKM/Blueprints/Characters/Player/BP_FPS_PlayerChar.MoveForward` (`self.ControlledChar`) AxisValue))))

(event `InputAxis|MoveRight`
  (params (AxisValue :type "Float (single-precision)"))
  ;[1 1 1] Input Graph
  (`/Engine/EditorBlueprintResources/StandardMacros.IsValid` (`self.ControlledChar`)
    (:`Is Valid`
      (`/Game/FPSKM/Blueprints/Characters/Player/BP_FPS_PlayerChar.MoveRight` (`self.ControlledChar`) AxisValue))))

(event `InputAction|Sprint`
  (params (Key :type "Key Structure"))
  (bind _controlledchar (`self.ControlledChar`))
  ;[1 1 1] Input Graph
  (:`Pressed`
    (`/Game/FPSKM/Blueprints/Characters/Player/BP_FPS_PlayerChar.Pressed_SprintInput` _controlledchar))
  (:`Released`
    (`/Game/FPSKM/Blueprints/Characters/Player/BP_FPS_PlayerChar.Released_SprintInput` _controlledchar)))

(event `InputAction|Fire`
  (params (Key :type "Key Structure"))
  (bind _controlledchar (`self.ControlledChar`))
  ;[1 1 1] Input Graph
  (:`Pressed`
    (`/Game/FPSKM/Blueprints/Characters/Player/BP_FPS_PlayerChar.Pressed_FireInput` _controlledchar))
  (:`Released`
    (`/Game/FPSKM/Blueprints/Characters/Player/BP_FPS_PlayerChar.Released_FireInput` _controlledchar)))

(event `InputAction|Aim`
  (params (Key :type "Key Structure"))
  ;[1 1 1] Input Graph
  (:`Pressed`
    (if (not (`/Game/FPSKM/Blueprints/Characters/BP_BaseChar.IsAiming` (`self.ControlledChar`)))
      (if (`/Game/FPSKM/Blueprints/Characters/Player/BP_FPS_PlayerChar.IsCurState` (`self.ControlledChar`) "NewEnumerator0")
        (`/Game/FPSKM/Blueprints/Characters/Player/BP_FPS_PlayerChar.SetAim` (`self.ControlledChar`) true))
      (else
        (`/Game/FPSKM/Blueprints/Characters/Player/BP_FPS_PlayerChar.SetAim` (`self.ControlledChar`) false)))))

(event `InputAction|Crouch`
  (params (Key :type "Key Structure"))
  ;[1 1 1] Input Graph
  (:`Pressed`
    (`/Engine/EditorBlueprintResources/StandardMacros.IsValid` (`self.ControlledChar`)
      (:`Is Valid`
        (if (not (`/Game/FPSKM/Blueprints/Characters/BP_BaseChar.IsCustomCrouch` (`self.ControlledChar`)))
          (if (`/Game/FPSKM/Blueprints/Characters/BP_BaseChar.CanCrouch_State` (`self.ControlledChar`))
            (`/Game/FPSKM/Blueprints/Characters/Player/BP_FPS_PlayerChar.Released_SprintInput` (`self.ControlledChar`))
            (`/Game/FPSKM/Blueprints/Characters/Player/BP_FPS_PlayerChar.CustomCrouch` (`self.ControlledChar`) true))
          (else
            (`/Game/FPSKM/Blueprints/Characters/Player/BP_FPS_PlayerChar.CustomCrouch` (`self.ControlledChar`) false)))))))

(event `InputAction|Jump`
  (params (Key :type "Key Structure"))
  ;[1 1 1] Input Graph
  (:`Pressed`
    (if (`/Game/FPSKM/Blueprints/Characters/BP_BaseChar.CanJump_State` (`self.ControlledChar`))
      (`/Game/FPSKM/Blueprints/Characters/BP_BaseChar.CustomCrouch` (`self.ControlledChar`) false)
      (`Character.UnCrouch` (`self.ControlledChar`))
      (`Character.Jump` (`self.ControlledChar`))))
  (:`Released`
    (`Character.StopJumping` (`self.ControlledChar`))))

(event `Key|Two`
  (params (Key :type "Key Structure"))
  ;[1 1 1] Input Graph
  (:`Pressed`
    (`/Game/FPSKM/Blueprints/Characters/Player/BP_FPS_PlayerChar.StartChangeWeapon` (`self.ControlledChar`) 1)))

(event `Key|Three`
  (params (Key :type "Key Structure"))
  ;[1 1 1] Input Graph
  (:`Pressed`
    (`/Game/FPSKM/Blueprints/Characters/Player/BP_FPS_PlayerChar.StartChangeWeapon` (`self.ControlledChar`) 2)))

(event `Key|Four`
  (params (Key :type "Key Structure"))
  ;[1 1 1] Input Graph
  (:`Pressed`
    (`/Game/FPSKM/Blueprints/Characters/Player/BP_FPS_PlayerChar.StartChangeWeapon` (`self.ControlledChar`) 3)))

(event `Key|One`
  (params (Key :type "Key Structure"))
  ;[1 1 1] Input Graph
  (:`Pressed`
    (`/Game/FPSKM/Blueprints/Characters/Player/BP_FPS_PlayerChar.StartChangeWeapon` (`self.ControlledChar`) 0)))

(event `Key|Five`
  (params (Key :type "Key Structure"))
  ;[1 1 1] Input Graph
  (:`Pressed`
    (`/Game/FPSKM/Blueprints/Characters/Player/BP_FPS_PlayerChar.StartChangeWeapon` (`self.ControlledChar`) 4)))

(event `InputAction|Interact`
  (params (Key :type "Key Structure"))
  ;[1 1 1] Input Graph
  (:`Pressed`
    (`/Game/FPSKM/Blueprints/Characters/Player/BP_FPS_PlayerChar.ReqInteract` (`self.ControlledChar`))))

(event `InputAction|Reload`
  (params (Key :type "Key Structure"))
  ;[1 1 1] Input Graph
  (:`Pressed`
    (`/Game/FPSKM/Blueprints/Components/WeaponControllers/BPC_BaseWeaponCtrl.ReqReloadStart` (`/Game/FPSKM/Blueprints/Characters/Player/BP_FPS_PlayerChar.CurWeaponCtrl` (`self.ControlledChar`)))))

(event `InputAction|EquipGrenade`
  (params (Key :type "Key Structure"))
  ;[1 1 1] Input Graph
  (:`Pressed`
    (`/Game/FPSKM/Blueprints/Characters/Player/BP_FPS_PlayerChar.StartChangeGrenade` (`self.ControlledChar`) 0)))

(event `self.ReceiveBeginPlay`
  ;[1 1 1] Event - BeginPlay
  (bind _asbp_fps_player_char (cast `/Game/FPSKM/Blueprints/Characters/Player/BP_FPS_PlayerChar` (`self.K2_GetPawn`)))
  (set `self.ControlledChar` _asbp_fps_player_char))

(event `self.ReceiveTick`
  (params (DeltaSeconds :type "Float (single-precision)"))
  (bind _controlledchar (`self.ControlledChar`))
  (bind _controlledchar_2 (`self.ControlledChar`))
  (bind _controlledchar_3 (`self.ControlledChar`))
  (bind (_icontexture _count) (`/Game/FPSKM/Blueprints/Characters/Player/BP_FPS_PlayerChar.GetGrenadeInfo` (`self.ControlledChar`) 3))
  (bind (_icontexture_2 _count_2) (`/Game/FPSKM/Blueprints/Characters/Player/BP_FPS_PlayerChar.GetGrenadeInfo` (`self.ControlledChar`) 0))
  (bind (_icon _ammo _totalammo) (`/Game/FPSKM/Blueprints/Characters/Player/BP_FPS_PlayerChar.GetWeaponInfo` _controlledchar 1))
  (bind (_icon_2 _ammo_2 _totalammo_2) (`/Game/FPSKM/Blueprints/Characters/Player/BP_FPS_PlayerChar.GetWeaponInfo` _controlledchar 0))
  (bind (_icontexture_3 _count_3) (`/Game/FPSKM/Blueprints/Characters/Player/BP_FPS_PlayerChar.GetGrenadeInfo` (`self.ControlledChar`) 1))
  (bind (_icontexture_4 _count_4) (`/Game/FPSKM/Blueprints/Characters/Player/BP_FPS_PlayerChar.GetGrenadeInfo` (`self.ControlledChar`) 2))
  (`/Engine/EditorBlueprintResources/StandardMacros.IsValid` (`self.ControlledChar`)
    (:`Is Valid`
      (`/Game/FPSKM/Blueprints/TouchInputCore/Widgets/Widget_MobileShootingMain.UpdateButtonWidgets` (`/Game/FPSKM/Blueprints/TouchInputCore/BPC_MobileTouchInput_Shooter.MainWidget` (`self.BPC_MobileTouchInput_Shooter`)) (`/Game/FPSKM/Blueprints/Characters/BP_BaseChar.IsSprint` _controlledchar_3) (`/Game/FPSKM/Blueprints/Characters/BP_BaseChar.IsAiming` _controlledchar_3) (`Character.bIsCrouched` _controlledchar_3) (`/Game/FPSKM/Blueprints/Characters/Player/BP_FPS_PlayerChar.CanPickup` _controlledchar_3))
      (`/Game/FPSKM/Blueprints/TouchInputCore/Widgets/Widget_MobileShootingMain.UpdateHpWidget` (`/Game/FPSKM/Blueprints/TouchInputCore/BPC_MobileTouchInput_Shooter.MainWidget` (`self.BPC_MobileTouchInput_Shooter`)) (`/Game/FPSKM/Blueprints/Characters/BP_BaseChar.Hp` _controlledchar_2) (`/Game/FPSKM/Blueprints/Characters/BP_BaseChar.MaxHp` _controlledchar_2))
      (`/Game/FPSKM/Blueprints/TouchInputCore/Widgets/Widget_MobileShootingMain.UpdateWeaponSlotWidgets` (`/Game/FPSKM/Blueprints/TouchInputCore/BPC_MobileTouchInput_Shooter.MainWidget` (`self.BPC_MobileTouchInput_Shooter`)) _icon_2 _ammo_2 _totalammo_2 _icon _ammo _totalammo (`/Game/FPSKM/Blueprints/Characters/Player/BP_FPS_PlayerChar.CurWeaponSlotIndex` (`self.ControlledChar`)) (`|EnumEquality` (`/Game/FPSKM/Blueprints/Characters/BP_BaseChar.CurWeaponItemType` (`self.ControlledChar`)) "NewEnumerator1"))
      (`/Game/FPSKM/Blueprints/TouchInputCore/Widgets/Widget_UseItemSlotAry.UpdateWidgets` (`/Game/FPSKM/Blueprints/TouchInputCore/Widgets/Widget_MobileShootingMain.Widget_GrenadeItemSlotAry` (`/Game/FPSKM/Blueprints/TouchInputCore/BPC_MobileTouchInput_Shooter.MainWidget` (`self.BPC_MobileTouchInput_Shooter`))) (`/Game/FPSKM/Blueprints/Characters/Player/BP_FPS_PlayerChar.CurGrenadeSlotIndex` (`self.ControlledChar`)) _icontexture_2 _count_2 _icontexture_3 _count_3 _icontexture_4 _count_4 _icontexture _count (`|EnumEquality` (`/Game/FPSKM/Blueprints/Characters/BP_BaseChar.CurWeaponItemType` (`self.ControlledChar`)) "NewEnumerator8")))
    (:`Is Not Valid`
      (bind _asbp_fps_player_char (cast `/Game/FPSKM/Blueprints/Characters/Player/BP_FPS_PlayerChar` (`self.K2_GetPawn`)))
      (set `self.ControlledChar` _asbp_fps_player_char))))

(event `OwningClient_DefenseGamePlayWidget`
  ;[1 1 1] Wave Logic - OwningClient
  (bind _returnvalue (`|CreateWidget` "/Game/FPSKM/Blueprints/Widgets/Widget_DefenseGamePlay.Widget_DefenseGamePlay_C" (`GameplayStatics.GetPlayerController` 0)))
  (bind _output_get (set `self.DefenseGamePlayWidget` _returnvalue))
  (`UserWidget.AddToViewport` _output_get 0)
  (`/Game/FPSKM/Blueprints/Widgets/Widget_DefenseGamePlay.SetMode` (`self.DefenseGamePlayWidget`) "NewEnumerator0"))

(event `OwningClient_WaveComplete_WaitNextWave`
  ;[1 1 1] Wave Logic - OwningClient
  (`/Game/FPSKM/Blueprints/Widgets/Widget_DefenseGamePlay.ShowMsgComplete` (`self.DefenseGamePlayWidget`) "SelfHitTestInvisible" 3.0)
  (`/Game/FPSKM/Blueprints/Widgets/Widget_DefenseGamePlay.SetMode` (`self.DefenseGamePlayWidget`) "NewEnumerator2")
  (`/Game/FPSKM/Blueprints/Characters/Player/BP_FPS_PlayerChar.ActivateWaypoints` (`self.ControlledChar`))
  (bind _outactors (`GameplayStatics.GetAllActorsOfClass` "/Game/FPSKM/Blueprints/Actors/BP_DefenseShop.BP_DefenseShop_C"))
  (for _array_element _outactors
    (`/Game/FPSKM/Blueprints/Actors/BP_DefenseShop.Show` _array_element true)))

(event `OwningClient_StartNextWave`
  ;[1 1 1] Wave Logic - OwningClient
  (`/Game/FPSKM/Blueprints/Widgets/Widget_DefenseGamePlay.ShowMsgInComming` (`self.DefenseGamePlayWidget`) "SelfHitTestInvisible" 5.0)
  (`/Game/FPSKM/Blueprints/Widgets/Widget_DefenseGamePlay.SetMode` (`self.DefenseGamePlayWidget`) "NewEnumerator1")
  (`/Game/FPSKM/Blueprints/Characters/Player/BP_FPS_PlayerChar.DeactivateWayPoints` (`self.ControlledChar`))
  (bind _outactors (`GameplayStatics.GetAllActorsOfClass` "/Game/FPSKM/Blueprints/Actors/BP_DefenseShop.BP_DefenseShop_C"))
  (for _array_element _outactors
    (`/Game/FPSKM/Blueprints/Actors/BP_DefenseShop.Show` _array_element false)))

(event `OwningClient_StartBossNextWave`
  ;[1 1 1] Wave Logic - OwningClient
  (`/Game/FPSKM/Blueprints/Widgets/Widget_DefenseGamePlay.ShowMsgBossInComing` (`self.DefenseGamePlayWidget`) "SelfHitTestInvisible" 5.0)
  (`/Game/FPSKM/Blueprints/Widgets/Widget_DefenseGamePlay.SetMode` (`self.DefenseGamePlayWidget`) "NewEnumerator1"))

(event `OwningClient_Victory`
  ;[1 1 1] Wave Logic - OwningClient
  (`/Game/FPSKM/Blueprints/Widgets/Widget_DefenseGamePlay.ShowVictory` (`self.DefenseGamePlayWidget`) "SelfHitTestInvisible" 5.0)
  (`/Game/FPSKM/Blueprints/Widgets/Widget_DefenseGamePlay.SetMode` (`self.DefenseGamePlayWidget`) "NewEnumerator4")
  (`KismetSystemLibrary.Delay` 5.2)
  (`self.ShowVictoryWidget`))

(event `ShowVictoryWidget`
  (bind _asbp_fps_game_inst (cast `/Game/FPSKM/Blueprints/Game/BP_FPS_GameInst` (`GameplayStatics.GetGameInstance`)))
  (`/Game/FPSKM/Blueprints/Game/BP_FPS_GameInst.ShowPlayerVictoryWidget` _asbp_fps_game_inst true)
  (`WidgetBlueprintLibrary.SetInputMode_UIOnlyEx` (`GameplayStatics.GetPlayerController` 0) (`/Game/FPSKM/Blueprints/Game/BP_FPS_GameInst.VictoryWidgetRef` _asbp_fps_game_inst))
  (set `PlayerController.bShowMouseCursor` true (`GameplayStatics.GetPlayerController` 0)))

(fn `UserConstructionScript`
  (`parent.UserConstructionScript`))