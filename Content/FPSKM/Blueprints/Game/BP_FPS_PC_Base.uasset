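; Base player controller for the FPS game that caches the controlled hero and handles player respawn requests.
; On BeginPlay it stores the possessed BP_FPS_PlayerChar as ControlledBaseHero.
; A respawn request copies the character's weapon slot array to the PlayerState when that character is possessed.
; After a short delay, it asks BP_FPS_GameMode to respawn this controller's player.
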(event `self.ReceiveBeginPlay`
  ;[1 1 1] Event - BeginPlay
  (bind _asbp_fps_player_char (cast `/Game/FPSKM/Blueprints/Characters/Player/BP_FPS_PlayerChar` (`self.K2_GetPawn`)))
  (set `self.ControlledBaseHero` _asbp_fps_player_char))

(event `ReqRespawnPlayerEvent`
  ;[1 1 1] RespawnPlayer
  ;;[1 1 1] Set WeaponSlotArt To PlayerState
  (bind _asbp_fps_player_char (cast `/Game/FPSKM/Blueprints/Characters/Player/BP_FPS_PlayerChar` (`self.K2_GetPawn`))
    (:`then`
      (bind _asbp_fps_player_state (cast `/Game/FPSKM/Blueprints/Game/BP_FPS_PlayerState` (`self.PlayerState`)))
      (set `/Game/FPSKM/Blueprints/Game/BP_FPS_PlayerState.WeaponSlotAry` (`/Game/FPSKM/Blueprints/Characters/Player/BP_FPS_PlayerChar.WeaponSlotAry` _asbp_fps_player_char) _asbp_fps_player_state))
    (:`CastFailed`
      _))
  ;;[1 1 1] Respawn Player Character
  (`KismetSystemLibrary.Delay` 0.5)
  (bind _asbp_fps_game_mode (cast `/Game/FPSKM/Blueprints/Game/BP_FPS_GameMode` (`GameplayStatics.GetGameMode`)))
  (`/Game/FPSKM/Blueprints/Game/BP_FPS_GameMode.RespawnPlayerEvent` _asbp_fps_game_mode self))

(fn `UserConstructionScript`)