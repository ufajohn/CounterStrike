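; FPS game mode that respawns player characters and relays character death and disappearance events to other actors.
; Respawning cycles through PlayerStarts by respawn count, replaces and possesses the pawn, then notifies DamageInterface actors.
; Deaths are forwarded to enemies, player characters and wave spawners for kill counting, while player disappearances go to all DamageInterface actors.
; A helper checks whether an actor is listed in the hero respawn info array.
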(event `self.ReceiveBeginPlay`
  ;[1 1 1] Event - BeginPlay
  (bind _asbp_fps_game_inst (cast `/Game/FPSKM/Blueprints/Game/BP_FPS_GameInst` (`GameplayStatics.GetGameInstance`)))
  (set `self.GameInstRef` _asbp_fps_game_inst))

(event `RespawnPlayerEvent`
  (params (IpPC :type "PlayerController Object Reference"))
  (bind _returnvalue (`Controller.K2_GetPawn` IpPC))
  ;[1 1 1] RespawnPlayerEvent
  (bind _outactors (`GameplayStatics.GetAllActorsOfClass` "/Script/Engine.PlayerStart"))
  ;;[1 1 1] Set Spawn Index and Set Respawn Count
  (set `self.SpawnIndex` (mod (`self.RespawnCount`) (`KismetArrayLibrary.Array_Length` _outactors)))
  (set `self.RespawnCount` (+ (`self.RespawnCount`) 1))
  (`|ExecutionSequence`
    (:`then_0`
      ;;[1 1 1] Destory Player Character
      (`/Engine/EditorBlueprintResources/StandardMacros.IsValid` _returnvalue
        (:`Is Valid`
          (`self.K2_DestroyActor` _returnvalue))))
    (:`then_1`
      ;;[1 1 1] Spawn a Player Character and Possess it
      (bind _returnvalue_2 (`|SpawnActorFromClass` (`self.HeroClass`) (`self.GetTransform` (`|GetArrayItem` _outactors (`self.SpawnIndex`))) "Undefined" "OverrideRootScale" null null))
      (bind _asbp_fps_player_char (cast `/Game/FPSKM/Blueprints/Characters/Player/BP_FPS_PlayerChar` _returnvalue_2))
      (`Controller.Possess` IpPC _asbp_fps_player_char)
      (set `self.TempNewHero` _asbp_fps_player_char))
    (:`then_2`
      ;;[1 1 1] Call OnRespawnPlayerEvent of all actors
      (bind _outactors_2 (`GameplayStatics.GetAllActorsWithInterface` "/Game/FPSKM/Blueprints/Interfaces/DamageInterface.DamageInterface_C"))
      (for _array_element _outactors_2
        (if (!= _array_element self)
          (message `/Game/FPSKM/Blueprints/Interfaces/DamageInterface.OnRespawnPlayerCharacter` _array_element (`self.TempNewHero`)))))))

(event `/Game/FPSKM/Blueprints/Interfaces/DamageInterface.OnCharDeath`
  (params (IpChar :type "/Game/FPSKM/Blueprints/Characters/BP_BaseChar Object Reference") (IpCHitInfo :type "/Game/FPSKM/Blueprints/Structures/S_C_HitInfo Structure"))
  ;[1 1 1] Event - OnCharDeath
  (set `self.TempDeathChar` IpChar)
  (set `self.TempDeathCHitInfo` IpCHitInfo)
  (`|ExecutionSequence`
    (:`then_0`
      (bind _outactors (`GameplayStatics.GetAllActorsOfClass` "/Game/FPSKM/Blueprints/Characters/Enemies/BP_FPS_BaseEnemy.BP_FPS_BaseEnemy_C"))
      (for _array_element _outactors
        (if (!= _array_element self)
          (message `/Game/FPSKM/Blueprints/Interfaces/DamageInterface.OnCharDeath` _array_element (`self.TempDeathChar`) (`self.TempDeathCHitInfo`)))))
    (:`then_1`
      (bind _outactors_2 (`GameplayStatics.GetAllActorsOfClass` "/Game/FPSKM/Blueprints/Characters/Player/BP_FPS_PlayerChar.BP_FPS_PlayerChar_C"))
      (for _array_element_2 _outactors_2
        (if (!= _array_element_2 self)
          (message `/Game/FPSKM/Blueprints/Interfaces/DamageInterface.OnCharDeath` _array_element_2 (`self.TempDeathChar`) (`self.TempDeathCHitInfo`)))))
    (:`then_2`
      ;;[1 1 1] Call OnCharDeathEvent of Spanwer to count kill number
      (bind _outactors_3 (`GameplayStatics.GetAllActorsOfClass` "/Game/FPSKM/Blueprints/Spanwer/BP_DefaultWaveSpawner.BP_DefaultWaveSpawner_C"))
      (for _array_element_3 _outactors_3
        (`/Game/FPSKM/Blueprints/Interfaces/DamageInterface.OnCharDeath` _array_element_3 (`self.TempDeathChar`) (`self.TempDeathCHitInfo`))))))

(event `/Game/FPSKM/Blueprints/Interfaces/DamageInterface.OnCharDisappear`
  (params (IpChar :type "/Game/FPSKM/Blueprints/Characters/BP_BaseChar Object Reference"))
  ;[1 1 1] Event - OnCharDisappear
  ;;[1 1 1] Call OnCharDisappear of all actors
  (cast `/Game/FPSKM/Blueprints/Characters/Player/BP_FPS_PlayerChar` IpChar)
  (bind _outactors (`GameplayStatics.GetAllActorsWithInterface` "/Game/FPSKM/Blueprints/Interfaces/DamageInterface.DamageInterface_C"))
  (for _array_element _outactors
    (if (!= _array_element self)
      (message `/Game/FPSKM/Blueprints/Interfaces/DamageInterface.OnCharDisappear` _array_element IpChar))))

(fn `IsPlayerChar`
  (params (IpCheckActor :type "/Game/FPSKM/Blueprints/Characters/BP_BaseChar Object Reference"))
  (returns (Result :type Boolean))
  (for _array_element (`self.HeroRespawnInfoAry`)
    (if (== (`.HeroRef_3_DEF437A4409BD0FA95B33FBE348BF2A1` (break `/Game/FPSKM/Blueprints/Structures/S_HeroRespawnInfo` _array_element)) IpCheckActor)
      (return true)))
  (return false))

(fn `UserConstructionScript`)