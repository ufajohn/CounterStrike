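; Game instance for the FPS kit that holds shared weapon and item data and manages global HUD widgets.
; On Init it copies every weapon DataTable row into an array, and it looks up use-item data by number.
; It lazily creates and caches crosshair, death and victory widgets to show or hide them.
; A helper converts world positions to viewport-scale-corrected screen coordinates.
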(event `self.ReceiveInit`
  ;[1 1 1] Event - Init
  ;;[1 1 1] Add All WeaponData to WeaponItemDataAry
  (bind _outrownames (`DataTableFunctionLibrary.GetDataTableRowNames` (`self.WeaponDBTable`)))
  (for _array_element _outrownames
    (bind _returnvalue (`|GetDataTableRow` (`self.WeaponDBTable`) _array_element)
      (:`then`
        (`KismetArrayLibrary.Array_Add` (`self.WeaponItemDataAry`) _returnvalue)))))

(fn `FindUseItemData`
  (params (IpNo :type Integer))
  (returns (IsFind :type Boolean) (UseItemData :type "/Game/FPSKM/Blueprints/Structures/ItemData/S_UseItemData Structure"))
  (for _array_element (`self.UseItemDataAry`)
    (if (== (`.No_2_3646AAE646050B71BCAA73A535E1A552` (break `/Game/FPSKM/Blueprints/Structures/ItemData/S_UseItemData` _array_element)) (`local.IpNo`))
      (return true _array_element)))
  (return false (make `/Game/FPSKM/Blueprints/Structures/ItemData/S_UseItemData` 0 "Injection" "" null "WeaponSocket_R_Injection" null null)))

(fn `ShowCrosshair`
  (params (IpCrosshairType :type "/Game/FPSKM/Blueprints/Crosshair/Enums/E_CrosshairType Enum" :default "NewEnumerator2") (Visible :type Boolean))
  (locals (LocalIsDeathMatchMode :type Boolean))
  (bind _crosshairwidgetref (`self.CrosshairWidgetRef`))
  (`/Engine/EditorBlueprintResources/StandardMacros.IsValid` (`self.CrosshairWidgetRef`)
    (:`Is Valid`
      _)
    (:`Is Not Valid`
      (bind _returnvalue (`|CreateWidget` "/Game/FPSKM/Blueprints/Crosshair/Widgets/Widget_Crosshair_Main.Widget_Crosshair_Main_C"))
      (set `self.CrosshairWidgetRef` _returnvalue)))
  (if (not (`Widget.IsInViewport` _crosshairwidgetref))
    (`UserWidget.AddToViewport` _crosshairwidgetref 0))
  (`/Game/FPSKM/Blueprints/Crosshair/Widgets/Widget_Crosshair_Main.ShowCrosshair` (`self.CrosshairWidgetRef`) (`local.IpCrosshairType`) (`local.Visible`)))

(fn `ShowPlayerDeathWidget`
  (params (Visible :type Boolean))
  (bind _playerdeathwidgetref (`self.PlayerDeathWidgetRef`))
  (`/Engine/EditorBlueprintResources/StandardMacros.IsValid` (`self.PlayerDeathWidgetRef`)
    (:`Is Valid`
      _)
    (:`Is Not Valid`
      (bind _returnvalue (`|CreateWidget` "/Game/FPSKM/Blueprints/Widgets/Widget_PlayerDeath.Widget_PlayerDeath_C" (`GameplayStatics.GetPlayerController` 0)))
      (set `self.PlayerDeathWidgetRef` _returnvalue)))
  (if Visible
    (`UserWidget.AddToViewport` _playerdeathwidgetref 0)
    (else
      (`Widget.RemoveFromParent` _playerdeathwidgetref))))

(fn `ShowPlayerVictoryWidget`
  (params (Visible :type Boolean))
  (bind _victorywidgetref (`self.VictoryWidgetRef`))
  (`/Engine/EditorBlueprintResources/StandardMacros.IsValid` (`self.VictoryWidgetRef`)
    (:`Is Valid`
      _)
    (:`Is Not Valid`
      (bind _returnvalue (`|CreateWidget` "/Game/FPSKM/Blueprints/Widgets/Widget_PlayerVictory.Widget_PlayerVictory_C" (`GameplayStatics.GetPlayerController` 0)))
      (set `self.VictoryWidgetRef` _returnvalue)))
  (if Visible
    (`UserWidget.AddToViewport` _victorywidgetref 0)
    (else
      (`Widget.RemoveFromParent` _victorywidgetref))))

(fn `WorldToScreen`
  (params (IpPos :type "Vector Structure"))
  (returns (IpResult :type "Vector2D Structure"))
  (bind _returnvalue (`WidgetLayoutLibrary.GetViewportScale`))
  (bind (_x _y) (`KismetMathLibrary.BreakVector2D` (`GameplayStatics.ProjectWorldToScreen` (`GameplayStatics.GetPlayerController` 0) IpPos true)))
  (return (`KismetMathLibrary.MakeVector2D` (/ _x _returnvalue) (/ _y _returnvalue))))