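; Thrown grenade projectile that explodes when its fuse time runs out after release.
; Throw launches the physics-simulated skeletal mesh, hides its pin and ignores the owner, then sets Pawn collision to block after a short delay.
; Tick counts the fuse, then makes noise and triggers Bomb: radial impulse, particles, sound, optional camera shake and actor destruction.
; Mesh hits play a bounce sound for the first few impacts.
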(event `self.ReceiveTick`
  (params (DeltaSeconds :type "Float (single-precision)"))
  ;[1 1 1] Tick
  (if (`self.IsThrow`)
    (if (not (`self.IsBomb`))
      ;;[1 1 1] Increase Life Time
      (set `self.CheckLifeTime` (+ DeltaSeconds (`self.CheckLifeTime`)))
      ;;[1 1 1] Check if Life Time is over
      (if (>= (`self.CheckLifeTime`) (`self.LifeTime`))
        (set `self.IsBomb` true)
        (`self.MakeNoise` 1.0 (`self.GetInstigator`) (`self.K2_GetActorLocation`))
        (`SceneComponent.K2_SetWorldLocation` (`self.RadialForce`) (`self.K2_GetActorLocation`) false false)
        (`self.Bomb`)))))

(event `Bomb`
  ;[1 1 1] Bomb
  (`RadialForceComponent.FireImpulse` (`self.RadialForce`))
  (`GameplayStatics.SpawnEmitterAtLocation` (`self.BombParticleSystem`) (`self.K2_GetActorLocation`) (`KismetMathLibrary.Conv_VectorToRotator` (0.0 0.0 0.0)) (3.0 3.0 3.0))
  (`GameplayStatics.PlaySoundAtLocation` (`self.BombSound`) (`self.K2_GetActorLocation`) (struct) 1.0 1.0 0.0 null null null)
  (if (`KismetSystemLibrary.IsValidClass` (`self.BombCamShake`))
    (`PlayerController.ClientStartCameraShake` (`GameplayStatics.GetPlayerController` 0) (`self.BombCamShake`) 1.0 "UserDefined" (`self.K2_GetActorRotation`)))
  (`self.K2_DestroyActor`))

(event `Throw`
  (params (Vel :type "Vector Structure"))
  (bind _skeletalmeshcomponent (`self.SkeletalMeshComponent`))
  ;[1 1 1] Throw
  (`PrimitiveComponent.IgnoreActorWhenMoving` (`self.SkeletalMeshComponent`) (`self.GetOwner`) true)
  (`PrimitiveComponent.SetCollisionEnabled` (`self.SkeletalMeshComponent`) "QueryAndPhysics")
  (`PrimitiveComponent.SetSimulatePhysics` _skeletalmeshcomponent true)
  (`PrimitiveComponent.SetPhysicsLinearVelocity` _skeletalmeshcomponent Vel false "None")
  (`SkinnedMeshComponent.HideBoneByName` (`self.SkeletalMeshComponent`) "Pin" "PBO_None")
  (set `self.IsThrow` true)
  (clear `self.OnWarningTime_Grendae`)
  (`KismetSystemLibrary.Delay` 0.32)
  (`PrimitiveComponent.SetCollisionResponseToChannel` (`self.SkeletalMeshComponent`) "ECC_Pawn" "ECR_Block"))

(event `PullPin`
  ;[1 1 1] Pull Pin
)

(event `self.SkeletalMeshComponent.OnComponentHit`
  (params (HitComponent :type "PrimitiveComponent Object Reference") (OtherActor :type "Actor Object Reference") (OtherComp :type "PrimitiveComponent Object Reference") (NormalImpulse :type "Vector Structure") (Hit :type "HitResult Structure (by ref)"))
  ;[1 1 1] OnComponentHit(SkeletalMeshComponent)
  (set `self.IsHit` true)
  (bind _result (`/Engine/EditorBlueprintResources/StandardMacros.IncrementInt` (`self.BounceCount`))
    (:`  `
      (if (< _result 3)
        (`GameplayStatics.PlaySoundAtLocation` (`self.BounceSound`) (`self.K2_GetActorLocation`) (struct) 1.0 1.0 0.0 null null null)))))

(event `HidePin`
  ;[1 1 1] Hide Pin
  (`SkinnedMeshComponent.HideBoneByName` (`self.SkeletalMeshComponent`) "Pin" "PBO_None"))

(fn `GetAnimInst`
  (returns (ReturnValue :type "AnimInstance Object Reference"))
  (return (`SkeletalMeshComponent.GetAnimInstance` (`self.SkeletalMeshComponent`))))

(fn `UserConstructionScript`)