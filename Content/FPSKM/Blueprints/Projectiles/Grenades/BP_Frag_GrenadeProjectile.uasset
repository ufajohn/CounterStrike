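; Frag grenade projectile that runs a fuse on Tick once its pin is pulled.
; It fires a warning event one second before expiry, then makes AI noise, moves its radial force and calls Bomb.
; Hits apply a warning emissive material and play sound for the first few bounces.
; Bomb is empty here; the explosion chain of impulse, effects, sphere-trace damage and destroy is disconnected.
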(event `self.ReceiveTick`
  (params (DeltaSeconds :type "Float (single-precision)"))
  ;[1 1 1] Tick
  (if (`self.IsPullPin`)
    (`|ExecutionSequence`
      (:`then_0`
        (if (not (`self.IsBomb`))
          ;;[1 1 1] Increase Life Time
          (set `self.CheckLifeTime` (+ (`GameplayStatics.GetWorldDeltaSeconds`) (`self.CheckLifeTime`)))
          ;;[1 1 1] Check if Life Time is over
          (if (>= (`self.CheckLifeTime`) (`self.LifeTime`))
            (set `self.IsBomb` true)
            (`self.MakeNoise` 1.0 (`self.GetInstigator`) (`self.K2_GetActorLocation`))
            (`SceneComponent.K2_SetWorldLocation` (`self.RadialForce`) (`self.K2_GetActorLocation`) false false)
            (`self.Bomb`))))
      (:`then_1`
        (if (not (`self.IsFireWarningEvent`))
          (if (>= (`self.CheckLifeTime`) (- (`self.LifeTime`) 1.0))
            (set `self.IsFireWarningEvent` true)
            (`self.OnWarningTime_Grendae`)))))))

(event `self.PullPin`
  ;[1 1 1] Event - Pull Pin
  (set `self.IsPullPin` true))

(event `self.SkeletalMeshComponent.OnComponentHit`
  (params (HitComponent :type "PrimitiveComponent Object Reference") (OtherActor :type "Actor Object Reference") (OtherComp :type "PrimitiveComponent Object Reference") (NormalImpulse :type "Vector Structure") (Hit :type "HitResult Structure (by ref)"))
  ;[1 1 1] OnComponentHit(SkeletalMeshComponent)
  (set `self.IsHit` true)
  (`PrimitiveComponent.SetMaterial` (`self.SkeletalMeshComponent`) 0 "/Game/FPSKM/Materials/MI_Emissive_GrenadeWarning.MI_Emissive_GrenadeWarning")
  (bind _result (`/Engine/EditorBlueprintResources/StandardMacros.IncrementInt` (`self.BounceCount`))
    (:`  `
      (if (< _result 3)
        (`GameplayStatics.PlaySoundAtLocation` (`self.BounceSound`) (`self.K2_GetActorLocation`) (struct) 1.0 1.0 0.0 null null null)))))

(event `self.Bomb`
  ;[1 1 1] Bomb
)

(fn `UserConstructionScript`
  (`parent.UserConstructionScript`))