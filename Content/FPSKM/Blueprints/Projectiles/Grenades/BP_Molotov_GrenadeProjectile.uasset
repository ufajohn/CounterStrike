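; Molotov grenade projectile for the FPS weapon set that detonates on impact once thrown.
; Tick accumulates lifetime but triggers only on the hit flag, then makes noise, repositions the radial force and calls Bomb.
; Bomb is empty here, overriding any inherited behavior without calling it.
; Disconnected, never-executed nodes hold fire-area spawning, explosion effects, camera shake, sphere-trace random damage and actor destruction.
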(event `self.ReceiveTick`
  (params (DeltaSeconds :type "Float (single-precision)"))
  ;[1 1 1] Tick
  (if (`self.IsThrow`)
    (if (not (`self.IsBomb`))
      ;;[1 1 1] Increase Life Time
      (set `self.CheckLifeTime` (+ DeltaSeconds (`self.CheckLifeTime`)))
      ;;[1 1 1] Check if Life Time is over
      (if (`self.IsHit`)
        (set `self.IsBomb` true)
        (`self.MakeNoise` 1.0 (`self.GetInstigator`) (`self.K2_GetActorLocation`))
        (`SceneComponent.K2_SetWorldLocation` (`self.RadialForce`) (`self.K2_GetActorLocation`) false false)
        (`self.Bomb`)))))

(event `self.Bomb`
  ;[1 1 1] Bomb
)

(fn `UserConstructionScript`
  (`parent.UserConstructionScript`))