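; Base projectile Blueprint for weapons: Launch stores weapon data, ignores the instigator, activates movement and destroys itself after its lifetime.
; On hit it makes noise, then damages DamageInterface actors with random weapon or upgrade damage, doubled for criticals and again for headshots.
; Those hits also spawn surface-based particles and decals before destroying the projectile.
; Team collision setup runs on BeginPlay, but its channel logic is disconnected, as is hit sound.
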(event `self.ReceiveBeginPlay`
  ;[1 1 1] Event - BeginPlay
  (`self.SettingTeamCollision` (`self.TeamNumber`)))

(event `self.SphereCollision.OnComponentHit`
  (params (HitComponent :type "PrimitiveComponent Object Reference") (OtherActor :type "Actor Object Reference") (OtherComp :type "PrimitiveComponent Object Reference") (NormalImpulse :type "Vector Structure") (Hit :type "HitResult Structure (by ref)"))
  (`self.DamageProcess` OtherActor Hit))

(event `HitEffect`
  (params (IpLoc :type "Vector Structure") (IpNormal :type "Vector Structure") (SurfaceType :type "EPhysicalSurface Enum" :default "SurfaceType_Default"))
  (`self.SpawnHitEffects` IpLoc IpNormal SurfaceType)
  (`self.K2_DestroyActor`))

(event `Launch`
  (params (IpWeaponData :type "/Game/FPSKM/Blueprints/Structures/ItemData/S_WeaponItemData Structure"))
  ;[1 1 1] Launch
  (set `self.WeaponInfo` IpWeaponData)
  (`PrimitiveComponent.IgnoreActorWhenMoving` (`self.SphereCollision`) (`self.GetInstigator`) true)
  (`ActorComponent.SetActive` (`self.ProjectileMovement`) true false)
  (`KismetSystemLibrary.Delay` (`self.LifeTime`))
  (`self.K2_DestroyActor`))

(event `SettingTeamCollision`
  (params (IpTeamNumber :type Integer))
  ;[1 1 1] Set Team Collision
  (if (== IpTeamNumber 0)
    (`self.SettingBodySphereCollision` "ECC_GameTraceChannel2")
    (elif (== IpTeamNumber 1)
      (`self.SettingBodySphereCollision` "ECC_GameTraceChannel8"))))

(event `SettingBodySphereCollision`
  (params (IpCollisionChannel :type "ECollisionChannel Enum" :default "ECC_WorldStatic")))

(fn `CalculateDamage`
  (returns (ResultDamage :type "Float (double-precision)") (IsCritical :type Boolean) (IsHeadshot :type Boolean))
  (locals (LocalDamage :type "Float (double-precision)"))
  (bind ((`DamageMin_10_8D9A4F434855B342C47F6AAE2C1BAB67` _damagemin) (`DamageMax_12_F236EEB247F9DD17023170B34B70BDCA` _damagemax)) (break `/Game/FPSKM/Blueprints/Structures/ItemData/S_WeaponItemData` (`self.WeaponInfo`)))
  (bind ((`MinDamage_2_B6D3377E4A7D97AF877F9E840A123843` _mindamage) (`MaxDamage_4_0B6602644140C1E0EDA7838609EED9E3` _maxdamage)) (break `/Game/FPSKM/Blueprints/Structures/S_WeaponUpgradeData` (`self.WeaponUpgradeData`)))
  (`|ExecutionSequence`
    (:`then_0`
      ;[1 1 1] Set Damage
      (if (not (`self.IsUseUpgradeData`))
        (set `local.LocalDamage` (`KismetMathLibrary.RandomFloatInRange` _damagemin _damagemax))
        (else
          (set `local.LocalDamage` (`KismetMathLibrary.RandomFloatInRange` _mindamage _maxdamage)))))
    (:`then_1`
      ;[1 1 1] Set Critical Damage
      (if (<= (`KismetMathLibrary.RandomFloatInRange` 0.0 1.0) (`.CriticalRate_115_BB2420C04B4480709ECF4FA6BABAE53B` (break `/Game/FPSKM/Blueprints/Structures/ItemData/S_WeaponItemData` (`self.WeaponInfo`))))
        (set `self.IsCritical` true)
        (set `local.LocalDamage` (* (`local.LocalDamage`) 2.0))
        (else
          (set `self.IsCritical` false)))
      ;[1 1 1] Set headshot damage
      (bind _output_get (set `self.IsHeadshot` (== (`.HitBoneName` (`GameplayStatics.BreakHitResult` (`self.HitInfo`))) "Head")))
      (if _output_get
        (set `local.LocalDamage` (* (`local.LocalDamage`) 2.0)))
      (bind _output_get_2 (set `self.HitDamage` (`local.LocalDamage`)))
      (return _output_get_2 (`self.IsCritical`) (`self.IsHeadshot`)))))

(fn `DamageProcess`
  (params (HitActor :type "Actor Object Reference") (HitInfo :type "HitResult Structure"))
  (bind _hitinfo (`self.HitInfo`))
  (bind (_bblockinghit _binitialoverlap _time _distance _location _impactpoint _normal) (`GameplayStatics.BreakHitResult` _hitinfo))
  (`self.SaveHitInfo` HitActor HitInfo)
  ;[1 1 1] Make Noise
  (`self.MakeNoise` 1.0 (`self.Instigator`) (`self.K2_GetActorLocation`) 200.0)
  ;[1 1 1] Check if projectile can take damage
  (cast `/Game/FPSKM/Blueprints/Interfaces/DamageInterface` (`self.HitActor`))
  (if (!= (`self.HitActor`) (`self.GetInstigator`))
    ;[1 1 1] Take damage
    (message `/Game/FPSKM/Blueprints/Interfaces/DamageInterface.TakeDamage` (`self.HitActor`) (`self.DamageType`) (`self.CalculateDamage`) 0.0 75000.0 (`KismetMathLibrary.Conv_RotatorToVector` (`self.K2_GetActorRotation`)) (`self.HitInfo`) (`self.GetInstigator`) (0.0 0.0 0.0))
    ;[1 1 1] Hit effect
    (`self.HitEffect` _location _normal (`GameplayStatics.GetSurfaceType` _hitinfo))))

(fn `SaveHitInfo`
  (params (HitActor :type "Actor Object Reference") (HitInfo :type "HitResult Structure"))
  (bind (_bblockinghit _binitialoverlap _time _distance _location _impactpoint _normal _impactnormal _physmat _hitactor _hitcomponent _hitbonename) (`GameplayStatics.BreakHitResult` (`local.HitInfo`)))
  (set `self.HitInfo` HitInfo)
  (set `self.HitActor` HitActor)
  (set `self.HitImpactPoint` _impactpoint)
  (set `self.IsHeadshot` (== _hitbonename "Head")))

(fn `SpawnHitEffects`
  (params (IpHitLoc :type "Vector Structure") (IpHitNormal :type "Vector Structure") (IpSurfaceType :type "EPhysicalSurface Enum" :default "SurfaceType_Default"))
  (locals (LocalDecal :type "DecalComponent Object Reference"))
  ;[1 1 1] Spawn Eimmter
  (`GameplayStatics.SpawnEmitterAtLocation` (select `EPhysicalSurface` (`local.IpSurfaceType`) :!type "ParticleSystem Object Reference") (`local.IpHitLoc`) (`KismetMathLibrary.MakeRotator` (+ (.roll (`KismetMathLibrary.Conv_VectorToRotator` (`local.IpHitNormal`))) 90.0) (.pitch (`KismetMathLibrary.Conv_VectorToRotator` (`local.IpHitNormal`))) (.yaw (`KismetMathLibrary.Conv_VectorToRotator` (`local.IpHitNormal`)))) (`self.HitPSScale`))
  ;[1 1 1] Spawn Decal
  (bind _returnvalue (`GameplayStatics.SpawnDecalAtLocation` (select `EPhysicalSurface` (`local.IpSurfaceType`) :`SurfaceType_Default` "/Game/FPSKM/Materials/Decals/M_Decals_DefaultBullet.M_Decals_DefaultBullet" :!type "MaterialInterface Object Reference") (`KismetMathLibrary.MakeVector` 4.0 4.0 4.0) (`local.IpHitLoc`) (`KismetMathLibrary.MakeRotFromX` (`local.IpHitNormal`)) 10.0))
  (bind _output_get (set `local.LocalDecal` _returnvalue))
  (`/Engine/EditorBlueprintResources/StandardMacros.IsValid` _output_get
    (:`Is Valid`
      (`SceneComponent.K2_AddLocalRotation` (`local.LocalDecal`) (`KismetMathLibrary.MakeRotator` (`KismetMathLibrary.RandomFloatInRange` -360.0 360.0) 0.0 180.0) false false)
      (`DecalComponent.SetFadeScreenSize` (`local.LocalDecal`) 1e-05)
      (`DecalComponent.SetFadeOut` (`local.LocalDecal`) 10.0 3.0 false))))

(fn `UserConstructionScript`)