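; Base character class for the FPS, providing shared combat, ammo, movement-state and death logic, with empty hooks for subclasses.
; An anim notify runs a server-only melee sphere trace that damages player characters with Atk and non-character actors with DestructAtk.
; It spawns weapons from database entries, manages per-type ammo and flashes damage materials before restoring cached originals.
; Helpers cover ragdoll impulses from saved hit info, falling death, throw velocity and looping sounds.
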(event `self.ReceiveBeginPlay`
  ;[1 1 1] Event - BeginPlay
  ;;[1 1 1] Set variables
  (`|ExecutionSequence`
    (:`then_0`
      (bind _asbp_fps_game_inst (cast `/Game/FPSKM/Blueprints/Game/BP_FPS_GameInst` (`GameplayStatics.GetGameInstance`)))
      (set `self.GameInstRef` _asbp_fps_game_inst))
    (:`then_1`
      (`self.CollectOriginMat`)
      (`self.CreateDamageMatIfNone`))
    (:`then_2`
      (set `self.OriginCapsuleHalfHeight` (`CapsuleComponent.CapsuleHalfHeight` (`self.CapsuleComponent`))))))

(event `DamageEffectEvent`
  ;[1 1 1] Damage Effect
  (for (_array_element _array_index) (`self.DamagedMaterials`)
    (`PrimitiveComponent.SetMaterial` (`self.Mesh`) _array_index _array_element)
    (`KismetSystemLibrary.Delay` 0.2)
    (for (_array_element_2 _array_index_2) (`self.OriginMaterials`)
      (`PrimitiveComponent.SetMaterial` (`self.Mesh`) _array_index_2 _array_element_2))))

(event `/Game/FPSKM/Blueprints/Interfaces/AnimNotifyInterface.AnimNotify_OnAnim_CheckTraceMeleeAttack`
  ;[1 1 1] Checking Melee Attack Collision
  (`/Engine/EditorBlueprintResources/ActorMacros.Switch Has Authority`
    (:`Authority`
      (bind _outhits (`KismetSystemLibrary.SphereTraceMultiForObjects` (`self.K2_GetActorLocation`) (+ (`self.K2_GetActorLocation`) (* (`self.GetActorForwardVector`) (`self.DefaultMeleeAttackRange`))) 50.0 (`|MakeArray` "ObjectTypeQuery3" "ObjectTypeQuery2" :!type "EObjectTypeQuery Enum")))
      (for _array_element _outhits
        (bind (_bblockinghit _binitialoverlap _time _distance _location _impactpoint _normal _impactnormal _physmat _hitactor _hitcomponent) (`GameplayStatics.BreakHitResult` _array_element))
        (bind _output_get (set `self.MeleeTraceHitActor` _hitactor))
        (bind _asbp_base_char (cast `/Game/FPSKM/Blueprints/Characters/BP_BaseChar` _output_get)
          (:`then`
            (cast `/Game/FPSKM/Blueprints/Characters/Player/BP_FPS_PlayerChar` _asbp_base_char)
            (set `self.ApplyAtk` (`self.Atk`)))
          (:`CastFailed`
            (set `self.ApplyAtk` (`self.DestructAtk`))))
        (bind _returnvalue (`self.K2_GetActorLocation` _hitactor))
        (message `/Game/FPSKM/Blueprints/Interfaces/DamageInterface.TakeDamage` (`self.MeleeTraceHitActor`) "NewEnumerator0" (`self.ApplyAtk`) 0.0 75000.0 _impactnormal (`GameplayStatics.MakeHitResult` false false 0.0 0.0 _returnvalue _returnvalue _normal _impactnormal null _hitactor _hitcomponent) self (0.0 0.0 0.0))))))

(event `StartPlaySound`
  (params (Sound :type "SoundBase Object Reference") (Time :type "Float (double-precision)") (Volume :type "Float (double-precision)" :default 1.0))
  ;[1 1 1] Sound
  ;;[1 1 1] Play Sound repeatedly
  (`self.StopPlaySound`)
  (`self.PlaySoundEvent`)
  (bind _returnvalue (`KismetSystemLibrary.K2_SetTimerDelegate` (delegate `PlaySoundEvent`) Time true))
  (set `self.PlaySoundHandle` _returnvalue))

(event `PlaySoundEvent`
  ;[1 1 1] Sound
  ;;[1 1 1] Play Sound repeatedly
  (`GameplayStatics.PlaySoundAtLocation` (stale `StartPlaySound` Sound) (`self.K2_GetActorLocation`) (struct) 1.0 1.0 0.0 null null null))

(event `StopPlaySound`
  ;[1 1 1] Sound
  ;;[1 1 1] Stop Sound
  (if (`KismetSystemLibrary.K2_IsValidTimerHandle` (`self.PlaySoundHandle`))
    (`KismetSystemLibrary.K2_ClearAndInvalidateTimerHandle` (`self.PlaySoundHandle`))))

(event `AnimBP BeginPlay`
  ;[1 1 1] Animations
)

(event `PlayAnimMontageEvent`
  (params (IpAnimMontage :type "AnimMontage Object Reference") (IpPlayRate :type "Float (double-precision)" :default 1.0))
  ;[1 1 1] Animations
  (`/Engine/EditorBlueprintResources/StandardMacros.IsValid` IpAnimMontage
    (:`Is Valid`
      (`self.PlayAnimMontage` IpAnimMontage IpPlayRate))))

(event `OnDeath`
  ;[1 1 1] Death & Destroyed
)

(event `CommonDeath`
  (params (IpHitDeathKnockbackPower :type "Float (double-precision)") (IpHitNormal :type "Vector Structure") (IpHitLoc :type "Vector Structure") (IpHitBoneName :type Name) (IsSimulatePhysics :type Boolean))
  ;[1 1 1] Death & Destroyed
)

(event `self.ReceiveDestroyed`
  ;[1 1 1] Death & Destroyed
  (`/Engine/EditorBlueprintResources/StandardMacros.IsValid` (`self.CurWeapon`)
    (:`Is Valid`
      (`self.K2_DestroyActor` (`self.CurWeapon`)))))

(event `Event_SetIsMoving`
  (params (IpIsMoving :type Boolean))
  (set `self.IsMoving` IpIsMoving))

(event `CustomCrouch`
  (params (IpIsCrouch :type Boolean)))

(event `SpawnEmitterAtLocationEvent`
  (params (EmitterTemplate :type "ParticleSystem Object Reference") (Location :type "Vector Structure") (Rotation :type "Rotator Structure") (Scale :type "Vector Structure") (bAutoDestroy :type Boolean :default true) (PoolingMethod :type "EPSCPoolMethod Enum" :default "None"))
  (`GameplayStatics.SpawnEmitterAtLocation` EmitterTemplate Location Rotation Scale bAutoDestroy PoolingMethod))

(fn `AddAmmo`
  (params (IpAmmo :type Integer))
  (returns (Result :type Boolean))
  (bind _ipammo (`local.IpAmmo`))
  (`self.AddToCharInvenAmmo` "NewEnumerator0" _ipammo)
  (`self.AddToCharInvenAmmo` "NewEnumerator1" _ipammo)
  (`self.AddToCharInvenAmmo` "NewEnumerator2" _ipammo)
  (return true))

(fn `AddMultiplyMoveSpeed`
  (params (AddValue :type "Float (double-precision)"))
  (set `self.MultiplyMoveSpeed` (+ (`self.MultiplyMoveSpeed`) AddValue)))

(fn `AddToCharInvenAmmo`
  (params (IpAmmoType :type "/Game/FPSKM/Blueprints/Enums/E_A_AmmoType Enum" :default "NewEnumerator0") (IpAddCount :type Integer))
  (`self.SetCharInvenAmmo` IpAmmoType (+ (`self.GetCharInvenAmmo` IpAmmoType) IpAddCount)))

(fn `CalculateBestThrowVel`
  (params (StartLoc :type "Vector Structure") (TargetLoc :type "Vector Structure") (Time :type "Float (double-precision)"))
  (returns (Result :type "Vector Structure"))
  (locals (TargetDisVector :type "Vector Structure") (TargetDisXYVector :type "Vector Structure") (TargetDisZ :type "Float (double-precision)") (TargetDisXYLength :type "Float (double-precision)") (VelZ :type "Float (double-precision)") (VelXY :type "Float (double-precision)") (ResultVel :type "Vector Structure") (TimeToTarget :type "Float (double-precision)"))
  (bind _charactermovement (`self.CharacterMovement`))
  (set `local.TimeToTarget` Time)
  (bind _output_get (set `local.TargetDisVector` (- TargetLoc StartLoc)))
  (bind _output_get_2 (set `local.TargetDisXYVector` _output_get))
  (set `local.TargetDisXYVector` (`KismetMathLibrary.MakeVector` (.x _output_get_2) (.y _output_get_2)))
  (set `local.TargetDisZ` (.z (`local.TargetDisVector`)))
  (set `local.TargetDisXYLength` (`KismetMathLibrary.VSize` (`local.TargetDisXYVector`)))
  (set `local.VelZ` (+ (/ (`local.TargetDisZ`) (`local.TimeToTarget`)) (* 0.5 (/ (`KismetMathLibrary.Abs` (`MovementComponent.GetGravityZ` _charactermovement)) (`CharacterMovementComponent.GravityScale` _charactermovement)) (`local.TimeToTarget`))))
  (set `local.VelXY` (/ (`local.TargetDisXYLength`) (`local.TimeToTarget`)))
  (bind _output_get_3 (set `local.ResultVel` (* (`KismetMathLibrary.Normal` (`local.TargetDisXYVector`)) (`local.VelXY`))))
  (return (`KismetMathLibrary.MakeVector` (.x _output_get_3) (.y _output_get_3) (`local.VelZ`))))

(fn `CanCrouch_State`
  (returns (Result :type Boolean))
  (return (and (not (`self.IsDash`)) (not (`self.IsDeath`)) (not (`NavMovementComponent.IsFalling` (`self.CharacterMovement`))))))

(fn `CanFire_State`
  (returns (Result :type Boolean))
  (return false))

(fn `CanJump_State`
  (returns (Result :type Boolean))
  (return (and (not (`self.IsDash`)) (not (`self.IsDeath`)))))

(fn `CanThrowGrenade_State`
  (returns (Result :type Boolean))
  (return false))

(fn `CollectOriginMat`
  (`KismetArrayLibrary.Array_Clear` (`self.OriginMaterials`))
  (`/Engine/EditorBlueprintResources/StandardMacros.IsValid` (`self.Mesh`)
    (:`Is Valid`
      (for _array_element (`MeshComponent.GetMaterials` (`self.Mesh`))
        (`KismetArrayLibrary.Array_Add` (`self.OriginMaterials`) _array_element)))))

(fn `CreateDamageMatIfNone`
  (if (== (`KismetArrayLibrary.Array_Length` (`self.DamagedMaterials`)) 0)
    (for _ (`self.OriginMaterials`)
      (`KismetArrayLibrary.Array_Add` (`self.DamagedMaterials`) (`self.DefaultDamagedMaterials`)))))

(fn `CreateWeapon`
  (params (IpWeaponDBNo :type Integer))
  (returns (Result :type "/Game/FPSKM/Blueprints/Weapons/BP_BaseWeapon Object Reference"))
  (locals (LocalCreatedWeapon :type "/Game/FPSKM/Blueprints/Weapons/BP_BaseWeapon Object Reference") (LocalWeaponDBNo :type Integer) (LocalWeaponInfo_0 :type "/Game/FPSKM/Blueprints/Structures/ItemData/S_WeaponItemData Structure"))
  (bind (_isfind _weapondata) (`/Game/FPSKM/Blueprints/Game/BPFL_FPS.FindWeaponDBData` (`local.IpWeaponDBNo`)))
  ;[1 1 1] Find Weapon Data
  (if _isfind
    ;[1 1 1] Get Weapon Blueprint Class From WeaponData
    (bind _output_get (set `local.LocalWeaponInfo_0` _weapondata))
    ;[1 1 1] Spawn a New Weapon
    (bind _returnvalue (`|SpawnActorFromClass` (`.WeaponClassBP_104_3C89EB8E4D8FCE183ED0EF8F6FFF0534` (break `/Game/FPSKM/Blueprints/Structures/ItemData/S_WeaponItemData` _output_get)) (`self.GetTransform`) "Undefined" "OverrideRootScale" self (`local.LocalWeaponInfo_0`) (`self.TeamNumber`) self))
    (set `local.LocalCreatedWeapon` _returnvalue)
    (return (`local.LocalCreatedWeapon`))
    (else
      (return null))))

(fn `DeathEffects`
  (`GameplayStatics.SpawnEmitterAtLocation` "/Game/FPSKM/Particles/PS_BloodHit_Big.PS_BloodHit_Big" (.location (`SceneComponent.GetSocketTransform` (`self.Mesh`) (`self.HitBoneName`) "RTS_World")) (.rotation (`SceneComponent.GetSocketTransform` (`self.Mesh`) (`self.HitBoneName`) "RTS_World")) (1.4 1.4 1.4)))

(fn `GetArmAnimInst`
  (returns (AnimInst :type "AnimInstance Object Reference"))
  (return null))

(fn `GetArmSkMesh`
  (returns (Result :type "SkeletalMeshComponent Object Reference"))
  (return null))

(fn `GetCharInvenAmmo`
  (params (IpAmmoType :type "/Game/FPSKM/Blueprints/Enums/E_A_AmmoType Enum (by ref)" :default "NewEnumerator0"))
  (returns (Result :type Integer))
  (bind (_lightammo _mediumammo _heavyammo) (break `/Game/FPSKM/Blueprints/Structures/S_CharInvenInfo` (`self.CharInvenInfo`)))
  (switch `/Game/FPSKM/Blueprints/Enums/E_A_AmmoType` IpAmmoType
    (:`NewEnumerator0`
      (return _lightammo))
    (:`NewEnumerator1`
      (return _mediumammo))
    (:`NewEnumerator2`
      (return _heavyammo))))

(fn `GetDeltaAngle`
  (params (TargetActor1 :type "Actor Object Reference"))
  (returns (ResultYaw1 :type "Float (double-precision)"))
  (return (.yaw (`KismetMathLibrary.NormalizedDeltaRotator` (`KismetMathLibrary.Conv_VectorToRotator` (- (`self.K2_GetActorLocation` TargetActor1) (`self.K2_GetActorLocation`))) (`self.K2_GetActorRotation`)))))

(fn `GetFireRate`
  (returns (FireRate :type "Float (double-precision)"))
  (`|ExecutionSequence`
    (:`then_0`
      (bind _asbp_fps_player_state (cast `/Game/FPSKM/Blueprints/Game/BP_FPS_PlayerState` (`self.PlayerState`)))
      (bind (_isfind _result) (`/Game/FPSKM/Blueprints/Game/BP_FPS_PlayerState.FindWeaponUpgradeData` _asbp_fps_player_state (`.No_2_B1B1004445E04EA72D06E797626700C8` (break `/Game/FPSKM/Blueprints/Structures/ItemData/S_WeaponItemData` (`self.CurWeaponData`)))))
      (if _isfind
        (return (`.FireRate_6_8361091043D22391DDFCC0ACCC7E8FD4` (break `/Game/FPSKM/Blueprints/Structures/S_WeaponUpgradeData` _result)))))
    (:`then_1`
      (return (`.FireRate_31_8636439E4E4C4D13ECD3958D1711D44D` (break `/Game/FPSKM/Blueprints/Structures/ItemData/S_WeaponItemData` (`self.CurWeaponData`)))))))

(fn `ResetHp`
  (set `self.Hp` (`self.MaxHp`)))

(fn `SaveHitInfo`
  (params (HitDamage :type "Float (double-precision)") (HitDefaultKnockbackPower :type "Float (double-precision)") (HitDeathKnockbackPower :type "Float (double-precision)") (HitNormal :type "Vector Structure") (HitInfo :type "HitResult Structure") (HitSpreadCenterLoc :type "Vector Structure") (HitDamageCauser :type "Actor Object Reference"))
  (set `self.HitDamage` HitDamage)
  (set `self.HitDefaultKnockbackPower` HitDefaultKnockbackPower)
  (set `self.HitDeathKnockbackPower` (* HitDeathKnockbackPower 0.36))
  (set `self.HitNormal` HitNormal)
  (set `self.HitSpreadCenterLoc` HitSpreadCenterLoc)
  (bind _output_get (set `self.HitHitInfo` HitInfo))
  (set `self.HitDamageCauser` HitDamageCauser)
  (bind (_bblockinghit _binitialoverlap _time _distance _location _impactpoint _normal _impactnormal _physmat _hitactor _hitcomponent _hitbonename) (`GameplayStatics.BreakHitResult` _output_get))
  (set `self.HitLocation` _location)
  (set `self.HitBoneName` _hitbonename))

(fn `SetCharInvenAmmo`
  (params (IpAmmoType :type "/Game/FPSKM/Blueprints/Enums/E_A_AmmoType Enum" :default "NewEnumerator0") (Ammo :type Integer))
  (switch `/Game/FPSKM/Blueprints/Enums/E_A_AmmoType` IpAmmoType
    (:`NewEnumerator0`
      (setmembers `/Game/FPSKM/Blueprints/Structures/S_CharInvenInfo` :`StructRef` (`self.CharInvenInfo`) :`LightAmmo` Ammo))
    (:`NewEnumerator1`
      (setmembers `/Game/FPSKM/Blueprints/Structures/S_CharInvenInfo` :`StructRef` (`self.CharInvenInfo`) :`MediumAmmo` Ammo))
    (:`NewEnumerator2`
      (setmembers `/Game/FPSKM/Blueprints/Structures/S_CharInvenInfo` :`StructRef` (`self.CharInvenInfo`) :`HeavyAmmo` Ammo))))

(fn `SetCharMaxWalkSpeed`
  (params (IpMaxWalkSpeed :type "Float (double-precision)"))
  (set `CharacterMovementComponent.MaxWalkSpeed` IpMaxWalkSpeed (`self.CharacterMovement`)))

(fn `SimulateDeathPhysics`
  (`PrimitiveComponent.SetSimulatePhysics` (`self.Mesh`) true)
  (`PrimitiveComponent.AddImpulse` (`self.Mesh`) (* (`self.HitNormal`) (* (`self.HitDeathKnockbackPower`) (`KismetMathLibrary.RandomFloatInRange` 0.5 1.0))) (`self.HitBoneName`) false))

(fn `Update_FallingDeath`
  (bind (_returnvalue_x _returnvalue_y _returnvalue_z) (`KismetMathLibrary.BreakVector` (- (`self.PrevLoc`) (`self.K2_GetActorLocation`))))
  ;[1 1 1] Check if character is falling
  (if (`NavMovementComponent.IsFalling` (`self.CharacterMovement`))
    ;[1 1 1] Calculate falling distance if character is falling
    (bind _output_get (set `self.FallingDistance` (+ _returnvalue_z (`self.FallingDistance`))))
    ;[1 1 1] Check if falling distance is more than death falling distance
    (if (and (>= _output_get (`self.DeathFallingDistance`)) (not (`self.IsDeath`)))
      (`ActorComponent.SetActive` (`self.CharacterMovement`) false false)
      (set `self.DeathToDisappearWaitTime` 0.0)
      ;[1 1 1] Call OnDeath event to destroy a character falling
      (`self.OnDeath`))))

(fn `UpdateStandTargetRot`
  (params (IpTargetActor :type "Actor Object Reference") (IpDeltaTime :type "Float (double-precision)"))
  (`/Engine/EditorBlueprintResources/StandardMacros.IsValid` IpTargetActor
    (:`Is Valid`
      (if (`self.IsStandTargetRotating`)
        (`self.K2_SetActorRotation` (`KismetMathLibrary.RInterpTo` (`self.K2_GetActorRotation`) (`KismetMathLibrary.Conv_VectorToRotator` (`KismetMathLibrary.MakeVector` (.x (- (`self.K2_GetActorLocation` (`local.IpTargetActor`)) (`self.K2_GetActorLocation`))) (.y (- (`self.K2_GetActorLocation` (`local.IpTargetActor`)) (`self.K2_GetActorLocation`))))) (`local.IpDeltaTime`) 5.0))))))

(fn `UseCharInvenAmmo`
  (params (IpAmmoType :type "/Game/FPSKM/Blueprints/Enums/E_A_AmmoType Enum" :default "NewEnumerator0") (IpUseCount :type Integer))
  (returns (ResultUseCount :type Integer))
  (locals (LocalLeftAmmo :type Integer :default 0))
  (bind _result (`self.GetCharInvenAmmo` (`local.IpAmmoType`)))
  (bind _returnvalue (- _result (`local.IpUseCount`)))
  (set `local.LocalLeftAmmo` _result)
  (if (< _returnvalue 0)
    (`self.SetCharInvenAmmo` (`local.IpAmmoType`))
    (return (`local.LocalLeftAmmo`))
    (else
      (`self.SetCharInvenAmmo` (`local.IpAmmoType`) _returnvalue)
      (return (`local.IpUseCount`)))))

(fn `UserConstructionScript`)