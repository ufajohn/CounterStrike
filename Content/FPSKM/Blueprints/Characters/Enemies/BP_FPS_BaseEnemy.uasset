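; Base FPS enemy character that detects players and drives its AI through an enum state mirrored to the Blackboard.
; On authority, Tick seeds the Blackboard once with state, patrol points, speeds and ranges.
; PawnSensing sight and noise feed SetToCombat, which sets the target and enters follow from certain states.
; Target death, disappearance and respawn events update target or state; OnSeeTargetHero is an empty hook, and UpdateTargetRot offers smoothed yaw tracking.
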(event `OnSeeTargetHero`
  (params (IpTargetHero :type "/Game/FPSKM/Blueprints/Characters/Player/BP_FPS_PlayerChar Object Reference")))

(event `self.AnimBP BeginPlay`
  (`self.SaveInfoToBlackboard`))

(event `FollowToHero`
  (bind _outactors (`GameplayStatics.GetAllActorsOfClass` "/Game/FPSKM/Blueprints/Characters/Player/BP_FPS_PlayerChar.BP_FPS_PlayerChar_C"))
  (if (> (`KismetArrayLibrary.Array_Length` _outactors) 0)
    (`self.ChangeState` "NewEnumerator7")
    (set `self.TargetHero` (`|GetArrayItem` _outactors))
    (`self.ApplyTargetHeroToBlackboard`)
    (`self.ApplyCurStateToBlackboard`)))

(event `self.ReceiveBeginPlay`
  ;[1 1 1] Event - BeginPlay
  (`parent.ReceiveBeginPlay`))

(event `self.ReceiveTick`
  (params (DeltaSeconds :type "Float (single-precision)"))
  ;[1 1 1] Event - Tick
  (`/Engine/EditorBlueprintResources/ActorMacros.Switch Has Authority`
    (:`Authority`
      ;;[1 1 1] Initializing Own Blackboard
      (if (not (`self.IsInitBlackboard`))
        (`self.SaveInfoToBlackboard`)))))

(event `/Game/FPSKM/Blueprints/Interfaces/DamageInterface.OnCharDeath`
  (params (IpChar :type "/Game/FPSKM/Blueprints/Characters/BP_BaseChar Object Reference") (IpCHitInfo :type "/Game/FPSKM/Blueprints/Structures/S_C_HitInfo Structure"))
  ;[1 1 1] Event - OnCharDeath
  (`/Engine/EditorBlueprintResources/ActorMacros.Switch Has Authority`
    (:`Authority`
      (if (== IpChar (`self.TargetHero`))
        (set `self.TargetHero` null)
        (`self.ApplyTargetHeroToBlackboard`)))))

(event `/Game/FPSKM/Blueprints/Interfaces/DamageInterface.OnCharDisappear`
  (params (IpChar :type "/Game/FPSKM/Blueprints/Characters/BP_BaseChar Object Reference"))
  ;[1 1 1] Event - OnCharDisappear
  (`/Engine/EditorBlueprintResources/ActorMacros.Switch Has Authority`
    (:`Authority`
      (if (== IpChar (`self.TargetHero`))
        (if (not (`self.IsCurState` "NewEnumerator3"))
          (`self.ChangeState` "NewEnumerator8")
          (`self.ApplyCurStateToBlackboard`))))))

(event `/Game/FPSKM/Blueprints/Interfaces/DamageInterface.OnRespawnPlayerCharacter`
  (params (IpHeroChar :type "/Game/FPSKM/Blueprints/Characters/Player/BP_FPS_PlayerChar Object Reference"))
  ;[1 1 1] Event - OnRespawnPlayer
  (`/Engine/EditorBlueprintResources/ActorMacros.Switch Has Authority`
    (:`Authority`
      (`self.ChangeState` "NewEnumerator8")
      (`self.ApplyCurStateToBlackboard`))))

(event `self.PawnSensing.OnSeePawn`
  (params (Pawn :type "Pawn Object Reference"))
  ;[1 1 1] PawnSesing - OnSeePawn, OnHearNoise
  (`/Engine/EditorBlueprintResources/ActorMacros.Switch Has Authority`
    (:`Authority`
      (bind _asbp_fps_player_char (cast `/Game/FPSKM/Blueprints/Characters/Player/BP_FPS_PlayerChar` Pawn))
      (`self.SetToCombat` _asbp_fps_player_char))))

(event `self.PawnSensing.OnHearNoise`
  (params (Instigator :type "Pawn Object Reference") (Location :type "Vector Structure (by ref)") (Volume :type "Float (single-precision)"))
  ;[1 1 1] PawnSesing - OnSeePawn, OnHearNoise
  (`/Engine/EditorBlueprintResources/ActorMacros.Switch Has Authority`
    (:`Authority`
      (bind _asbp_fps_player_char (cast `/Game/FPSKM/Blueprints/Characters/Player/BP_FPS_PlayerChar` Instigator))
      (`self.SetToCombat` _asbp_fps_player_char))))

(fn `ApplyCurStateToBlackboard`
  (bind _returnvalue (`AIBlueprintHelperLibrary.GetBlackboard` null))
  (`/Engine/EditorBlueprintResources/StandardMacros.IsValid` _returnvalue
    (:`Is Valid`
      (`BlackboardComponent.SetValueAsEnum` _returnvalue "EnemyState" (`self.CurState`)))))

(fn `ApplyTargetHeroToBlackboard`
  (`/Engine/EditorBlueprintResources/StandardMacros.IsValid` (`AIBlueprintHelperLibrary.GetBlackboard` null)
    (:`Is Valid`
      (`BlackboardComponent.SetValueAsObject` (`AIBlueprintHelperLibrary.GetBlackboard` null) "TargetActor" (`self.TargetHero`)))))

(fn `ChangeState`
  (params (State :type "/Game/FPSKM/Blueprints/Enums/E_EnemyState Enum" :default "NewEnumerator10"))
  (set `self.PrevState` (`self.CurState`))
  (set `self.CurState` State))

(fn `IsCurState`
  (params (State :type "/Game/FPSKM/Blueprints/Enums/E_EnemyState Enum" :default "NewEnumerator10"))
  (returns (Result :type Boolean))
  (return (`|EnumEquality` State (`self.CurState`))))

(fn `SaveInfoToBlackboard`
  (bind _returnvalue (`AIBlueprintHelperLibrary.GetBlackboard` null))
  (`/Engine/EditorBlueprintResources/StandardMacros.IsValid` (`AIBlueprintHelperLibrary.GetBlackboard` null)
    (:`Is Valid`
      (`self.ApplyCurStateToBlackboard`)
      ;[1 1 1] Set Blackboard Variables - Patrol2Loc, Patrol2Loc, PatrolWalkSpeed, HeroFollowWalkSpeed, HeroApprochDis, MaxAttackRange
      (`BlackboardComponent.SetValueAsVector` _returnvalue "Patrol1Loc" (`SceneComponent.K2_GetComponentLocation` (`self.Patrol_Waypoint1`)))
      (`BlackboardComponent.SetValueAsVector` _returnvalue "Patrol2Loc" (`SceneComponent.K2_GetComponentLocation` (`self.Patrol_Waypoint2`)))
      (`BlackboardComponent.SetValueAsFloat` _returnvalue "PatrolWalkSpeed" (`self.PatrolWalkSpeed`))
      (`BlackboardComponent.SetValueAsFloat` _returnvalue "HeroFollowWalkSpeed" (`self.HeroFollowWalkSpeed`))
      (`BlackboardComponent.SetValueAsFloat` _returnvalue "HeroApprochDis" (`self.HeroApprochDis`))
      (`BlackboardComponent.SetValueAsFloat` _returnvalue "MaxAttackRange" (`self.MaxAttackRange`))
      (set `self.IsInitBlackboard` true))))

(fn `SetToCombat`
  (params (IpTargetHero :type "/Game/FPSKM/Blueprints/Characters/Player/BP_FPS_PlayerChar Object Reference"))
  (returns (IsChangeCombat :type Boolean))
  (`/Engine/EditorBlueprintResources/StandardMacros.IsValid` IpTargetHero
    (:`Is Valid`
      (`|ExecutionSequence`
        (:`then_0`
          ;[1 1 1] If TargetHero is valid, set TargetHero
          (if (not (`KismetSystemLibrary.IsValid` (`self.TargetHero`)))
            (`self.OnSeeTargetHero` (`local.IpTargetHero`)))
          (set `self.TargetHero` (`local.IpTargetHero`))
          (`BlackboardComponent.SetValueAsObject` (`AIBlueprintHelperLibrary.GetBlackboard` null) "TargetActor" (`self.TargetHero`)))
        (:`then_1`
          ;[1 1 1] Check if Character follow
          (if (or (`self.IsCurState` "NewEnumerator0") (`self.IsCurState` "NewEnumerator8") (`self.IsCurState` "NewEnumerator10") (`self.IsCurState` "NewEnumerator13"))
            (if (`KismetSystemLibrary.IsValid` (`self.TargetHero`))
              ;[1 1 1] Follow hero
              (`self.ChangeState` "NewEnumerator7")
              (`self.ApplyCurStateToBlackboard`)
              (`/Engine/EditorBlueprintResources/StandardMacros.IsValid` (`AIBlueprintHelperLibrary.GetBlackboard` self)
                (:`Is Valid`
                  (return true))
                (:`Is Not Valid`
                  (return false))))
            (else
              (return false))))))
    (:`Is Not Valid`
      (return false))))

(fn `UpdateTargetRot`
  (if (`self.IsUpdateTargetRot`)
    (`/Engine/EditorBlueprintResources/StandardMacros.IsValid` (`self.TargetHero`)
      (:`Is Valid`
        (`self.K2_SetActorRotation` (`KismetMathLibrary.RInterpTo` (`self.K2_GetActorRotation`) (`KismetMathLibrary.Conv_VectorToRotator` (`KismetMathLibrary.MakeVector` (.x (- (`self.K2_GetActorLocation` (`self.TargetHero`)) (`self.K2_GetActorLocation`))) (.y (- (`self.K2_GetActorLocation` (`self.TargetHero`)) (`self.K2_GetActorLocation`))))) (`GameplayStatics.GetWorldDeltaSeconds`) (`self.TargetRotateSpeed`)))))))

(fn `UserConstructionScript`
  (`parent.UserConstructionScript`))