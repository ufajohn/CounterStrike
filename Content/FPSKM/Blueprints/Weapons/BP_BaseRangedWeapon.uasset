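; Base ranged weapon Blueprint for an FPS, handling firing, ammo, hit damage and fire/reload animation calls.
; Fire takes a barrel socket position, adds random weapon and character spread, then either line traces or launches a projectile.
; Player-state upgrade data, when found, overrides clip size and damage stats and passes to projectiles.
; Trace hits make noise, then deal bone-aware damage with floating text through DamageInterface, or spawn surface-based effects.
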(event `self.ReceiveBeginPlay`
  (`parent.ReceiveBeginPlay`))

(event `self.ReceiveTick`
  (params (DeltaSeconds :type "Float (single-precision)")))

(event `self.Fire`
  (params (IpFireTarget :type "Vector Structure") (IpBarrelIndex :type Integer) (IpCharSpreadHalfAngleY :type "Float (single-precision)") (IpCharSpreadHalfAngleZ :type "Float (single-precision)"))
  (bind _returnvalue (`self.GetInstigator`))
  (bind ((`FireSpreadHalfAngleY_43_9606943941B0AAE89145F3884E65A655` _firespreadhalfangley) (`FireSpreadHalfAngleZ_45_8BE99D6A4D17EF3B13FDFBB1120FAB24` _firespreadhalfanglez)) (break `/Game/FPSKM/Blueprints/Structures/ItemData/S_WeaponItemData` (`self.WeaponData`)))
  (bind _location (.location (`self.FireTrm`)))
  (bind _returnvalue_2 (+ _firespreadhalfangley (`self.CharSpreadHalfAngleY`)))
  (bind _returnvalue_3 (+ _firespreadhalfanglez (`self.CharSpreadHalfAngleZ`)))
  (set `self.TargetLoc` IpFireTarget)
  (set `self.CharSpreadHalfAngleY` IpCharSpreadHalfAngleY)
  (set `self.CharSpreadHalfAngleZ` IpCharSpreadHalfAngleZ)
  (set `self.FireStartLoc` (`self.GetFireLoc` IpBarrelIndex))
  (set `self.Ammo` (- (`self.Ammo`) 1))
  (set `self.FireRot` (`KismetMathLibrary.Conv_VectorToRotator` (`KismetMathLibrary.Normal` (- (`self.TargetLoc`) (`self.FireStartLoc`)))))
  (`|ExecutionSequence`
    (:`then_0`
      (set `self.IsUseUpgradeData` false)
      (`/Engine/EditorBlueprintResources/StandardMacros.IsValid` _returnvalue
        (:`Is Valid`
          (bind _asbp_fps_player_state (cast `/Game/FPSKM/Blueprints/Game/BP_FPS_PlayerState` (`Pawn.PlayerState` _returnvalue)))
          (bind (_isfind _result) (`/Game/FPSKM/Blueprints/Game/BP_FPS_PlayerState.FindWeaponUpgradeData` _asbp_fps_player_state (`.No_2_B1B1004445E04EA72D06E797626700C8` (break `/Game/FPSKM/Blueprints/Structures/ItemData/S_WeaponItemData` (`self.WeaponData`)))))
          (set `self.IsUseUpgradeData` _isfind)
          (set `self.WeaponUpgradeData` _result))))
    (:`then_1`
      (set `self.FireTrm` (`KismetMathLibrary.MakeTransform` (`self.FireStartLoc`) (`KismetMathLibrary.MakeRotator` (.roll (`self.FireRot`)) (+ (.pitch (`self.FireRot`)) (`KismetMathLibrary.RandomFloatInRange` (* _returnvalue_2 -1.0) _returnvalue_2)) (+ (.yaw (`self.FireRot`)) (`KismetMathLibrary.RandomFloatInRange` (* _returnvalue_3 -1.0) _returnvalue_3))))))
    (:`then_2`
      (if (`self.IsUseLinecast`)
        (bind (_outhit _returnvalue_4) (`KismetSystemLibrary.LineTraceSingle` _location (+ _location (* (`KismetMathLibrary.GetForwardVector` (.rotation (`self.FireTrm`))) 10000.0)) "TraceTypeQuery1" false (`|MakeArray` (`self.GetOwner`))))
        (if _returnvalue_4
          (`self.DamageProcess` (`.HitActor` (`GameplayStatics.BreakHitResult` _outhit)) _outhit))
        (else
          (bind _returnvalue_5 (`|SpawnActorFromClass` (`.ProjectileClass_103_2FA73F944BB2A8758E4563B286BB50EC` (break `/Game/FPSKM/Blueprints/Structures/ItemData/S_WeaponItemData` (`self.WeaponData`))) (`self.FireTrm`) "AlwaysSpawn" "OverrideRootScale" (`self.GetOwner`) (`self.TeamNumber`) (`self.IsUseUpgradeData`) (`self.WeaponUpgradeData`) (`self.GetInstigator`)))
          (`/Game/FPSKM/Blueprints/Projectiles/BP_BaseProjectile.Launch` _returnvalue_5 (`self.WeaponData`)))))))

(event `self.FireEffect`
  (params (BarrelIndex :type Integer)))

(event `self.Show`
  (params (Visible :type Boolean))
  (`parent.Show` Visible))

(event `self.PlayFireAnim`
  (message `/Game/FPSKM/Blueprints/Interfaces/WeaponAnimInterface.PlayFireAnim` (`SkeletalMeshComponent.GetAnimInstance` (`self.SkeletalMesh`))))

(event `self.Reload`
  (message `/Game/FPSKM/Blueprints/Interfaces/WeaponAnimInterface.PlayReloadAnim` (`SkeletalMeshComponent.GetAnimInstance` (`self.SkeletalMesh`))))

(event `self.HitEffect`
  (params (IpLoc :type "Vector Structure") (IpNormal :type "Vector Structure") (SurfaceType :type "EPhysicalSurface Enum" :default "SurfaceType_Default"))
  (`self.SpawnHitEffect` IpLoc IpNormal SurfaceType))

(fn `AddAmmo`
  (params (AddValue :type Integer))
  (returns (Result :type Boolean))
  (bind _returnvalue (+ (`local.AddValue`) (`self.Ammo`)))
  (`|ExecutionSequence`
    (:`then_0`
      (if (> _returnvalue (`self.GetMaxAmmo`))
        (set `self.Ammo` (`self.GetMaxAmmo`))
        (else
          (set `self.Ammo` _returnvalue))))
    (:`then_1`
      (return true))))

(fn `DamageProcess`
  (params (IpHitActor :type "Actor Object Reference") (IpHitResult :type "HitResult Structure"))
  (returns (Result :type Boolean) (Damage :type "Float (double-precision)"))
  (locals (LocalDamage :type "Float (double-precision)" :default 0.0))
  (bind _iphitresult (`local.IpHitResult`))
  (bind ((`DamageMin_10_8D9A4F434855B342C47F6AAE2C1BAB67` _damagemin) (`DamageMax_12_F236EEB247F9DD17023170B34B70BDCA` _damagemax) (`CriticalRate_115_BB2420C04B4480709ECF4FA6BABAE53B` _criticalrate)) (break `/Game/FPSKM/Blueprints/Structures/ItemData/S_WeaponItemData` (`self.WeaponData`)))
  (bind ((`MinDamage_2_B6D3377E4A7D97AF877F9E840A123843` _mindamage) (`MaxDamage_4_0B6602644140C1E0EDA7838609EED9E3` _maxdamage) (`CriticalRate_17_C55047BF4A5EBBB771D6898B13E54497` _criticalrate_2)) (break `/Game/FPSKM/Blueprints/Structures/S_WeaponUpgradeData` (`self.WeaponUpgradeData`)))
  (bind (_bblockinghit _binitialoverlap _time _distance _location _impactpoint _normal) (`GameplayStatics.BreakHitResult` _iphitresult))
  (`|ExecutionSequence`
    (:`then_0`
      ;[1 1 1] Make Noise
      (`self.MakeNoise` 1.0 (`self.Instigator`) (`self.K2_GetActorLocation`) 200.0)
      ;[1 1 1] Check if can take damage
      (cast `/Game/FPSKM/Blueprints/Interfaces/DamageInterface` (`local.IpHitActor`)
        (:`then`
          (if (!= (`local.IpHitActor`) (`self.GetInstigator`))
            ;[1 1 1] Check if use upgrade data and set damage
            (if (`self.IsUseUpgradeData`)
              (set `local.LocalDamage` (`self.CalculateDamage` _mindamage _maxdamage _criticalrate_2 (`.HitBoneName_19_C518A751499D626195D0C4906C2979B0` (break `/Game/FPSKM/Blueprints/Structures/S_C_HitInfo` (`/Game/FPSKM/Blueprints/Game/BPFL_FPS.ToCHitInfo` (`local.IpHitResult`))))))
              (else
                (set `local.LocalDamage` (`self.CalculateDamage` _damagemin _damagemax _criticalrate (`.HitBoneName_19_C518A751499D626195D0C4906C2979B0` (break `/Game/FPSKM/Blueprints/Structures/S_C_HitInfo` (`/Game/FPSKM/Blueprints/Game/BPFL_FPS.ToCHitInfo` (`local.IpHitResult`))))))))
            ;[1 1 1] Take damage
            (message `/Game/FPSKM/Blueprints/Interfaces/DamageInterface.TakeDamage` (`local.IpHitActor`) "NewEnumerator0" (`local.LocalDamage`) 0.0 75000.0 (`KismetMathLibrary.Conv_RotatorToVector` (`self.K2_GetActorRotation`)) (`local.IpHitResult`) (`self.GetInstigator`) (0.0 0.0 0.0))
            ;[1 1 1] Damage Text
            (bind _returnvalue (`|CreateWidget` "/Game/FPSKM/Blueprints/Widgets/Widget_DamageText.Widget_DamageText_C"))
            (`UserWidget.AddToViewport` _returnvalue 0)
            (`/Game/FPSKM/Blueprints/Widgets/Widget_DamageText.Launch` _returnvalue (`.Location` (`GameplayStatics.BreakHitResult` (`local.IpHitResult`))) 1.0 (`local.LocalDamage`))
            (return true (`local.LocalDamage`))))
        (:`CastFailed`
          ;[1 1 1] Hit effect
          (`self.HitEffect` _location _normal (`GameplayStatics.GetSurfaceType` _iphitresult)))))
    (:`then_1`
      (return false 0.0))))

(fn `GetFireLoc`
  (params (IpBarrelIndex :type Integer))
  (returns (FireLoc :type "Vector Structure"))
  (locals (LocalFireLoc :type "Vector Structure") (LocalSocketName :type Name))
  (return (.location (`self.GetFireTrm` IpBarrelIndex))))

(fn `GetFireTrm`
  (params (BarrelIndex :type Integer))
  (returns (FireLoc :type "Transform Structure"))
  (locals (LocalFireLoc :type "Vector Structure") (LocalSocketName :type Name) (LocalFireTrm :type "Transform Structure"))
  (set `local.LocalSocketName` (`KismetStringLibrary.Conv_StringToName` (`|GetArrayItem` (`.BarrelSocketNameAry_108_A8E4A2E8473D1AC44DFFF3951EB5A585` (break `/Game/FPSKM/Blueprints/Structures/ItemData/S_WeaponItemData` (`self.WeaponData`))) BarrelIndex)))
  ;[1 1 1] Check use static mesh
  (`/Engine/EditorBlueprintResources/StandardMacros.IsValid` (`StaticMeshComponent.StaticMesh` (`self.StaticMesh`))
    (:`Is Valid`
      (return (`SceneComponent.GetSocketTransform` (`self.StaticMesh`) (`local.LocalSocketName`) "RTS_World")))
    (:`Is Not Valid`
      ;[1 1 1] Check use skeleton mesh
      (`/Engine/EditorBlueprintResources/StandardMacros.IsValid` (`SkinnedMeshComponent.SkeletalMesh` (`self.SkeletalMesh`))
        (:`Is Valid`
          (return (`SceneComponent.GetSocketTransform` (`self.SkeletalMesh`) (`local.LocalSocketName`) "RTS_World")))
        (:`Is Not Valid`
          (bind _asbp_base_char (cast `/Game/FPSKM/Blueprints/Characters/BP_BaseChar` (`self.GetOwner`)))
          (return (`SceneComponent.GetSocketTransform` (`Character.Mesh` _asbp_base_char) (`local.LocalSocketName`) "RTS_World")))))))

(fn `GetMaxAmmo`
  (returns (MaxAmmo :type Integer))
  (locals (LocalIsUseUpgradeData :type Boolean) (LocalWeaponUpgradeData :type "/Game/FPSKM/Blueprints/Structures/S_WeaponUpgradeData Structure"))
  (bind _returnvalue (`self.GetInstigator`))
  (`|ExecutionSequence`
    (:`then_0`
      ;[1 1 1] Check use upgrade data
      (if (> (`KismetArrayLibrary.Array_Length` (`.UpgradeAry_147_13D23180428AC3EB5D4D4DBD9BD4A56A` (break `/Game/FPSKM/Blueprints/Structures/ItemData/S_WeaponItemData` (`self.WeaponData`)))) 0)
        (`/Engine/EditorBlueprintResources/StandardMacros.IsValid` _returnvalue
          (:`Is Valid`
            (bind _asbp_fps_player_state (cast `/Game/FPSKM/Blueprints/Game/BP_FPS_PlayerState` (`Pawn.PlayerState` _returnvalue)))
            (bind (_isfind _result) (`/Game/FPSKM/Blueprints/Game/BP_FPS_PlayerState.FindWeaponUpgradeData` _asbp_fps_player_state (`.No_2_B1B1004445E04EA72D06E797626700C8` (break `/Game/FPSKM/Blueprints/Structures/ItemData/S_WeaponItemData` (`self.WeaponData`)))))
            (set `local.LocalIsUseUpgradeData` _isfind)
            (set `local.LocalWeaponUpgradeData` _result)
            (if (`local.LocalIsUseUpgradeData`)
              (return (`.ClipSize_11_8FB0528C4D9617D5B71CBEA63F2585CE` (break `/Game/FPSKM/Blueprints/Structures/S_WeaponUpgradeData` (`local.LocalWeaponUpgradeData`))))
              (else
                (return (`self.MaxAmmo`))))))))
    (:`then_1`
      (return (`.MaxAmmo_36_F0673EA840826A9B4983ADAE08D4DF21` (break `/Game/FPSKM/Blueprints/Structures/ItemData/S_WeaponItemData` (`self.WeaponData`)))))))

(fn `GetReloadAmmoCount`
  (returns (AmmoCount :type Integer))
  (return (- (`self.GetMaxAmmo`) (`self.Ammo`))))

(fn `IsFullAmmo`
  (returns (Result :type Boolean))
  (return (>= (`self.Ammo`) (`self.GetMaxAmmo`))))

(fn `IsLeftAmmo`
  (returns (Result :type Boolean))
  (return (> (`self.Ammo`) 0)))

(fn `UserConstructionScript`
  (`parent.UserConstructionScript`)
  (bind _output_get (set `self.MaxAmmo` (`self.GetMaxAmmo`)))
  (set `self.Ammo` _output_get))