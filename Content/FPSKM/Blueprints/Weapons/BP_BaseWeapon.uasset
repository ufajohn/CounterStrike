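; Base weapon Blueprint that declares placeholder fire, reload, ammo and collision hooks, presumably for child weapons to override, plus shared visibility helpers.
; DamageProcess makes noise, then sends damage to non-instigator actors implementing DamageInterface, or calls the empty HitEffect event for other actors.
; CalculateDamage rolls base or upgrade damage ranges, doubling for CriChance criticals and Head-bone hits.
; SpawnHitEffect provides surface-selected impact sound, particles and a randomly rotated, fading decal.
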(event `Fire`
  (params (IpFireTarget :type "Vector Structure") (IpBarrelIndex :type Integer) (IpCharSpreadHalfAngleY :type "Float (double-precision)") (IpCharSpreadHalfAngleZ :type "Float (double-precision)")))

(event `FireEffect`
  (params (BarrelIndex :type Integer)))

(event `Reload`)

(event `UpdateFireTarget`
  (params (IpFireTarget :type "Vector Structure") (IpBarrelIndex :type Integer)))

(event `ShowBone`
  (params (IsVisible :type Boolean) (IpBoneName :type Name))
  (if (not IsVisible)
    (`SkinnedMeshComponent.HideBoneByName` (`self.SkeletalMesh`) IpBoneName "PBO_None")
    (else
      (`SkinnedMeshComponent.UnHideBoneByName` (`self.SkeletalMesh`) IpBoneName))))

(event `PlayFireAnim`)

(event `StartFire`
  (params (IpFireTarget :type "Vector Structure") (IpBarrelIndex :type Integer)))

(event `EndFire`)

(event `HitEffect`
  (params (IpLoc :type "Vector Structure") (IpNormal :type "Vector Structure") (SurfaceType :type "EPhysicalSurface Enum" :default "SurfaceType_Default")))

(fn `AddAmmo`
  (params (AddValue :type Integer))
  (returns (Result :type Boolean))
  (return true))

(fn `CalculateDamage`
  (params (IpMinDmg :type "Float (double-precision)") (IpMaxDmg :type "Float (double-precision)") (IpCriRate :type "Float (double-precision)") (IpHitBoneName :type Name))
  (returns (ResultDamage :type "Float (double-precision)") (IsCritical :type Boolean) (IsHeadshot :type Boolean))
  (locals (LocalDamage :type "Float (double-precision)") (LocalIsCritical :type Boolean :default false) (LocalIsHeadshot :type Boolean :default false))
  (`|ExecutionSequence`
    (:`then_0`
      ;[1 1 1] Set damage
      (set `local.LocalDamage` (`KismetMathLibrary.RandomFloatInRange` (`local.IpMinDmg`) (`local.IpMaxDmg`))))
    (:`then_1`
      ;[1 1 1] Set Critical Damage
      (if (<= (`KismetMathLibrary.RandomFloatInRange` 0.0 1.0) (`self.CriChance`))
        (set `local.LocalIsCritical` true)
        (set `local.LocalDamage` (* (`local.LocalDamage`) 2.0))
        (else
          (set `local.LocalIsCritical` false)))
      ;[1 1 1] Set Headshot damage
      (bind _output_get (set `local.LocalIsHeadshot` (== (`local.IpHitBoneName`) "Head")))
      (if _output_get
        (set `local.LocalDamage` (* (`local.LocalDamage`) 2.0)))
      (return (`local.LocalDamage`) (`local.LocalIsCritical`) (`local.LocalIsHeadshot`)))))

(fn `DamageProcess`
  (params (IpHitActor :type "Actor Object Reference") (IpHitResult :type "HitResult Structure"))
  (returns (Result :type Boolean) (Damage :type "Float (double-precision)"))
  (locals (LocalDamage :type "Float (double-precision)"))
  (bind _iphitresult (`local.IpHitResult`))
  (bind ((`DamageMin_10_8D9A4F434855B342C47F6AAE2C1BAB67` _damagemin) (`DamageMax_12_F236EEB247F9DD17023170B34B70BDCA` _damagemax) (`FireRate_31_8636439E4E4C4D13ECD3958D1711D44D` _firerate)) (break `/Game/FPSKM/Blueprints/Structures/ItemData/S_WeaponItemData` (`self.WeaponData`)))
  (bind ((`MinDamage_2_B6D3377E4A7D97AF877F9E840A123843` _mindamage) (`MaxDamage_4_0B6602644140C1E0EDA7838609EED9E3` _maxdamage) (`FireRate_6_8361091043D22391DDFCC0ACCC7E8FD4` _firerate_2)) (break `/Game/FPSKM/Blueprints/Structures/S_WeaponUpgradeData` (`self.WeaponUpgradeData`)))
  (bind (_bblockinghit _binitialoverlap _time _distance _location _impactpoint _normal) (`GameplayStatics.BreakHitResult` _iphitresult))
  (`|ExecutionSequence`
    (:`then_0`
      ;[1 1 1] Make Noise
      (`self.MakeNoise` 1.0 (`self.Instigator`) (`self.K2_GetActorLocation`) 200.0)
      ;[1 1 1] Check if can take damage
      (cast `/Game/FPSKM/Blueprints/Interfaces/DamageInterface` (`local.IpHitActor`)
        (:`then`
          (if (!= (`local.IpHitActor`) (`self.GetInstigator`))
            ;[1 1 1] Check if use upgrade data and set damage
            (if (`self.IsUseUpgradeData`)
              (set `local.LocalDamage` (`self.CalculateDamage` _mindamage _maxdamage _firerate_2 (`.HitBoneName_19_C518A751499D626195D0C4906C2979B0` (break `/Game/FPSKM/Blueprints/Structures/S_C_HitInfo` (`/Game/FPSKM/Blueprints/Game/BPFL_FPS.ToCHitInfo` (`local.IpHitResult`))))))
              (else
                (set `local.LocalDamage` (`self.CalculateDamage` _damagemin _damagemax _firerate (`.HitBoneName_19_C518A751499D626195D0C4906C2979B0` (break `/Game/FPSKM/Blueprints/Structures/S_C_HitInfo` (`/Game/FPSKM/Blueprints/Game/BPFL_FPS.ToCHitInfo` (`local.IpHitResult`))))))))
            ;[1 1 1] Take damage
            (message `/Game/FPSKM/Blueprints/Interfaces/DamageInterface.TakeDamage` (`local.IpHitActor`) "NewEnumerator0" (`local.LocalDamage`) 0.0 75000.0 (`KismetMathLibrary.Conv_RotatorToVector` (`self.K2_GetActorRotation`)) (`local.IpHitResult`) (`self.GetInstigator`) (0.0 0.0 0.0))))
        (:`CastFailed`
          ;[1 1 1] Hit effect
          (`self.HitEffect` _location _normal (`GameplayStatics.GetSurfaceType` _iphitresult)))))
    (:`then_1`
      (return false 0.0))))

(fn `EndCheckCollision`
  (returns (Result :type Boolean))
  (return true))

(fn `GetAmmoType`
  (returns (ResultAmmoType :type "/Game/FPSKM/Blueprints/Enums/E_A_AmmoType Enum"))
  (return (`.AmmoType_111_A99AFC6F49F4437EA31C79B709FCBFE4` (break `/Game/FPSKM/Blueprints/Structures/ItemData/S_WeaponItemData` (`self.WeaponData`)))))

(fn `GetMaxAmmo`
  (returns (MaxAmmo :type Integer))
  (locals (LocalIsUseUpgradeData :type Boolean :default false) (LocalWeaponUpgradeData :type "/Game/FPSKM/Blueprints/Structures/S_WeaponUpgradeData Structure"))
  (return 0))

(fn `GetReloadAmmoCount`
  (returns (AmmoCount :type Integer))
  (return 0))

(fn `IsFullAmmo`
  (returns (Result :type Boolean))
  (return false))

(fn `IsLeftAmmo`
  (returns (Result :type Boolean))
  (return false))

(fn `IsReadyFireMinigunFunc`
  (returns (Result :type Boolean))
  (return true))

(fn `Show`
  (params (Visible :type Boolean))
  (`|ExecutionSequence`
    (:`then_0`
      (`/Engine/EditorBlueprintResources/StandardMacros.IsValid` (`self.StaticMesh`)
        (:`Is Valid`
          (`SceneComponent.SetVisibility` (`self.StaticMesh`) (`local.Visible`) true))))
    (:`then_1`
      (`/Engine/EditorBlueprintResources/StandardMacros.IsValid` (`self.SkeletalMesh`)
        (:`Is Valid`
          (`SceneComponent.SetVisibility` (`self.SkeletalMesh`) (`local.Visible`) true))))))

(fn `SpawnHitEffect`
  (params (IpHitLoc :type "Vector Structure") (IpHitNormal :type "Vector Structure") (IpSurfaceType :type "EPhysicalSurface Enum" :default "SurfaceType_Default"))
  (locals (LocalDecal :type "DecalComponent Object Reference"))
  ;[1 1 1] Play Sound
  (`GameplayStatics.PlaySoundAtLocation` (select `EPhysicalSurface` (`local.IpSurfaceType`) :`SurfaceType_Default` "/Game/FPSKM/Audios/Cues/Concrete_01_Cue.Concrete_01_Cue" :!type "SoundBase Object Reference") (`local.IpHitLoc`) (struct) 1.0 1.0 0.0 "/Game/FPSKM/Audios/DefaultSoundAttenuation.DefaultSoundAttenuation" null null)
  ;[1 1 1] Spawn Eimmter
  (`GameplayStatics.SpawnEmitterAtLocation` (select `EPhysicalSurface` (`local.IpSurfaceType`) :`SurfaceType_Default` "/Game/FPSKM/Particles/PS_Impact_Default.PS_Impact_Default" :!type "ParticleSystem Object Reference") (`local.IpHitLoc`) (`KismetMathLibrary.MakeRotator` (.roll (`KismetMathLibrary.Conv_VectorToRotator` (`local.IpHitNormal`))) (+ (.pitch (`KismetMathLibrary.Conv_VectorToRotator` (`local.IpHitNormal`))) -90.0) (.yaw (`KismetMathLibrary.Conv_VectorToRotator` (`local.IpHitNormal`)))))
  ;[1 1 1] Spawn Decal
  (bind _returnvalue (`GameplayStatics.SpawnDecalAtLocation` (select `EPhysicalSurface` (`local.IpSurfaceType`) :`SurfaceType_Default` "/Game/FPSKM/Materials/Decals/M_Decals_DefaultBullet.M_Decals_DefaultBullet" :!type "MaterialInterface Object Reference") (`KismetMathLibrary.MakeVector` 4.0 4.0 4.0) (`local.IpHitLoc`) (`KismetMathLibrary.MakeRotFromX` (`local.IpHitNormal`)) 10.0))
  (bind _output_get (set `local.LocalDecal` _returnvalue))
  (`/Engine/EditorBlueprintResources/StandardMacros.IsValid` _output_get
    (:`Is Valid`
      (`SceneComponent.K2_AddLocalRotation` (`local.LocalDecal`) (`KismetMathLibrary.MakeRotator` (`KismetMathLibrary.RandomFloatInRange` -360.0 360.0) 0.0 180.0) false false)
      (`DecalComponent.SetFadeScreenSize` (`local.LocalDecal`) 1e-05)
      (`DecalComponent.SetFadeOut` (`local.LocalDecal`) 10.0 3.0 false))))

(fn `StartCheckCollision`
  (returns (Result :type Boolean))
  (return false))

(fn `UserConstructionScript`)