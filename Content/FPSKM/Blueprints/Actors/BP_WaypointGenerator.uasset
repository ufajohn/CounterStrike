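; BP_WaypointGenerator draws a navmesh waypoint trail between its parent actor and an objective actor.
; GenerateWaypoints starts a Tick-driven refresh that rebuilds a spline from the reversed navigation path, adding intermediate points at mesh-spacing intervals.
; Instanced static meshes are placed along the spline at that spacing, reusing existing instances and trimming extras.
; ClearWaypoints, also called on EndPlay, stops Tick and empties the spline and meshes.
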(event `self.ReceiveTick`
  (params (DeltaSeconds :type "Float (single-precision)"))
  ;[1 1 1] Event - Tick, GenerateWaypoints
  (`/Engine/EditorBlueprintResources/StandardMacros.IsValid` (`self.ObjectiveActor`) :!label _label
    (:`Is Valid`
      (`self.CreateSplinePointsForWaypointPath` (`self.ObjectiveActor`))
      (`self.DisplayWaypointsUsingInstancedStaticMeshes`)
      (`self.SetActorTickEnabled` true)
      (set `self.WaypointsActivated?` true))))

(event `GenerateWaypoints`
  (params (ObjectiveActor :type "Actor Object Reference"))
  ;[1 1 1] Event - Tick, GenerateWaypoints
  (set `self.ObjectiveActor` ObjectiveActor)
  (if (not (`self.WaypointsActivated?`))
    (goto _label)))

(event `ClearWaypoints`
  ;[1 1 1] Event - ClearWayponts
  (`self.SetActorTickEnabled` false)
  (`InstancedStaticMeshComponent.ClearInstances` (`self.WaypointDisplay`))
  (`SplineComponent.ClearSplinePoints` (`self.WaypointSpline`) true)
  (set `self.WaypointsActivated?` false))

(event `self.ReceiveEndPlay`
  (params (EndPlayReason :type "EEndPlayReason Enum" :default "Destroyed"))
  ;[1 1 1] Event - EndPlay
  (`self.ClearWaypoints`))

(fn `CalculateNumberOfSplinePathSegments`
  (returns (ReturnValue :type Integer))
  (return (`.ReturnValue` (`KismetMathLibrary.FMod` (`SplineComponent.GetSplineLength` (`self.WaypointSpline`)) (`self.PathMeshSpacing`)))))

(fn `CreateSplinePointsForWaypointPath`
  (params (GoalActor :type "Actor Object Reference"))
  (locals (Local_PathPoints :type "Array of Vector Structure"))
  (bind _returnvalue (`NavigationSystemV1.FindPathToActorSynchronously` (`NavigationSystemV1.K2_ProjectPointToNavigation` (`self.K2_GetActorLocation` (`self.GetParentActor`))) GoalActor 50.0 null null))
  (bind (_arrayindex _arrayelement) (`/Engine/EditorBlueprintResources/StandardMacros.ReverseForEachLoop` (`NavigationPath.PathPoints` _returnvalue))
    (:`LoopBody`
      (`KismetArrayLibrary.Array_Add` (`local.Local_PathPoints`) _arrayelement))
    (:`Completed`
      (if (> (`KismetArrayLibrary.Array_Length` (`local.Local_PathPoints`)) 1)
        (`SplineComponent.ClearSplinePoints` (`self.WaypointSpline`) true)
        (`self.GenerateAdditionalSplinePoints` (`local.Local_PathPoints`))
        (return)))))

(fn `DisplayWaypointsUsingInstancedStaticMeshes`
  (locals (Local_CurrentPathMeshLocation :type "Vector Structure") (LocalIndex :type Integer) (LocalSegNum :type Integer :default 0) (LocalInstCount :type Integer :default 0))
  (bind _waypointdisplay (`self.WaypointDisplay`))
  (bind _returnvalue (- (`local.LocalInstCount`) 1))
  (`|ExecutionSequence`
    (:`then_0`
      (bind _returnvalue_2 (`self.CalculateNumberOfSplinePathSegments`))
      (bind _output_get (set `local.LocalSegNum` _returnvalue_2))
      (for _index (range 1 (+ _output_get 1))
        (bind _output_get_2 (set `local.LocalIndex` _index))
        (set `local.Local_CurrentPathMeshLocation` (+ (+ (.location (`SplineComponent.GetTransformAtDistanceAlongSpline` (`self.WaypointSpline`) (* _output_get_2 (`self.PathMeshSpacing`)) "World" false)) (`self.MeshPlacementTraceStartOffset`)) (`self.PathMeshToSplineOffset`)))
        (if (< (- (`local.LocalIndex`) 1) (`InstancedStaticMeshComponent.GetInstanceCount` (`self.WaypointDisplay`)))
          (bind _returnvalue_3 (`KismetMathLibrary.MakeTransform` (`local.Local_CurrentPathMeshLocation`) (`KismetMathLibrary.MakeRotator` (+ (+ (.roll (.rotation (`SplineComponent.GetTransformAtDistanceAlongSpline` (`self.WaypointSpline`) (* _output_get_2 (`self.PathMeshSpacing`)) "World" false))) (.pitch (.rotation (`SplineComponent.GetTransformAtDistanceAlongSpline` (`self.WaypointSpline`) (* _output_get_2 (`self.PathMeshSpacing`)) "World" false)))) 180.0) 0.0 (+ (.yaw (.rotation (`SplineComponent.GetTransformAtDistanceAlongSpline` (`self.WaypointSpline`) (* _output_get_2 (`self.PathMeshSpacing`)) "World" false))) 180.0)) (.scale (`SplineComponent.GetTransformAtDistanceAlongSpline` (`self.WaypointSpline`) (* _output_get_2 (`self.PathMeshSpacing`)) "World" false))))
          (`InstancedStaticMeshComponent.UpdateInstanceTransform` _waypointdisplay (- (`local.LocalIndex`) 1) _returnvalue_3 true false true)
          (else
            (`InstancedStaticMeshComponent.AddInstanceWorldSpace` _waypointdisplay _returnvalue_3)))))
    (:`then_1`
      (set `local.LocalInstCount` (`InstancedStaticMeshComponent.GetInstanceCount` (`self.WaypointDisplay`)))
      (if (> (`local.LocalInstCount`) (`local.LocalSegNum`))
        (for _index_2 (range (`local.LocalSegNum`) (`local.LocalInstCount`))
          (`InstancedStaticMeshComponent.RemoveInstance` (`self.WaypointDisplay`) _index_2)))
      (`InstancedStaticMeshComponent.UpdateInstanceTransform` (`self.WaypointDisplay`) _returnvalue (`InstancedStaticMeshComponent.GetInstanceTransform` (`self.WaypointDisplay`) _returnvalue true) true true true)
      (return))))

(fn `GenerateAdditionalSplinePoints`
  (params (PathPoints :type "Array of Vector Structure"))
  (locals (Local_PathPoints :type "Array of Vector Structure") (Local_CurrentPathPointIndex :type Integer) (Local_CurrentPathLength :type "Float (double-precision)") (Local_CurrentPathUnitVector :type "Vector Structure") (Local_CurrentPathStartingPoint :type "Vector Structure"))
  (bind _pathpoints (`local.PathPoints`))
  (bind (_remainder _returnvalue) (`KismetMathLibrary.FMod` (`local.Local_CurrentPathLength`) (`self.PathMeshSpacing`)))
  (`SplineComponent.AddSplinePoint` (`self.WaypointSpline`) (`|GetArrayItem` (`local.PathPoints`)) "World" true)
  (for _index (range (+ (- (`KismetArrayLibrary.Array_Length` (`local.PathPoints`)) 2) 1))
    (bind _output_get (set `local.Local_CurrentPathPointIndex` _index))
    (bind _returnvalue_2 (- (`|GetArrayItem` _pathpoints (+ _output_get 1)) (`|GetArrayItem` _pathpoints (`local.Local_CurrentPathPointIndex`))))
    (set `local.Local_CurrentPathLength` (`KismetMathLibrary.VSize` _returnvalue_2))
    (set `local.Local_CurrentPathUnitVector` (`KismetMathLibrary.Normal` _returnvalue_2))
    (set `local.Local_CurrentPathStartingPoint` (`|GetArrayItem` (`local.PathPoints`) (`local.Local_CurrentPathPointIndex`)))
    (if (> _returnvalue 0)
      (for _index_2 (range 1 (+ _returnvalue 1))
        (`SplineComponent.AddSplinePoint` (`self.WaypointSpline`) (+ (`local.Local_CurrentPathStartingPoint`) (* (`local.Local_CurrentPathUnitVector`) (* _index_2 (`self.PathMeshSpacing`)))) "World" true)))
    (`SplineComponent.AddSplinePoint` (`self.WaypointSpline`) (`|GetArrayItem` (`local.PathPoints`) (+ (`local.Local_CurrentPathPointIndex`) 1)) "World" true) ; Add a spline point at the next path point location
  )
  (return))

(fn `UserConstructionScript`)