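; BP_MolotovFireDamageArea is a temporary fire area from a Molotov that repeatedly damages characters standing inside it.
; Box overlap events maintain an array of the characters currently inside.
; A looping timer sends each one a TakeDamageMessage with random damage between the minimum and maximum at a set interval.
; The actor destroys itself once its lifetime ends.
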(event `self.ReceiveBeginPlay`
  (`KismetSystemLibrary.K2_SetTimer` null "Damage" (`self.DamageIntervalTime`) true)
  (`KismetSystemLibrary.Delay` (`self.LifeTime`))
  (`self.K2_DestroyActor`))

(event `self.Box.OnComponentBeginOverlap`
  (params (OverlappedComponent :type "PrimitiveComponent Object Reference") (OtherActor :type "Actor Object Reference") (OtherComp :type "PrimitiveComponent Object Reference") (OtherBodyIndex :type Integer) (bFromSweep :type Boolean) (SweepResult :type "HitResult Structure (by ref)"))
  (bind _ascharacter (cast `Character` OtherActor))
  (`KismetArrayLibrary.Array_AddUnique` (`self.OverlapCharacterAry`) _ascharacter))

(event `self.Box.OnComponentEndOverlap`
  (params (OverlappedComponent :type "PrimitiveComponent Object Reference") (OtherActor :type "Actor Object Reference") (OtherComp :type "PrimitiveComponent Object Reference") (OtherBodyIndex :type Integer))
  (bind _ascharacter (cast `Character` OtherActor))
  (`KismetArrayLibrary.Array_RemoveItem` (`self.OverlapCharacterAry`) _ascharacter))

(event `Damage`
  (for _array_element (`self.OverlapCharacterAry`)
    (message `/Game/FPSKM/Blueprints/Interfaces/DamageInterface.TakeDamage` _array_element "NewEnumerator0" (`KismetMathLibrary.RandomFloatInRange` (`self.MinDamage`) (`self.MaxDamage`)) 0.0 75000.0 (0.0 0.0 0.0) (struct) null (0.0 0.0 0.0))))

(fn `UserConstructionScript`)