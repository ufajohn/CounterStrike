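; Melee weapon controller component that runs the owning hero's melee attacks.
; Starting an attack from either of two allowed hero states switches the state and plays the attack animation on the arm anim instance.
; Anim notify events open and close collision checking on the current weapon, then return the hero's state when the attack ends.
; Tick and SetAim are empty, and the input-driven firing logic is disconnected.
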(event `self.ReceiveTick`
  (params (DeltaSeconds :type "Float (single-precision)"))
  ;[1 1 1] Tick - Firing
)

(event `StartFireMeleeWeapon`
  ;[1 1 1] Starting MeleeAttack
  (if (or (`/Game/FPSKM/Blueprints/Characters/Player/BP_FPS_PlayerChar.IsCurState` (`self.OwnerHero`) "NewEnumerator0") (`/Game/FPSKM/Blueprints/Characters/Player/BP_FPS_PlayerChar.IsCurState` (`self.OwnerHero`) "NewEnumerator3"))
    (`/Game/FPSKM/Blueprints/Characters/Player/BP_FPS_PlayerChar.ChangeState` (`self.OwnerHero`) "NewEnumerator2")
    (message `/Game/FPSKM/Blueprints/Interfaces/ArmAnimInterface.PlayMeleeAttackAnim` (`/Game/FPSKM/Blueprints/Characters/BP_BaseChar.GetArmAnimInst` (`self.OwnerHero`)) 0)))

(event `/Game/FPSKM/Blueprints/Interfaces/AnimNotifyInterface.AnimNotify_OnAnim_StartCheckMeleeCollision`
  ;[1 1 1] Checking Melee Attack Collision
  (`/Game/FPSKM/Blueprints/Weapons/BP_BaseWeapon.StartCheckCollision` (`/Game/FPSKM/Blueprints/Characters/BP_BaseChar.CurWeapon` (`self.OwnerHero`))))

(event `/Game/FPSKM/Blueprints/Interfaces/AnimNotifyInterface.AnimNotify_OnAnim_EndCheckMeleeCollision`
  ;[1 1 1] Checking Melee Attack Collision
  (`/Game/FPSKM/Blueprints/Weapons/BP_BaseWeapon.EndCheckCollision` (`/Game/FPSKM/Blueprints/Characters/BP_BaseChar.CurWeapon` (`self.OwnerHero`))))

(event `/Game/FPSKM/Blueprints/Interfaces/AnimNotifyInterface.AnimNotify_OnAnimEnd_MeleeAttack`
  (`/Game/FPSKM/Blueprints/Characters/Player/BP_FPS_PlayerChar.ChangeState` (`self.OwnerHero`) "NewEnumerator0"))

(event `self.SetAim`
  (params (IsAming :type Boolean)))