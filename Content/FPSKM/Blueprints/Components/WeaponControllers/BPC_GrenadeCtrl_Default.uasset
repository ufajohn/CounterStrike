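; Character component that controls first-person grenade equipping, switching and throwing on the player's arms mesh.
; Input press pulls the pin and plays the ready animation; release or the grenade's warning timer lets Tick start the throw once ready.
; An anim notify detaches and launches the socket-attached projectile along camera forward, and a fresh one spawns afterwards.
; Switching uses animation-length delays, swapping the arms' anim class and per-grenade offsets.
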(event `self.ReceiveBeginPlay`
  ;[1 1 1] Event - BeginPlay
  (bind _ascharacter (cast `Character` (`self.GetOwner`)))
  (set `self.OwnerPlayerChar` _ascharacter))

(event `self.ReceiveTick`
  (params (DeltaSeconds :type "Float (single-precision)"))
  ;[1 1 1] Event - Tick
  (if (not (`self.IsThrowing`))
    (if (and (`self.IsReadyComplete`) (`self.IsReleaseThrowKey`))
      (set `self.IsThrowing` true)
      (set `self.IsReadyToThrowGrenade` false)
      (set `self.IsReadyComplete` false)
      (set `self.IsReleaseThrowKey` false)
      (bind _result (message `/Game/FPSKM/Blueprints/Interfaces/FPSGrenades/FPS_Grenade_ArmAnimInterface.PlayThrowAnim` (`SkeletalMeshComponent.GetAnimInstance` (`self.OwnerCharArms`))))
      (if (`self.IsUse`)
        (`KismetSystemLibrary.Delay` _result)
        (`KismetSystemLibrary.Delay` 0.02)
        (set `self.IsThrowing` false)
        (`self.CreateGrenadeProjectile` (`self.CurSelectGrenadeIndex`))
        (if (`self.IsEquip`)
          (`self.OnFinish_Throw`))))))

(event `InputPressed`
  (bind _curgrenadeprojectile (`self.CurGrenadeProjectile`))
  ;[1 1 1] Input Pressed
  (if (and (> (`self.CurSelectGrenadeIndex`) -1) (not (`self.IsChangingWeapon`)))
    (if (and (not (`self.IsReadyToThrowGrenade`)) (not (`self.IsThrowing`)))
      (set `self.IsReadyToThrowGrenade` true)
      (set `self.IsReleaseThrowKey` false)
      (set `self.IsReadyComplete` false)
      (`|ExecutionSequence`
        (:`then_0`
          (message `/Game/FPSKM/Blueprints/Interfaces/FPSGrenades/FPS_Grenade_WeaponAnimInterface.PlayThrowGrenade` (`/Game/FPSKM/Blueprints/Projectiles/Grenades/BP_GrenadeProjectile.GetAnimInst` (`self.CurGrenadeProjectile`)))
          (`/Game/FPSKM/Blueprints/Projectiles/Grenades/BP_GrenadeProjectile.PullPin` _curgrenadeprojectile)
          (add `/Game/FPSKM/Blueprints/Projectiles/Grenades/BP_GrenadeProjectile.OnWarningTime_Grendae` _curgrenadeprojectile (delegate `OnWarningTime_Grenade`)))
        (:`then_1`
          (bind _result (message `/Game/FPSKM/Blueprints/Interfaces/FPSGrenades/FPS_Grenade_ArmAnimInterface.PlayReadyThrowAnim` (`SkeletalMeshComponent.GetAnimInstance` (`self.OwnerCharArms`))))
          (`KismetSystemLibrary.Delay` _result)
          (if (`self.IsUse`)
            (set `self.IsReadyComplete` true)
            (message `/Game/FPSKM/Blueprints/Interfaces/FPSGrenades/FPS_Grenade_ArmAnimInterface.PlayReadyThrowIdleAnim` (`SkeletalMeshComponent.GetAnimInstance` (`self.OwnerCharArms`)))
            (`/Game/FPSKM/Blueprints/Projectiles/Grenades/BP_GrenadeProjectile.HidePin` (`self.CurGrenadeProjectile`))))))))

(event `OnWarningTime_Grenade`
  ;[1 1 1] Input Pressed
  (`self.InputReleased`))

(event `InputReleased`
  ;[1 1 1] StartThrow
  (set `self.IsReleaseThrowKey` true))

(event `/Game/FPSKM/Blueprints/Interfaces/FPSGrenades/FPS_Grenade_AnimNotifyInterface.AnimNotify_OnAnim_FireThrowGrenade`
  ;[1 1 1] Anim Notify - Fire Throw Grenade
  (`self.ThrowGrenade` (`Actor.K2_GetActorLocation` (`self.CurGrenadeProjectile`)) (* (`SceneComponent.GetForwardVector` (`self.OwnerCharCameraComp`)) (`self.GrenadeThrowPower`))))

(event `ThrowGrenade`
  (params (IpFireLoc :type "Vector Structure") (IpThrowVel :type "Vector Structure"))
  ;[1 1 1] Throw Grenade
  (`Actor.K2_DetachFromActor` (`self.CurGrenadeProjectile`) "KeepWorld" "KeepWorld" "KeepWorld")
  (`/Game/FPSKM/Blueprints/Projectiles/Grenades/BP_GrenadeProjectile.Throw` (`self.CurGrenadeProjectile`) IpThrowVel)
  (`self.OnThrowGrenade` (`self.CurSelectGrenadeIndex`)))

(event `StartChangeGrenade`
  (params (InTargetGrenadeIndex :type Integer))
  ;[1 1 1] StartChangeGrenade
  ;;[1 1 1] Check if player can change grenade
  (if (and (not (`self.IsReadyToThrowGrenade`)) (not (`self.IsThrowing`)) (not (`self.IsChangingWeapon`)) (!= InTargetGrenadeIndex (`self.CurSelectGrenadeIndex`)))
    (set `self.TargetSelectGrenadeIndex` InTargetGrenadeIndex)
    (set `self.IsUse` true)
    (set `self.IsChangingWeapon` true)
    ;;[1 1 1] UnEquip Grenade
    (bind _result (message `/Game/FPSKM/Blueprints/Interfaces/FPSGrenades/FPS_Grenade_ArmAnimInterface.PlayUnEquipAnim` (`SkeletalMeshComponent.GetAnimInstance` (`self.OwnerCharArms`))))
    (if (`self.IsUse`)
      (`KismetSystemLibrary.Delay` _result)
      (`self.OnFinish_UnEquipToChangeToGrenade`)
      (`self.SelectGrenade` (`self.TargetSelectGrenadeIndex`))
      ;;[1 1 1] Set Offset Rotation, Location
      (`SceneComponent.K2_SetRelativeRotation` (`self.OwnerCharArms`) (`KismetMathLibrary.MakeRotator` (+ (.roll (`self.OriginArmsRot`)) (.roll (`.OffsetRot_35_D6E7664E4D9884366DF464B7ABB41A8D` (break `/Game/FPSKM/Blueprints/Structures/FPSGrenades/S_FPSGrenade_WeaponInfo` (`|GetArrayItem` (`self.GrenadeWeaponInfoAry`) (`self.CurSelectGrenadeIndex`)))))) (+ (.pitch (`self.OriginArmsRot`)) (.pitch (`.OffsetRot_35_D6E7664E4D9884366DF464B7ABB41A8D` (break `/Game/FPSKM/Blueprints/Structures/FPSGrenades/S_FPSGrenade_WeaponInfo` (`|GetArrayItem` (`self.GrenadeWeaponInfoAry`) (`self.CurSelectGrenadeIndex`)))))) (+ (.yaw (`self.OriginArmsRot`)) (.yaw (`.OffsetRot_35_D6E7664E4D9884366DF464B7ABB41A8D` (break `/Game/FPSKM/Blueprints/Structures/FPSGrenades/S_FPSGrenade_WeaponInfo` (`|GetArrayItem` (`self.GrenadeWeaponInfoAry`) (`self.CurSelectGrenadeIndex`))))))) false false)
      (`SceneComponent.K2_SetRelativeLocation` (`self.OwnerCharArms`) (+ (`self.OriginArmsLoc`) (`.OffsetLoc_32_7E4F08854EAF5B3F653E72A61732D8A3` (break `/Game/FPSKM/Blueprints/Structures/FPSGrenades/S_FPSGrenade_WeaponInfo` (`|GetArrayItem` (`self.GrenadeWeaponInfoAry`) (`self.CurSelectGrenadeIndex`))))) false false)
      ;;[1 1 1] Equip Grenade
      (bind _result_2 (message `/Game/FPSKM/Blueprints/Interfaces/FPSGrenades/FPS_Grenade_ArmAnimInterface.GetEquipAnimLength` (`SkeletalMeshComponent.GetAnimInstance` (`self.OwnerCharArms`))))
      (`KismetSystemLibrary.Delay` _result_2)
      (set `self.IsChangingWeapon` false)
      (`self.OnFinish_EquipGrenade`))))

(event `UnEquipEvent`
  ;[1 1 1] Check if player can change grenade
  (if (and (not (`self.IsReadyToThrowGrenade`)) (not (`self.IsThrowing`)) (not (`self.IsChangingWeapon`)))
    (set `self.TargetSelectGrenadeIndex` -1)
    (set `self.IsChangingWeapon` true)
    ;[1 1 1] UnEquip Grenade
    (bind _result (message `/Game/FPSKM/Blueprints/Interfaces/FPSGrenades/FPS_Grenade_ArmAnimInterface.PlayUnEquipAnim` (`SkeletalMeshComponent.GetAnimInstance` (`self.OwnerCharArms`))))
    (`KismetSystemLibrary.Delay` _result)
    (if (`self.IsEquip`)
      (`self.OnFinish_UnEquipToChangeToAnother`)
      (set `self.IsChangingWeapon` false)
      (set `self.IsUse` false)
      (`self.SelectGrenade` -1)
      (`|ExecutionSequence`
        (:`then_0`
          (`/Engine/EditorBlueprintResources/StandardMacros.IsValid` (`self.OwnerCharArms`)
            (:`Is Valid`
              (`SceneComponent.K2_SetRelativeLocation` (`self.OwnerCharArms`) (`self.OriginArmsLoc`) false false)
              (`SceneComponent.K2_SetRelativeRotation` (`self.OwnerCharArms`) (`self.OriginArmsRot`) false false))))
        (:`then_1`
          (`/Engine/EditorBlueprintResources/StandardMacros.IsValid` (`self.CurGrenadeProjectile`)
            (:`Is Valid`
              (if (not (`/Game/FPSKM/Blueprints/Projectiles/Grenades/BP_GrenadeProjectile.IsThrow` (`self.CurGrenadeProjectile`)))
                (`Actor.K2_DestroyActor` (`self.CurGrenadeProjectile`))))))))))

(fn `CreateGrenadeProjectile`
  (params (InSelectGrenadeIndex :type Integer))
  (bind _ownerplayerchar (`self.OwnerPlayerChar`))
  (bind ((`GrenadeClass_37_5BF0F3D341559659D6A1338DAF1D0231` _grenadeclass) (`AttachSocketName_13_325FA23047C7B83131CCCF934996E543` _attachsocketname)) (break `/Game/FPSKM/Blueprints/Structures/FPSGrenades/S_FPSGrenade_WeaponInfo` (`|GetArrayItem` (`self.GrenadeWeaponInfoAry`) (`local.InSelectGrenadeIndex`))))
  (bind _returnvalue (`|SpawnActorFromClass` _grenadeclass (`SceneComponent.GetSocketTransform` (`self.OwnerCharArms`) (`KismetStringLibrary.Conv_StringToName` _attachsocketname) "RTS_World") "Undefined" "OverrideRootScale" _ownerplayerchar _ownerplayerchar))
  (bind _output_get (set `self.CurGrenadeProjectile` _returnvalue))
  (`PrimitiveComponent.IgnoreActorWhenMoving` (`SkeletalMeshActor.SkeletalMeshComponent` _output_get) (`self.OwnerPlayerChar`) true)
  (`PrimitiveComponent.IgnoreActorWhenMoving` (`Character.CapsuleComponent` (`self.OwnerPlayerChar`)) (`self.CurGrenadeProjectile`) true)
  (`PrimitiveComponent.SetCollisionResponseToChannel` (`SkeletalMeshActor.SkeletalMeshComponent` (`self.CurGrenadeProjectile`)) "ECC_Pawn" "ECR_Ignore")
  (`PrimitiveComponent.SetCollisionEnabled` (`SkeletalMeshActor.SkeletalMeshComponent` (`self.CurGrenadeProjectile`)) "NoCollision")
  (`Actor.K2_AttachToComponent` (`self.CurGrenadeProjectile`) (`self.OwnerCharArms`) (`KismetStringLibrary.Conv_StringToName` (`.AttachSocketName_13_325FA23047C7B83131CCCF934996E543` (break `/Game/FPSKM/Blueprints/Structures/FPSGrenades/S_FPSGrenade_WeaponInfo` (`|GetArrayItem` (`self.GrenadeWeaponInfoAry`) (`local.InSelectGrenadeIndex`))))) "SnapToTarget" "SnapToTarget" "SnapToTarget" true))

(fn `Init`
  (params (InArms :type "SkeletalMeshComponent Object Reference") (InCamComp :type "CameraComponent Object Reference"))
  (bind _output_get (set `self.OwnerCharArms` InArms))
  (set `self.OriginArmsLoc` (`SceneComponent.RelativeLocation` _output_get))
  (set `self.OriginArmsRot` (`SceneComponent.RelativeRotation` (`self.OwnerCharArms`)))
  (set `self.OwnerCharCameraComp` (`local.InCamComp`)))

(fn `IsEquip`
  (returns (Result :type Boolean))
  (return (> (`self.CurSelectGrenadeIndex`) -1)))

(fn `IsReadyOrThrowing`
  (returns (ReturnValue :type Boolean))
  (return (or (`self.IsReadyToThrowGrenade`) (`self.IsThrowing`))))

(fn `SelectGrenade`
  (params (InSelectIndex :type Integer))
  (bind _output_get (set `self.CurSelectGrenadeIndex` InSelectIndex))
  (if (> _output_get -1)
    (`|ExecutionSequence`
      (:`then_0`
        (`/Engine/EditorBlueprintResources/StandardMacros.IsValid` (`self.CurGrenadeProjectile`)
          (:`Is Valid`
            (if (not (`/Game/FPSKM/Blueprints/Projectiles/Grenades/BP_GrenadeProjectile.IsThrow` (`self.CurGrenadeProjectile`)))
              (`Actor.K2_DestroyActor` (`self.CurGrenadeProjectile`))))))
      (:`then_1`
        (`self.CreateGrenadeProjectile` (`self.CurSelectGrenadeIndex`))
        (`SkeletalMeshComponent.K2_SetAnimInstanceClass` (`self.OwnerCharArms`) (`.ArmAnimBPClass_38_FABA84DE4ACF15BC620103A726EA624E` (break `/Game/FPSKM/Blueprints/Structures/FPSGrenades/S_FPSGrenade_WeaponInfo` (`|GetArrayItem` (`self.GrenadeWeaponInfoAry`) (`self.CurSelectGrenadeIndex`)))))))))

(fn `UnEquipImmediately`
  (set `self.IsReadyToThrowGrenade` false)
  (set `self.IsReleaseThrowKey` false)
  (set `self.IsReadyComplete` false)
  (set `self.IsThrowing` false)
  (set `self.IsUse` false)
  (`self.SelectGrenade` -1)
  (`|ExecutionSequence`
    (:`then_0`
      (`/Engine/EditorBlueprintResources/StandardMacros.IsValid` (`self.OwnerCharArms`)
        (:`Is Valid`
          (`SceneComponent.K2_SetRelativeLocation` (`self.OwnerCharArms`) (`self.OriginArmsLoc`) false false)
          (`SceneComponent.K2_SetRelativeRotation` (`self.OwnerCharArms`) (`self.OriginArmsRot`) false false))))
    (:`then_1`
      (`/Engine/EditorBlueprintResources/StandardMacros.IsValid` (`self.CurGrenadeProjectile`)
        (:`Is Valid`
          (if (not (`/Game/FPSKM/Blueprints/Projectiles/Grenades/BP_GrenadeProjectile.IsThrow` (`self.CurGrenadeProjectile`)))
            (`Actor.K2_DestroyActor` (`self.CurGrenadeProjectile`))))))))