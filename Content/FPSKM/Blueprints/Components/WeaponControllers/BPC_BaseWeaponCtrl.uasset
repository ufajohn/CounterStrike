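; Base weapon controller component for the FPS player character, handling firing, aiming, reloading and crosshair visibility.
; While in use, Tick polls fire input and plays fire animations, gated by character state, ammo and a fire-rate delay.
; Anim notifies trigger the actual shots with camera shake and, on reload end, move inventory ammo into the weapon and update PlayerState.
; An empty weapon auto-reloads, and aiming adjusts walk speed and FOV.
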(event `self.ReceiveBeginPlay`
  ;[1 1 1] Event - BeginPlay
  (bind _asbp_fps_player_char (cast `/Game/FPSKM/Blueprints/Characters/Player/BP_FPS_PlayerChar` (`self.GetOwner`)))
  (set `self.OwnerHero` _asbp_fps_player_char))

(event `self.ReceiveTick`
  (params (DeltaSeconds :type "Float (single-precision)"))
  (bind _ownerhero (`self.OwnerHero`))
  (if (`self.IsUse`)
    (if (`/Game/FPSKM/Blueprints/Characters/Player/BP_FPS_PlayerChar.IsPressingFireInput` (`self.OwnerHero`))
      (`/Game/FPSKM/Blueprints/Weapons/BP_BaseRangedWeapon.UpdateFireTarget` (`/Game/FPSKM/Blueprints/Characters/BP_BaseChar.CurWeapon` _ownerhero) (`/Game/FPSKM/Blueprints/Characters/Player/BP_FPS_PlayerChar.FireTargetLoc` _ownerhero) 0)
      (if (`/Game/FPSKM/Blueprints/Characters/BP_BaseChar.CanFire_State` (`self.OwnerHero`))
        (`self.StartFireRangedWeapon`)))))

(event `StartFireRangedWeapon`
  (bind ((`FireAnimMontage_2_4E3B9F774C7CF1AEEA18A490ADEFD0B6` _fireanimmontage) (`CrouchFireAnimMontage_27_EEE2DBD1400DC994C096E09007D499B2` _crouchfireanimmontage)) (break `/Game/FPSKM/Blueprints/Structures/S_WeaponAnimData` (`/Game/FPSKM/Blueprints/Characters/BP_BaseChar.CurWeaponAnimData` (`self.OwnerHero`))))
  (if (`/Game/FPSKM/Blueprints/Weapons/BP_BaseWeapon.IsLeftAmmo` (`/Game/FPSKM/Blueprints/Characters/BP_BaseChar.CurWeapon` (`self.OwnerHero`)))
    (if (not (`/Game/FPSKM/Blueprints/Characters/BP_BaseChar.IsFiring` (`self.OwnerHero`)))
      (`self.StartFireTimer`)
      (`/Game/FPSKM/Blueprints/Characters/Player/BP_FPS_PlayerChar.ChangeState` (`self.OwnerHero`) "NewEnumerator4")
      (set `/Game/FPSKM/Blueprints/Characters/BP_BaseChar.IsSprint` false (`self.OwnerHero`))
      (`/Game/FPSKM/Blueprints/Characters/Player/BP_FPS_PlayerChar.Set_FireWalkSpeed` (`self.OwnerHero`))
      (if (not (`Character.bIsCrouched` (`self.OwnerHero`)))
        (`/Game/FPSKM/Blueprints/Characters/BP_BaseChar.PlayAnimMontageEvent` (`self.OwnerHero`) _fireanimmontage 1.0)
        (else
          (`/Game/FPSKM/Blueprints/Characters/BP_BaseChar.PlayAnimMontageEvent` (`self.OwnerHero`) _crouchfireanimmontage 1.0)))
      (message `/Game/FPSKM/Blueprints/Interfaces/ArmAnimInterface.PlayFireAnim` (`/Game/FPSKM/Blueprints/Characters/BP_BaseChar.GetArmAnimInst` (`self.OwnerHero`)))
      (`/Game/FPSKM/Blueprints/Weapons/BP_BaseWeapon.PlayFireAnim` (`/Game/FPSKM/Blueprints/Characters/BP_BaseChar.CurWeapon` (`self.OwnerHero`))))
    (elif (not (`/Game/FPSKM/Blueprints/Characters/BP_BaseChar.IsFiring` (`self.OwnerHero`)))
      (`self.ReqReloadStart`))))

(event `StartFireWeapon`
  (params (IpFireTargetLoc :type "Vector Structure"))
  (`/Game/FPSKM/Blueprints/Weapons/BP_BaseWeapon.StartFire` (`/Game/FPSKM/Blueprints/Characters/BP_BaseChar.CurWeapon` (`self.OwnerHero`)) IpFireTargetLoc 0))

(event `StopFireWeaponEvent`
  (bind _ownerhero (`self.OwnerHero`))
  (set `self.FireCount` 0)
  (set `self.CurBurstCount` 0)
  (if (not (`/Game/FPSKM/Blueprints/Characters/BP_BaseChar.IsAiming` (`self.OwnerHero`)))
    (set `CharacterMovementComponent.MaxWalkSpeed` (`/Game/FPSKM/Blueprints/Characters/Player/BP_FPS_PlayerChar.OriginWalkSpeed` _ownerhero) (`Character.CharacterMovement` _ownerhero)))
  (`/Game/FPSKM/Blueprints/Weapons/BP_BaseWeapon.EndFire` (`/Game/FPSKM/Blueprints/Characters/BP_BaseChar.CurWeapon` (`self.OwnerHero`))))

(event `Fire`
  (params (BarrelIndex :type Integer))
  (bind _ownerhero (`self.OwnerHero`))
  (`self.FireCamShake`)
  (`/Game/FPSKM/Blueprints/Weapons/BP_BaseWeapon.Fire` (`/Game/FPSKM/Blueprints/Characters/BP_BaseChar.CurWeapon` (`self.OwnerHero`)) (`/Game/FPSKM/Blueprints/Characters/Player/BP_FPS_PlayerChar.FireTargetLoc` (`self.OwnerHero`)) BarrelIndex (`/Game/FPSKM/Blueprints/Characters/BP_BaseChar.CharWeaponSpreadHalfAngleY` _ownerhero) (`/Game/FPSKM/Blueprints/Characters/BP_BaseChar.CharWeaponSpreadHalfAngleZ` _ownerhero))
  (`self.WeaponFireEffect` BarrelIndex))

(event `WeaponFireEffect`
  (params (IpBarrelIndex :type Integer))
  (bind _curweapon (`/Game/FPSKM/Blueprints/Characters/BP_BaseChar.CurWeapon` (`self.OwnerHero`)))
  (`/Engine/EditorBlueprintResources/StandardMacros.IsValid` _curweapon
    (:`Is Valid`
      (`/Game/FPSKM/Blueprints/Weapons/BP_BaseWeapon.FireEffect` _curweapon IpBarrelIndex))))

(event `/Game/FPSKM/Blueprints/Interfaces/AnimNotifyInterface.AnimNotify_OnAnim_Fire`
  (params (FireIndex :type Integer))
  (if (`self.IsUse`)
    (`self.Fire` FireIndex)
    (if (== (`self.FireCount`) 0)
      (`self.StartFireWeapon` (`/Game/FPSKM/Blueprints/Characters/Player/BP_FPS_PlayerChar.FireTargetLoc` (`self.OwnerHero`))))
    (set `self.FireCount` (+ (`self.FireCount`) 1))
    (if (not (`.IsAutoFire_130_9FCC57534D11802DD4CE0BAF59592B69` (break `/Game/FPSKM/Blueprints/Structures/ItemData/S_WeaponItemData` (`/Game/FPSKM/Blueprints/Characters/BP_BaseChar.CurWeaponData` (`self.OwnerHero`)))))
      (`/Game/FPSKM/Blueprints/Characters/Player/BP_FPS_PlayerChar.Released_FireInput` (`self.OwnerHero`)))))

(event `SetAim`
  (params (IsAming :type Boolean))
  (bind _output_get (set `self.IsAiming` IsAming))
  (if _output_get
    (`/Game/FPSKM/Blueprints/Characters/BP_BaseChar.SetCharMaxWalkSpeed` (`self.OwnerHero`) (`/Game/FPSKM/Blueprints/Characters/Player/BP_FPS_PlayerChar.AimWalkSpeed` (`self.OwnerHero`)))
    (else
      (`/Game/FPSKM/Blueprints/Characters/BP_BaseChar.SetCharMaxWalkSpeed` (`self.OwnerHero`) (`/Game/FPSKM/Blueprints/Characters/Player/BP_FPS_PlayerChar.OriginWalkSpeed` (`self.OwnerHero`)))))
  (`/Game/FPSKM/Blueprints/Characters/Player/BP_FPS_PlayerChar.SetAimFOV` (`self.OwnerHero`) (`self.IsAiming`)))

(event `/Game/FPSKM/Blueprints/Interfaces/AnimNotifyInterface.AnimNotify_OnAnimEnd_Fire`
  (if (not (`/Game/FPSKM/Blueprints/Weapons/BP_BaseWeapon.IsLeftAmmo` (`/Game/FPSKM/Blueprints/Characters/BP_BaseChar.CurWeapon` (`self.OwnerHero`))))
    (`self.ReqReloadStart`)))

(event `FireCamShake`
  (`PlayerController.ClientStartCameraShake` :`self` (`GameplayStatics.GetPlayerController` 0) :`Scale` (/ (`KismetMathLibrary.FClamp` 2.0 0.0 10.0) 2.0)))

(event `TryStopFireWeapon`
  (if (or (`/Game/FPSKM/Blueprints/Characters/Player/BP_FPS_PlayerChar.IsCurState` (`self.OwnerHero`) "NewEnumerator2") (`/Game/FPSKM/Blueprints/Characters/Player/BP_FPS_PlayerChar.IsCurState` (`self.OwnerHero`) "NewEnumerator4") (`/Game/FPSKM/Blueprints/Characters/Player/BP_FPS_PlayerChar.IsCurState` (`self.OwnerHero`) "NewEnumerator0"))
    (`self.StopFireWeaponEvent`)
    (if (`/Game/FPSKM/Blueprints/Characters/Player/BP_FPS_PlayerChar.IsCurState` (`self.OwnerHero`) "NewEnumerator4")
      (`/Game/FPSKM/Blueprints/Characters/Player/BP_FPS_PlayerChar.ChangeState` (`self.OwnerHero`) "NewEnumerator0"))))

(event `StartFireTimer`
  (if (not (`/Game/FPSKM/Blueprints/Characters/BP_BaseChar.IsFiring` (`self.OwnerHero`)))
    (set `/Game/FPSKM/Blueprints/Characters/BP_BaseChar.IsFiring` true (`self.OwnerHero`))
    (`KismetSystemLibrary.RetriggerableDelay` (`/Game/FPSKM/Blueprints/Characters/BP_BaseChar.GetFireRate` (`self.OwnerHero`)))
    (set `/Game/FPSKM/Blueprints/Characters/BP_BaseChar.IsFiring` false (`self.OwnerHero`))))

(event `HideCrosshair`
  (params (IpReloadTime :type "Float (double-precision)"))
  (bind _asbp_fps_game_inst (cast `/Game/FPSKM/Blueprints/Game/BP_FPS_GameInst` (`GameplayStatics.GetGameInstance`)))
  (`/Game/FPSKM/Blueprints/Game/BP_FPS_GameInst.ShowCrosshair` _asbp_fps_game_inst "NewEnumerator2" false))

(event `/Game/FPSKM/Blueprints/Interfaces/AnimNotifyInterface.AnimNotify_OnAnimEnd_Reload`
  (bind _curweapon (`/Game/FPSKM/Blueprints/Characters/BP_BaseChar.CurWeapon` (`self.OwnerHero`)))
  (set `/Game/FPSKM/Blueprints/Characters/BP_BaseChar.IsReloading` false (`self.OwnerHero`))
  (`/Game/FPSKM/Blueprints/Characters/Player/BP_FPS_PlayerChar.ChangeState` (`self.OwnerHero`) "NewEnumerator0")
  (`self.ShowCrosshair` (`.CrosshairType_156_97ED99294EB36DCBACA54BA31E0A408A` (break `/Game/FPSKM/Blueprints/Structures/ItemData/S_WeaponItemData` (`/Game/FPSKM/Blueprints/Characters/BP_BaseChar.CurWeaponData` (`self.OwnerHero`)))) true)
  (bind _resultusecount (`/Game/FPSKM/Blueprints/Characters/BP_BaseChar.UseCharInvenAmmo` (`self.OwnerHero`) (`/Game/FPSKM/Blueprints/Weapons/BP_BaseWeapon.GetAmmoType` _curweapon) (`/Game/FPSKM/Blueprints/Weapons/BP_BaseWeapon.GetReloadAmmoCount` _curweapon)))
  (`/Game/FPSKM/Blueprints/Weapons/BP_BaseWeapon.AddAmmo` (`/Game/FPSKM/Blueprints/Characters/BP_BaseChar.CurWeapon` (`self.OwnerHero`)) _resultusecount)
  (bind _asbp_fps_player_state (cast `/Game/FPSKM/Blueprints/Game/BP_FPS_PlayerState` (`Pawn.PlayerState` (`self.OwnerHero`))))
  (set `/Game/FPSKM/Blueprints/Game/BP_FPS_PlayerState.CharInvenInfo` (`/Game/FPSKM/Blueprints/Characters/BP_BaseChar.CharInvenInfo` (`self.OwnerHero`)) _asbp_fps_player_state))

(event `StartReloadEvent`
  (`Character.PlayAnimMontage` (`self.OwnerHero`) (`.ReloadAnimMontage_4_9C62DF204213D0CEE6C315B9E1EA40B7` (break `/Game/FPSKM/Blueprints/Structures/S_WeaponAnimData` (`/Game/FPSKM/Blueprints/Characters/BP_BaseChar.CurWeaponAnimData` (`self.OwnerHero`)))) 1.0 "None")
  (message `/Game/FPSKM/Blueprints/Interfaces/ArmAnimInterface.PlayReloadAnim` (`/Game/FPSKM/Blueprints/Characters/BP_BaseChar.GetArmAnimInst` (`self.OwnerHero`)))
  (message `/Game/FPSKM/Blueprints/Interfaces/ArmAnimInterface.PlayReloadAnim_Shotgun` (`/Game/FPSKM/Blueprints/Characters/BP_BaseChar.GetArmAnimInst` (`self.OwnerHero`)) (`/Game/FPSKM/Blueprints/Weapons/BP_BaseWeapon.GetReloadAmmoCount` (`/Game/FPSKM/Blueprints/Characters/BP_BaseChar.CurWeapon` (`self.OwnerHero`))))
  (`/Game/FPSKM/Blueprints/Weapons/BP_BaseWeapon.Reload` (`/Game/FPSKM/Blueprints/Characters/BP_BaseChar.CurWeapon` (`self.OwnerHero`)))
  (if (not (`self.IsAiming`))
    (`/Game/FPSKM/Blueprints/Characters/BP_BaseChar.SetCharMaxWalkSpeed` (`self.OwnerHero`) (`/Game/FPSKM/Blueprints/Characters/Player/BP_FPS_PlayerChar.OriginWalkSpeed` (`self.OwnerHero`)))))

(event `ShowCrosshairEvent`
  (bind _asbp_fps_game_inst (cast `/Game/FPSKM/Blueprints/Game/BP_FPS_GameInst` (`GameplayStatics.GetGameInstance`)))
  (`/Game/FPSKM/Blueprints/Game/BP_FPS_GameInst.ShowCrosshair` _asbp_fps_game_inst (`.CrosshairType_156_97ED99294EB36DCBACA54BA31E0A408A` (break `/Game/FPSKM/Blueprints/Structures/ItemData/S_WeaponItemData` (`/Game/FPSKM/Blueprints/Characters/BP_BaseChar.CurWeaponData` (`self.OwnerHero`)))) true))

(event `ReqReloadStart`
  (if (not (`/Game/FPSKM/Blueprints/Characters/BP_BaseChar.IsReloading` (`self.OwnerHero`)))
    (if (not (`/Game/FPSKM/Blueprints/Characters/BP_BaseChar.IsDeath` (`self.OwnerHero`)))
      (if (`/Game/FPSKM/Blueprints/Weapons/BP_BaseWeapon.IsFullAmmo` (`/Game/FPSKM/Blueprints/Characters/BP_BaseChar.CurWeapon` (`self.OwnerHero`)))
        _
        (elif (> (`/Game/FPSKM/Blueprints/Characters/BP_BaseChar.GetCharInvenAmmo` (`self.OwnerHero`) (`/Game/FPSKM/Blueprints/Weapons/BP_BaseWeapon.GetAmmoType` (`/Game/FPSKM/Blueprints/Characters/BP_BaseChar.CurWeapon` (`self.OwnerHero`)))) 0)
          (`self.TryStopFireWeapon`)
          (set `/Game/FPSKM/Blueprints/Characters/BP_BaseChar.IsReloading` true (`self.OwnerHero`))
          (`/Game/FPSKM/Blueprints/Characters/Player/BP_FPS_PlayerChar.ChangeState` (`self.OwnerHero`) "NewEnumerator8")
          (`self.StartReloadEvent`)
          (bind _result (message `/Game/FPSKM/Blueprints/Interfaces/ArmAnimInterface.GetReloadAnimTime` (`/Game/FPSKM/Blueprints/Characters/BP_BaseChar.GetArmAnimInst` (`self.OwnerHero`))))
          (`self.HideCrosshair` _result))))))

(fn `ShowCrosshair`
  (params (InCrosshairType :type "/Game/FPSKM/Blueprints/Crosshair/Enums/E_CrosshairType Enum" :default "NewEnumerator2") (InVisible :type Boolean))
  (bind _crosshairwidgetref (`self.CrosshairWidgetRef`))
  (`/Engine/EditorBlueprintResources/StandardMacros.IsValid` (`self.CrosshairWidgetRef`)
    (:`Is Valid`
      _)
    (:`Is Not Valid`
      (bind _returnvalue (`|CreateWidget` "/Game/FPSKM/Blueprints/Crosshair/Widgets/Widget_Crosshair_Main.Widget_Crosshair_Main_C"))
      (set `self.CrosshairWidgetRef` _returnvalue)))
  (if (not (`Widget.IsInViewport` _crosshairwidgetref))
    (`UserWidget.AddToViewport` _crosshairwidgetref 0))
  (`/Game/FPSKM/Blueprints/Crosshair/Widgets/Widget_Crosshair_Main.ShowCrosshair` (`self.CrosshairWidgetRef`) (`local.InCrosshairType`) (`local.InVisible`)))