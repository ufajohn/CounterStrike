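; Wave spawner for the FPS defense mode that runs timed enemy waves through to victory.
; A looping timer spawns enemies at random points, choosing classes by percent weight.
; Tick detects cleared waves via tracked enemies and death counts, then starts a wait countdown or declares victory.
; It pushes wave state to BP_FPS_GameState and widgets to player controllers; IsBossWave always returns false, so boss announcements never show.
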(event `self.ReceiveBeginPlay`
  ;[1 1 1] Event - BeginPlay
  (`KismetSystemLibrary.Delay` 1.0)
  ;;[1 1 1] Show Defense Game Play Widget
  (bind _outactors (`GameplayStatics.GetAllActorsOfClass` "/Game/FPSKM/Blueprints/Game/BP_PC_FPS.BP_PC_FPS_C"))
  (for _array_element _outactors
    (`/Game/FPSKM/Blueprints/Game/BP_PC_FPS.OwningClient_DefenseGamePlayWidget` _array_element))
  ;;[1 1 1] Start Delay
  (`KismetSystemLibrary.Delay` (`self.WaveStartDelay`))
  (set `self.CurWaveInfo` (`|GetArrayItem` (`self.WaveInfoAry`) (`self.CurWaveIndex`)))
  ;;[1 1 1] Check if cur wave has boss
  (if (`self.IsBossWave` (`self.CurWaveInfo`))
    ;;[1 1 1] Show Boss Wave Widget
    (bind _outactors_2 (`GameplayStatics.GetAllActorsOfClass` "/Game/FPSKM/Blueprints/Game/BP_PC_FPS.BP_PC_FPS_C"))
    (for _array_element_2 _outactors_2
      (`/Game/FPSKM/Blueprints/Game/BP_PC_FPS.OwningClient_StartBossNextWave` _array_element_2)
      (`self.StartWaveEvent` (+ (`self.CurWaveIndex`) 1) (`KismetArrayLibrary.Array_Length` (`self.WaveInfoAry`)) :!label _label)
      ;;[1 1 1] Spawn a Enemy Actor
      (`self.StartSpawnEnemy`
        (:`NewParam`
          ;;[1 1 1] Set Left Enemy Count
          (set `/Game/FPSKM/Blueprints/Game/BP_FPS_GameState.LeftEnemyCount` (- (`.NumberOfEnemies_2_C03758C74F5B1AA87E2C3EBD3B1C1FD8` (break `/Game/FPSKM/Blueprints/Structures/S_DefaultWaveInfo` (`self.CurWaveInfo`))) (`self.CurWaveDeathCharCount`)) (`self.DefenseGameState`)))))
    (else
      ;;[1 1 1] Show Next Wave Widget
      (bind _outactors_3 (`GameplayStatics.GetAllActorsOfClass` "/Game/FPSKM/Blueprints/Game/BP_PC_FPS.BP_PC_FPS_C"))
      (for _array_element_3 _outactors_3
        (`/Game/FPSKM/Blueprints/Game/BP_PC_FPS.OwningClient_StartNextWave` _array_element_3)
        (goto _label)))))

(event `self.ReceiveTick`
  (params (DeltaSeconds :type "Float (single-precision)"))
  ;[1 1 1] Event - Tick
  (bind _asbp_fps_game_state (cast `/Game/FPSKM/Blueprints/Game/BP_FPS_GameState` (`GameplayStatics.GetGameState`)))
  (set `self.DefenseGameState` _asbp_fps_game_state)
  (if (`self.IsPlaying`)
    ;;[1 1 1] Check if cur wave finished
    (if (`self.CheckNextWave`)
      ;;[1 1 1] Check if All wave finished
      (if (>= (+ (`self.CurWaveIndex`) 1) (`KismetArrayLibrary.Array_Length` (`self.WaveInfoAry`)))
        ;;[1 1 1] All wave finished
        (`self.OnFinish_AllWave_Event` (+ (`self.CurWaveIndex`) 1) (`KismetArrayLibrary.Array_Length` (`self.WaveInfoAry`)))
        (set `self.IsPlaying` false)
        (bind _outactors (`GameplayStatics.GetAllActorsOfClass` "/Game/FPSKM/Blueprints/Game/BP_PC_FPS.BP_PC_FPS_C"))
        (for _array_element _outactors
          (`/Game/FPSKM/Blueprints/Game/BP_PC_FPS.OwningClient_Victory` _array_element))
        (else
          ;;[1 1 1] Change GameState To Wait Next Wave State
          (`KismetSystemLibrary.Delay` 3.0)
          (`self.OnEnd_Wave_Event` (+ (`self.CurWaveIndex`) 1) (`KismetArrayLibrary.Array_Length` (`self.WaveInfoAry`)))
          (set `self.IsPlaying` false)
          (set `/Game/FPSKM/Blueprints/Game/BP_FPS_GameState.CurDefensePlayState` "NewEnumerator2" (`self.DefenseGameState`))
          (bind _outactors_2 (`GameplayStatics.GetAllActorsOfClass` "/Game/FPSKM/Blueprints/Game/BP_PC_FPS.BP_PC_FPS_C"))
          (for _array_element_2 _outactors_2
            (`/Game/FPSKM/Blueprints/Game/BP_PC_FPS.OwningClient_WaveComplete_WaitNextWave` _array_element_2))
          (bind _returnvalue (`KismetSystemLibrary.K2_SetTimer` null "WaitTimerEvent" 1.0 true))
          (set `self.WaveWaitTimer` _returnvalue))))))

(event `StartNextWave`
  ;[1 1 1] StartNextWave
  (set `self.CurWaveDeathCharCount` 0)
  ;;[1 1 1] Set Left Enemy Count
  (set `/Game/FPSKM/Blueprints/Game/BP_FPS_GameState.LeftEnemyCount` (- (`.NumberOfEnemies_2_C03758C74F5B1AA87E2C3EBD3B1C1FD8` (break `/Game/FPSKM/Blueprints/Structures/S_DefaultWaveInfo` (`self.CurWaveInfo`))) (`self.CurWaveDeathCharCount`)) (`self.DefenseGameState`))
  ;;[1 1 1] Set Virables for start next wave
  (set `self.CurWaveIndex` (+ (`self.CurWaveIndex`) 1))
  (`KismetArrayLibrary.Array_Clear` (`self.AllSpawnedEnemyAry`))
  (set `self.CurWaveSpawnCount` 0)
  (set `self.CurWaveInfo` (`|GetArrayItem` (`self.WaveInfoAry`) (`self.CurWaveIndex`)))
  (`self.OnStart_Wave_Event` (+ (`self.CurWaveIndex`) 1) (`KismetArrayLibrary.Array_Length` (`self.WaveInfoAry`)))
  (if (`self.IsBossWave` (`self.CurWaveInfo`))
    ;;[1 1 1] Show Next Wave Widget
    (bind _outactors (`GameplayStatics.GetAllActorsOfClass` "/Game/FPSKM/Blueprints/Game/BP_PC_FPS.BP_PC_FPS_C"))
    (for _array_element _outactors
      (`/Game/FPSKM/Blueprints/Game/BP_PC_FPS.OwningClient_StartBossNextWave` _array_element))
    (else
      (bind _outactors_2 (`GameplayStatics.GetAllActorsOfClass` "/Game/FPSKM/Blueprints/Game/BP_PC_FPS.BP_PC_FPS_C"))
      (for _array_element_2 _outactors_2
        (`/Game/FPSKM/Blueprints/Game/BP_PC_FPS.OwningClient_StartNextWave` _array_element_2))))
  ;;[1 1 1] Start Spawn Enemy
  (`self.StartSpawnEnemy`
    (:`NewParam`
      (set `/Game/FPSKM/Blueprints/Game/BP_FPS_GameState.LeftEnemyCount` (- (`.NumberOfEnemies_2_C03758C74F5B1AA87E2C3EBD3B1C1FD8` (break `/Game/FPSKM/Blueprints/Structures/S_DefaultWaveInfo` (`self.CurWaveInfo`))) (`self.CurWaveDeathCharCount`)) (`self.DefenseGameState`)))))

(event `StartWaveEvent`
  (params (IpCurWave :type Integer) (IpMaxWave :type Integer))
  ;[1 1 1] Events - StartWave, OnEnd_Wave, OnStart_Wave, OnFinish_AllWave
  (bind _asbp_fps_game_state (cast `/Game/FPSKM/Blueprints/Game/BP_FPS_GameState` (`GameplayStatics.GetGameState`)))
  (bind _output_get (set `self.DefenseGameState` _asbp_fps_game_state))
  (set `/Game/FPSKM/Blueprints/Game/BP_FPS_GameState.CurWave` IpCurWave _output_get)
  (set `/Game/FPSKM/Blueprints/Game/BP_FPS_GameState.MaxWave` IpMaxWave _output_get))

(event `WaitTimerEvent`
  ;[1 1 1] WaitTimerEvent
  (bind _output_get (set `self.CurWaveWaitTime` (+ (`self.CurWaveWaitTime`) 1.0)))
  (`self.Multi_WaitTimerEvent` _output_get (`self.WaveWaitTime`))
  (if (>= (`self.CurWaveWaitTime`) (`self.WaveWaitTime`))
    (set `self.CurWaveWaitTime` 0.0)
    (`KismetSystemLibrary.K2_ClearAndInvalidateTimerHandle` (`self.WaveWaitTimer`))
    (set `self.IsPlaying` true)
    (`self.StartNextWave`)))

(event `OnEnd_Wave_Event`
  (params (IpCurWave :type Integer) (IpMaxWave :type Integer))
  ;[1 1 1] Events - StartWave, OnEnd_Wave, OnStart_Wave, OnFinish_AllWave
  (bind _asbp_fps_game_state (cast `/Game/FPSKM/Blueprints/Game/BP_FPS_GameState` (`GameplayStatics.GetGameState`)))
  (bind _output_get (set `self.DefenseGameState` _asbp_fps_game_state))
  (set `/Game/FPSKM/Blueprints/Game/BP_FPS_GameState.CurWave` IpCurWave _output_get)
  (set `/Game/FPSKM/Blueprints/Game/BP_FPS_GameState.MaxWave` IpMaxWave _output_get))

(event `Multi_WaitTimerEvent`
  (params (CurWaveWaitTime :type "Float (double-precision)") (WaveWaitTime :type "Float (double-precision)"))
  ;[1 1 1] Multi_WaitTimerEvent
  (bind _asbp_fps_game_state (cast `/Game/FPSKM/Blueprints/Game/BP_FPS_GameState` (`GameplayStatics.GetGameState`)))
  (bind _output_get (set `self.DefenseGameState` _asbp_fps_game_state))
  (set `/Game/FPSKM/Blueprints/Game/BP_FPS_GameState.CurWaveWaitTime` CurWaveWaitTime _output_get)
  (set `/Game/FPSKM/Blueprints/Game/BP_FPS_GameState.WaveWaitTime` WaveWaitTime _output_get))

(event `OnStart_Wave_Event`
  (params (IpCurWave :type Integer) (IpMaxWave :type Integer))
  ;[1 1 1] Events - StartWave, OnEnd_Wave, OnStart_Wave, OnFinish_AllWave
  (bind _asbp_fps_game_state (cast `/Game/FPSKM/Blueprints/Game/BP_FPS_GameState` (`GameplayStatics.GetGameState`)))
  (bind _output_get (set `self.DefenseGameState` _asbp_fps_game_state))
  (set `/Game/FPSKM/Blueprints/Game/BP_FPS_GameState.CurWave` IpCurWave _output_get)
  (set `/Game/FPSKM/Blueprints/Game/BP_FPS_GameState.MaxWave` IpMaxWave _output_get))

(event `OnFinish_AllWave_Event`
  (params (IpCurWave :type Integer) (IpMaxWave :type Integer))
  ;[1 1 1] Events - StartWave, OnEnd_Wave, OnStart_Wave, OnFinish_AllWave
  (bind _asbp_fps_game_state (cast `/Game/FPSKM/Blueprints/Game/BP_FPS_GameState` (`GameplayStatics.GetGameState`)))
  (bind _output_get (set `self.DefenseGameState` _asbp_fps_game_state))
  (set `/Game/FPSKM/Blueprints/Game/BP_FPS_GameState.CurWave` IpCurWave _output_get)
  (set `/Game/FPSKM/Blueprints/Game/BP_FPS_GameState.MaxWave` IpMaxWave _output_get))

(event `/Game/FPSKM/Blueprints/Interfaces/DamageInterface.OnCharDeath`
  (params (IpChar :type "/Game/FPSKM/Blueprints/Characters/BP_BaseChar Object Reference") (IpCHitInfo :type "/Game/FPSKM/Blueprints/Structures/S_C_HitInfo Structure"))
  ;[1 1 1] Event - OnCharDeath
  ;;[1 1 1] Check if IpChar spawned
  (if (`KismetArrayLibrary.Array_Contains` (`self.AllSpawnedEnemyAry`) IpChar)
    (bind _asbp_fps_game_state (cast `/Game/FPSKM/Blueprints/Game/BP_FPS_GameState` (`GameplayStatics.GetGameState`)))
    (set `self.DefenseGameState` _asbp_fps_game_state)
    ;;[1 1 1] add enemy kill count
    (`/Engine/EditorBlueprintResources/StandardMacros.IncrementInt` (`self.CurWaveDeathCharCount`)
      (:`  `
        ;;[1 1 1] Set Left Enemy Count
        (set `/Game/FPSKM/Blueprints/Game/BP_FPS_GameState.LeftEnemyCount` (- (`.NumberOfEnemies_2_C03758C74F5B1AA87E2C3EBD3B1C1FD8` (break `/Game/FPSKM/Blueprints/Structures/S_DefaultWaveInfo` (`self.CurWaveInfo`))) (`self.CurWaveDeathCharCount`)) (`self.DefenseGameState`))))))

(fn `CheckNextWave`
  (returns (Result :type Boolean))
  (for _array_element (`self.AllSpawnedEnemyAry`)
    (`/Engine/EditorBlueprintResources/StandardMacros.IsValid` _array_element
      (:`Is Valid`
        (if (not (`/Game/FPSKM/Blueprints/Characters/BP_BaseChar.IsDeath` _array_element))
          (return false)))))
  (if (<= (- (`.NumberOfEnemies_2_C03758C74F5B1AA87E2C3EBD3B1C1FD8` (break `/Game/FPSKM/Blueprints/Structures/S_DefaultWaveInfo` (`self.CurWaveInfo`))) (`self.CurWaveDeathCharCount`)) 0)
    (return true)
    (else
      (return false))))

(fn `GetRandomSpawnEnemy`
  (params (IpWaveInfo :type "/Game/FPSKM/Blueprints/Structures/S_DefaultWaveInfo Structure"))
  (returns (IsGetSuccess :type Boolean) (EnemyClass :type "/Game/FPSKM/Blueprints/Characters/Enemies/BP_FPS_BaseEnemy Class Reference"))
  (locals (LocalRandomMaxValue :type Integer :default 1) (LocalRandomValue :type Integer :default 0) (LocalCheckSumValue :type Integer :default 1))
  (for _array_element (`.SpawnEnemyInfoAry_24_474453A74D01F0C66483D997C96B104F` (break `/Game/FPSKM/Blueprints/Structures/S_DefaultWaveInfo` (`local.IpWaveInfo`)))
    ;[1 1 1] Set Random Max Value
    (set `local.LocalRandomMaxValue` (+ (`.Percent_6_94B6BDB048B95E4416B67B9A94CE7D6B` (break `/Game/FPSKM/Blueprints/Structures/S_SpawnEnemyPercentInfo` _array_element)) (`local.LocalRandomMaxValue`))))
  ;[1 1 1] Set Random Value
  (set `local.LocalRandomValue` (`KismetMathLibrary.RandomIntegerInRange` 0 (- (`local.LocalRandomMaxValue`) 1)))
  ;[1 1 1] Return Random Enemy Class
  (for _array_element_2 (`.SpawnEnemyInfoAry_24_474453A74D01F0C66483D997C96B104F` (break `/Game/FPSKM/Blueprints/Structures/S_DefaultWaveInfo` (`local.IpWaveInfo`)))
    (bind (_enemyclass _percent) (break `/Game/FPSKM/Blueprints/Structures/S_SpawnEnemyPercentInfo` _array_element_2))
    (set `local.LocalCheckSumValue` (+ _percent (`local.LocalCheckSumValue`)))
    (if (< (`local.LocalRandomValue`) (`local.LocalCheckSumValue`))
      (return true _enemyclass)))
  (return false null))

(fn `IsBossWave`
  (params (IpWaveInfo :type "/Game/FPSKM/Blueprints/Structures/S_DefaultWaveInfo Structure"))
  (returns (ReturnValue :type Boolean))
  (for _array_element (`.SpawnEnemyInfoAry_24_474453A74D01F0C66483D997C96B104F` (break `/Game/FPSKM/Blueprints/Structures/S_DefaultWaveInfo` (`local.IpWaveInfo`)))
    (if (`KismetMathLibrary.ClassIsChildOf` (`.EnemyClass_7_FBCF35684CEB35629C6402838CF23506` (break `/Game/FPSKM/Blueprints/Structures/S_SpawnEnemyPercentInfo` _array_element)))
      (return false)))
  (return false))

(fn `SpawnEnemyFunc`
  (bind ((`SpawnPointInfoAry_20_958C5F6F42A9EA6F5C80978F5FC641E2` _spawnpointinfoary)) (break `/Game/FPSKM/Blueprints/Structures/S_DefaultWaveInfo` (`self.CurWaveInfo`)))
  (bind (_isgetsuccess _enemyclass) (`self.GetRandomSpawnEnemy` (`self.CurWaveInfo`)))
  (set `self.IsPlaying` true)
  ;[1 1 1] Set Random Spawn Point
  (set `self.SelectSpawnPointInfo` (`|GetArrayItem` _spawnpointinfoary (`KismetMathLibrary.RandomIntegerInRange` 0 (- (`KismetArrayLibrary.Array_Length` _spawnpointinfoary) 1))))
  (if _isgetsuccess
    (set `self.SelectSpawnEnemyClass` _enemyclass)
    ;[1 1 1] Spawn a Enemy
    (bind _returnvalue (`|SpawnActorFromClass` (`self.SelectSpawnEnemyClass`) (`/Game/FPSKM/Blueprints/Spanwer/BP_DefaultSpawnPoint.GetRandomSpawnTrm2` (`self.SelectSpawnPointInfo`)) "AdjustIfPossibleButAlwaysSpawn" "OverrideRootScale" null null))
    (`KismetArrayLibrary.Array_Add` (`self.AllSpawnedEnemyAry`) _returnvalue)
    (`/Game/FPSKM/Blueprints/Characters/Enemies/BP_FPS_BaseEnemy.FollowToHero` _returnvalue)
    (set `self.CurWaveSpawnCount` (+ (`self.CurWaveSpawnCount`) 1))
    ;[1 1 1] If All enemy spawned, stop enemy spawn timer
    (if (>= (`self.CurWaveSpawnCount`) (`.NumberOfEnemies_2_C03758C74F5B1AA87E2C3EBD3B1C1FD8` (break `/Game/FPSKM/Blueprints/Structures/S_DefaultWaveInfo` (`self.CurWaveInfo`))))
      (`KismetSystemLibrary.K2_ClearAndInvalidateTimerHandle` (`self.SpawnEnemyTimerHandle`)))))

(fn `UserConstructionScript`)