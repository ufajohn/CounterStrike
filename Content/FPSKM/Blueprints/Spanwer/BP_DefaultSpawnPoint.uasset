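; BP_DefaultSpawnPoint is a spawn point actor that supplies random spawn transforms within its area.
; On construction and BeginPlay it filters nine preset capsules, hiding any that fail a capsule overlap-style trace or a line-of-sight trace from SpawnRadius.
; GetRandomSpawnTrm2 picks a random surviving capsule's transform.
; GetRandomSpawnTrm instead returns a random navigable point within Radius, keeping the actor's rotation and scale.
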(event `self.ReceiveBeginPlay`
  (`self.SettingSpawnPoints`))

(fn `GetRandomSpawnTrm`
  (returns (RandomTrm :type "Transform Structure") (ReturnValue :type Boolean))
  (locals (NewLocalVar_0 :type "NavigationData Object Reference"))
  (return (`KismetMathLibrary.MakeTransform` (`NavigationSystemV1.K2_GetRandomLocationInNavigableRadius` (.location (`self.GetTransform`)) (`self.Radius`) null null) (.rotation (`self.GetTransform`)) (.scale (`self.GetTransform`))) false))

(fn `GetRandomSpawnTrm2`
  (returns (RandomTrm :type "Transform Structure"))
  (locals (NewLocalVar_0 :type "NavigationData Object Reference") (LocalSpawnCapsuleAry :type "Array of CapsuleComponent Object Reference"))
  (return (`SceneComponent.K2_GetComponentToWorld` (`|GetArrayItem` (`self.SpawnCapsuleAry`) (`KismetMathLibrary.RandomIntegerInRange` 0 (- (`KismetArrayLibrary.Array_Length` (`self.SpawnCapsuleAry`)) 1))))))

(fn `SettingSpawnPoints`
  (locals (LocalCapsule :type "CapsuleComponent Object Reference") (LocalSpawnCapsuleAry :type "Array of CapsuleComponent Object Reference"))
  (bind _localcapsule (`local.LocalCapsule`))
  (bind _returnvalue (`SceneComponent.K2_GetComponentLocation` (`local.LocalCapsule`)))
  (`KismetArrayLibrary.Array_Clear` (`self.SpawnCapsuleAry`))
  (bind _output_get (set `local.LocalSpawnCapsuleAry` (`|MakeArray` (`self.SpawnPoint1`) (`self.SpawnPoint2`) (`self.SpawnPoint3`) (`self.SpawnPoint4`) (`self.SpawnPoint5`) (`self.SpawnPoint6`) (`self.SpawnPoint7`) (`self.SpawnPoint8`) (`self.SpawnPoint9`))))
  (for _array_element _output_get
    (bind _output_get_2 (set `local.LocalCapsule` _array_element))
    (`SceneComponent.SetVisibility` _output_get_2 true false)
    (bind (_outhit _returnvalue_2) (`KismetSystemLibrary.CapsuleTraceSingle` _returnvalue (+ _returnvalue (5.0 5.0 0.0)) (`CapsuleComponent.CapsuleRadius` _localcapsule) (`CapsuleComponent.CapsuleHalfHeight` _localcapsule) "TraceTypeQuery1"))
    (if _returnvalue_2
      (`SceneComponent.SetVisibility` (`local.LocalCapsule`) false false :!label _label)
      (else
        (bind (_outhit_2 _returnvalue_3) (`KismetSystemLibrary.LineTraceSingle` (`SceneComponent.K2_GetComponentLocation` (`self.SpawnRadius`)) (`SceneComponent.K2_GetComponentLocation` (`local.LocalCapsule`)) "TraceTypeQuery1"))
        (if _returnvalue_3
          (goto _label)
          (else
            (`KismetArrayLibrary.Array_Add` (`self.SpawnCapsuleAry`) (`local.LocalCapsule`))))))))

(fn `UserConstructionScript`
  (`self.SettingSpawnPoints`))