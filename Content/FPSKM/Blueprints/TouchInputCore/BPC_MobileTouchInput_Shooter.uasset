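; Actor component that provides mobile touch controls for a shooter, attachable to a PlayerController or Pawn.
; On BeginPlay, for a local controller or locally controlled pawn only, it creates the MobileShootingMain widget and adds it to the viewport.
; It forwards touch press, move and release to that widget.
; It binds the widget's movement, look, fire, action, sprint and slot inputs, re-broadcasting them as its own dispatchers.
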(event `self.ReceiveBeginPlay`
  (bind _returnvalue (`self.GetOwner`))
  ;[1 1 1] Event - BeginPlay
  (bind _asplayer_controller (cast `PlayerController` _returnvalue)
    (:`then`
      (if (`Controller.IsLocalPlayerController` _asplayer_controller)
        (`|ExecutionSequence` :!label _label
          (:`then_0`
            ;;[1 1 1] Create Mobile Shooter Main Widget and Add it to Viewport.
            (bind _returnvalue_2 (`|CreateWidget` "/Game/FPSKM/Blueprints/TouchInputCore/Widgets/Widget_MobileShootingMain.Widget_MobileShootingMain_C" (`GameplayStatics.GetPlayerController` 0)))
            (bind _output_get (set `self.MainWidget` _returnvalue_2))
            (`UserWidget.AddToViewport` _output_get 0))
          (:`then_1`
            (`|ExecutionSequence`
              (:`then_0`
                (add `/Game/FPSKM/Blueprints/TouchInputCore/Widgets/Widget_MobileShootingMain.InputTouch Axis MoveForward` (`self.MainWidget`) (delegate `Event Axis MoveForward`))
                (add `/Game/FPSKM/Blueprints/TouchInputCore/Widgets/Widget_MobileShootingMain.InputTouch Axis MoveRight` (`self.MainWidget`) (delegate `Event Axis MoveRight`))
                (add `/Game/FPSKM/Blueprints/TouchInputCore/Widgets/Widget_MobileShootingMain.InputTouch Axis LookUp` (`self.MainWidget`) (delegate `Event Axis LookUp`))
                (add `/Game/FPSKM/Blueprints/TouchInputCore/Widgets/Widget_MobileShootingMain.InputTouch Axis Turn` (`self.MainWidget`) (delegate `Event Axis Turn`))
                (add `/Game/FPSKM/Blueprints/TouchInputCore/Widgets/Widget_MobileShootingMain.InputTouch Axis Fire` (`self.MainWidget`) (delegate `Event Axis Fire`)))
              (:`then_1`
                (add `/Game/FPSKM/Blueprints/TouchInputCore/Widgets/Widget_MobileShootingMain.OnPressed_Button_Fire` (`self.MainWidget`) (delegate `Event OnPressed_Button_Fire`))
                (add `/Game/FPSKM/Blueprints/TouchInputCore/Widgets/Widget_MobileShootingMain.OnReleased_Button_Fire` (`self.MainWidget`) (delegate `Event OnReleased_Button_Fire`))
                (add `/Game/FPSKM/Blueprints/TouchInputCore/Widgets/Widget_MobileShootingMain.OnPressed_Button_Reload` (`self.MainWidget`) (delegate `Event OnPressed_Button_Reload`)))
              (:`then_2`
                (add `/Game/FPSKM/Blueprints/TouchInputCore/Widgets/Widget_MobileShootingMain.OnPressed_Button_Jump` (`self.MainWidget`) (delegate `Event OnPressed_Button_Jump`))
                (add `/Game/FPSKM/Blueprints/TouchInputCore/Widgets/Widget_MobileShootingMain.OnReleased_Button_Jump` (`self.MainWidget`) (delegate `Event OnReleased_Button_Jump`)))
              (:`then_3`
                (add `/Game/FPSKM/Blueprints/TouchInputCore/Widgets/Widget_MobileShootingMain.OnPressed_Button_Crouch` (`self.MainWidget`) (delegate `Event OnPressed_Button_Crouch`))
                (add `/Game/FPSKM/Blueprints/TouchInputCore/Widgets/Widget_MobileShootingMain.OnReleased_Button_Crouch` (`self.MainWidget`) (delegate `Event OnReleased_Button_Crouch`))
                (add `/Game/FPSKM/Blueprints/TouchInputCore/Widgets/Widget_MobileShootingMain.OnPressed_Button_Aim` (`self.MainWidget`) (delegate `Event OnPressed_Button_Aim`)))
              (:`then_4`
                (add `/Game/FPSKM/Blueprints/TouchInputCore/Widgets/Widget_MobileShootingMain.OnStart_SprintInput` (`self.MainWidget`) (delegate `Event OnStart_SprintInput`))
                (add `/Game/FPSKM/Blueprints/TouchInputCore/Widgets/Widget_MobileShootingMain.OnEnd_SprintInput` (`self.MainWidget`) (delegate `Event OnEnd_SprintInput`))
                (add `/Game/FPSKM/Blueprints/TouchInputCore/Widgets/Widget_MobileShootingMain.OnPressed_Button_Pickup` (`self.MainWidget`) (delegate `Event OnPressed_Button_Pickup`)))
              (:`then_5`
                (add `/Game/FPSKM/Blueprints/TouchInputCore/Widgets/Widget_MobileShootingMain.OnPressed_Button_WeaponSlot1` (`self.MainWidget`) (delegate `Event OnPressed_Button_WeaponSlot1`))
                (add `/Game/FPSKM/Blueprints/TouchInputCore/Widgets/Widget_MobileShootingMain.OnPressed_Button_WeaponSlot2` (`self.MainWidget`) (delegate `Event OnPressed_Button_WeaponSlot2`)))
              (:`then_6`
                (add `/Game/FPSKM/Blueprints/TouchInputCore/Widgets/Widget_MobileShootingMain.OnPressed_Button_GrenadeSlot` (`self.MainWidget`) (delegate `Event OnPressed_Button_GrenadeSlot`))))))))
    (:`CastFailed`
      (bind _aspawn (cast `Pawn` _returnvalue))
      (if (`Pawn.IsLocallyControlled` _aspawn)
        (goto _label)))))

(event `Event Axis MoveForward`
  (params (AxisValue :type "Float (double-precision)") (JoystickAngle :type "Float (double-precision)") (JoystickMoveLength :type "Float (double-precision)"))
  ;[1 1 1] Event - BeginPlay
  (`self.InputTouch Axis MoveForward` AxisValue JoystickAngle JoystickMoveLength))

(event `Event Axis MoveRight`
  (params (AxisValue :type "Float (double-precision)"))
  ;[1 1 1] Event - BeginPlay
  (`self.InputTouch Axis MoveRight` AxisValue))

(event `Event Axis LookUp`
  (params (AxisValue :type "Float (double-precision)"))
  ;[1 1 1] Event - BeginPlay
  (`self.InputTouch Axis LookUp` AxisValue))

(event `Event Axis Turn`
  (params (AxisValue :type "Float (double-precision)"))
  ;[1 1 1] Event - BeginPlay
  (`self.InputTouch Axis Turn` AxisValue))

(event `Event Axis Fire`
  ;[1 1 1] Event - BeginPlay
  (`self.InputTouch Axis Fire`))

(event `Event OnPressed_Button_Fire`
  ;[1 1 1] Event - BeginPlay
  (`self.OnPressed Button Fire`))

(event `Event OnReleased_Button_Fire`
  ;[1 1 1] Event - BeginPlay
  (`self.OnReleased Button Fire`))

(event `Event OnPressed_Button_Reload`
  ;[1 1 1] Event - BeginPlay
  (`self.OnPressed Button Reload`))

(event `Event OnPressed_Button_Jump`
  ;[1 1 1] Event - BeginPlay
  (`self.OnPressed Button Jump`))

(event `Event OnPressed_Button_Crouch`
  ;[1 1 1] Event - BeginPlay
  (`self.OnPressed Button Crouch`))

(event `Event OnPressed_Button_Aim`
  ;[1 1 1] Event - BeginPlay
  (`self.OnPressed Button Aim`))

(event `Event OnReleased_Button_Jump`
  ;[1 1 1] Event - BeginPlay
  (`self.OnReleased Button Jump`))

(event `Event OnReleased_Button_Crouch`
  ;[1 1 1] Event - BeginPlay
  (`self.OnReleased Button Crouch`))

(event `Event OnStart_SprintInput`
  ;[1 1 1] Event - BeginPlay
  (`self.OnStart Sprint Input`))

(event `Event OnEnd_SprintInput`
  ;[1 1 1] Event - BeginPlay
  (`self.OnEnd Sprint Input`))

(event `Event OnPressed_Button_Pickup`
  ;[1 1 1] Event - BeginPlay
  (`self.OnPressed Button Pickup`))

(event `Event OnPressed_Button_WeaponSlot1`
  ;[1 1 1] Event - BeginPlay
  (`self.OnPressed Button WeaponSlot1`))

(event `Event OnPressed_Button_WeaponSlot2`
  ;[1 1 1] Event - BeginPlay
  (`self.OnPressed Button WeaponSlot2`))

(event `Event OnPressed_Button_GrenadeSlot`
  (params (IpSlotIndex :type Integer))
  ;[1 1 1] Event - BeginPlay
  (`self.OnPressed_Button_GrenadeSlot` IpSlotIndex))

(event `/Game/FPSKM/Blueprints/TouchInputCore/TouchInputInterface.OnPressed_InputTouch`
  (params (Location :type "Vector Structure") (FingerIndex :type Byte))
  ;[1 1 1] Input Touch Events
  (`/Game/FPSKM/Blueprints/TouchInputCore/TouchInputInterface.OnPressed_InputTouch` (`self.MainWidget`) Location FingerIndex))

(event `/Game/FPSKM/Blueprints/TouchInputCore/TouchInputInterface.OnReleased_InputTouch`
  (params (Location :type "Vector Structure") (FingerIndex :type Byte))
  ;[1 1 1] Input Touch Events
  (`/Game/FPSKM/Blueprints/TouchInputCore/TouchInputInterface.OnReleased_InputTouch` (`self.MainWidget`) Location FingerIndex))

(event `/Game/FPSKM/Blueprints/TouchInputCore/TouchInputInterface.OnMoved_InputTouch`
  (params (Location :type "Vector Structure") (FingerIndex :type Byte))
  ;[1 1 1] Input Touch Events
  (`/Game/FPSKM/Blueprints/TouchInputCore/TouchInputInterface.OnMoved_InputTouch` (`self.MainWidget`) Location FingerIndex))