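; BP_BaseInteractItem is a base Blueprint for interactable items, providing a highlight toggle.
; It has a static mesh component and a skeletal mesh component.
; HighLight switches Render Custom Depth on the static mesh if a mesh asset is assigned, otherwise on the skeletal mesh if that has one.
; The construction script is empty, and no interaction logic is defined here.
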(fn `HighLight`
  (params (InputIsHighLight :type Boolean))
  (`/Engine/EditorBlueprintResources/StandardMacros.IsValid` (`StaticMeshComponent.StaticMesh` (`self.StaticMesh`))
    (:`Is Valid`
      (`PrimitiveComponent.SetRenderCustomDepth` (`self.StaticMesh`) (`local.InputIsHighLight`)))
    (:`Is Not Valid`
      (`/Engine/EditorBlueprintResources/StandardMacros.IsValid` (`SkinnedMeshComponent.SkeletalMesh` (`self.SkeletalMesh`))
        (:`Is Valid`
          (`PrimitiveComponent.SetRenderCustomDepth` (`self.SkeletalMesh`) (`local.InputIsHighLight`)))))))

(fn `UserConstructionScript`)