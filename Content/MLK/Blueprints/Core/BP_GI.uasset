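; Game Instance that manages multiplayer sessions, map travel and error reporting, and applies the base sound mix on init.
; It hosts a listen-server lobby from stored match settings and broadcasts session search results through a delegate.
; Server travel multicasts a warning, then passes settings as URL options, using DataTable lookups and capping MaxPlayers to the current count for matches.
; Network and travel errors queue up for display in chained dialog boxes.
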(event `self.ReceiveInit`
  ;[1 1 1] Project has no sounds, but we still set and push the SoundMix modifier in case you wish to use the already existing soundclasses
  (`GameplayStatics.SetBaseSoundMix` "/Game/MLK/Audio/SoundClasses/SM_Main.SM_Main")
  (`GameplayStatics.PushSoundMixModifier` "/Game/MLK/Audio/SoundClasses/SM_Main.SM_Main"))

(event `HostMatch`
  (bind _currentmatchsettings (`self.CurrentMatchSettings`))
  (bind ((`GameMode_23_0FC75F574F0BB05B36C23997982B5EF0` _gamemode) (`NextMap_18_5D862F524A41C8398926368742F5047C` _nextmap) (`MatchTime_24_19A1859244E7184C85868DB74EC103FD` _matchtime)) (break `/Game/MLK/Blueprints/Structs/FMatchSettings` _currentmatchsettings))
  (bind ((`MaxPlayers_22_5E2B5EE64D3DE00128638F99F43DDC71` _maxplayers) (`bIsLanMatch_21_42018E5D4C57A99B98C34B9FC9778845` _bislanmatch)) (break `/Game/MLK/Blueprints/Structs/FMatchSettings` _currentmatchsettings))
  ;[1 1 1] HOST MATCH | Create a Session using the current settings, as well as opening the Lobby, passing over all additional settings, like GameMode.
  (`CreateSessionCallbackProxy.CreateSession` (`GameplayStatics.GetPlayerController` 0) _maxplayers _bislanmatch
    (:`OnSuccess`
      (`GameplayStatics.OpenLevel` "Map_Lobby" true (`KismetStringLibrary.Concat_StrStr` "listen" "?GameMode=" _gamemode "?Map=" _nextmap "?MatchTime=" (`KismetStringLibrary.Conv_IntToString` _matchtime))))))

(event `FindMatch`
  (bind (_numresults _blan) (break `/Game/MLK/Blueprints/Structs/FFindMatchSettings` (`self.CurrentFindMatchSettings`)))
  ;[1 1 1] FIND MATCH | If we aren't already finding a Match, search with the current settings. After that, notify everyone who is listening to the OnFindMatchComplete Delegate.
  (if (not (`self.bIsFindingMatch`))
    (bind _results (`FindSessionsCallbackProxy.FindSessions` (`GameplayStatics.GetPlayerController` 0) _numresults _blan)
      (:`then`
        (set `self.bIsFindingMatch` true))
      (:`OnSuccess`
        (`self.OnFindMatchComplete` true _results)
        (set `self.bIsFindingMatch` false))
      (:`OnFailure`
        (`self.OnFindMatchComplete` false (`|MakeArray` (struct) :!type "BlueprintSessionResult Structure"))
        (set `self.bIsFindingMatch` false)))))

(event `self.HandleNetworkError`
  (params (FailureType :type "ENetworkFailure Enum" :default "NetDriverAlreadyExists") (bIsServer :type Boolean))
  ;[1 1 1] ERROR HANDLING | Since errors happen between all traveling, we need to keep track of them by adding them to an array.
  ; Once we want to know if there are any pending errors, we can query these and display them.
  (`KismetArrayLibrary.Array_Add` (`self.PendingErrors`) (`KismetTextLibrary.Conv_StringToText` (`|GetEnumeratorNameAsString` FailureType))))

(event `self.HandleTravelError`
  (params (FailureType :type "ETravelFailure Enum" :default "NoLevel"))
  ;[1 1 1] ERROR HANDLING | Since errors happen between all traveling, we need to keep track of them by adding them to an array.
  ; Once we want to know if there are any pending errors, we can query these and display them.
  (`KismetArrayLibrary.Array_Add` (`self.PendingErrors`) (`KismetTextLibrary.Conv_StringToText` (`|GetEnumeratorNameAsString` FailureType))))

(event `TryShowPendingError`
  ;[1 1 1] ERROR HANDLING | Since errors happen between all traveling, we need to keep track of them by adding them to an array.
  ; Once we want to know if there are any pending errors, we can query these and display them.
  (if (> (`KismetArrayLibrary.Array_Length` (`self.PendingErrors`)) 0)
    (bind _returnvalue (`|CreateWidget` "/Game/MLK/Widgets/Core/WB_DialogBox.WB_DialogBox_C" (`GameplayStatics.GetPlayerController` 0)))
    (`/Game/MLK/Widgets/Core/WB_DialogBox.SetupDialog` _returnvalue "ERROR" (`|GetArrayItem` (`self.PendingErrors`)) "OKAY" false "NO")
    (add `/Game/MLK/Widgets/Core/WB_DialogBox.OnLeftButtonClicked` _returnvalue (`|CreateDelegate` :!event `OnErrorDialogOkay`))
    (`KismetArrayLibrary.Array_Remove` (`self.PendingErrors`))))

(event `OnErrorDialogOkay`
  ;[1 1 1] ERROR HANDLING | Since errors happen between all traveling, we need to keep track of them by adding them to an array.
  ; Once we want to know if there are any pending errors, we can query these and display them.
  (`self.TryShowPendingError`))

(fn `ServerTravelToLobby`
  (bind ((`GameMode_23_0FC75F574F0BB05B36C23997982B5EF0` _gamemode) (`NextMap_18_5D862F524A41C8398926368742F5047C` _nextmap) (`MaxPlayers_22_5E2B5EE64D3DE00128638F99F43DDC71` _maxplayers) (`MatchTime_24_19A1859244E7184C85868DB74EC103FD` _matchtime)) (break `/Game/MLK/Blueprints/Structs/FMatchSettings` (`self.CurrentMatchSettings`)))
  ;[1 1 1] When traveling to the Lobby, notify everyone in the game that we are about to move. Then "ServerTravel" back to the lobby.
  (bind _asbp_gs_base (cast `/Game/MLK/Blueprints/GameModes/Base/Core/BP_GS_Base` (`GameplayStatics.GetGameState`)))
  (`/Game/MLK/Blueprints/GameModes/Base/Core/BP_GS_Base.Multicast_OnTravel` _asbp_gs_base)
  (`KismetSystemLibrary.ExecuteConsoleCommand` (`KismetStringLibrary.Concat_StrStr` "ServerTravel Map_Lobby" "?game=Lobby" "?GameMode=" _gamemode "?Map=" _nextmap "?MaxPlayers=" (`KismetStringLibrary.Conv_IntToString` _maxplayers) "?MatchTime=" (`KismetStringLibrary.Conv_IntToString` _matchtime)) null))

(fn `ServerTravelToNextMap`
  (bind _currentmatchsettings (`self.CurrentMatchSettings`))
  (bind ((`GameMode_23_0FC75F574F0BB05B36C23997982B5EF0` _gamemode) (`MatchTime_24_19A1859244E7184C85868DB74EC103FD` _matchtime)) (break `/Game/MLK/Blueprints/Structs/FMatchSettings` _currentmatchsettings))
  ;[1 1 1] Notify everyone that we are about to travel to a new level.
  (bind _asbp_gs_base (cast `/Game/MLK/Blueprints/GameModes/Base/Core/BP_GS_Base` (`GameplayStatics.GetGameState`)))
  (`/Game/MLK/Blueprints/GameModes/Base/Core/BP_GS_Base.Multicast_OnTravel` _asbp_gs_base)
  ;[1 1 1] Update the MaxPlayer value, so that no additional Players can join (e.g. hosted for 4 players, but only 3 actually joined the Lobby). Then ServerTravel to the next map.
  (bind _returnvalue (`GameModeBase.GetNumPlayers` (`GameplayStatics.GetGameMode`)))
  (bind _returnvalue_2 (`|GetDataTableRow` "/Game/MLK/Blueprints/Data/DT_GameModeData.DT_GameModeData" (`KismetStringLibrary.Conv_StringToName` (`.GameMode_23_0FC75F574F0BB05B36C23997982B5EF0` (break `/Game/MLK/Blueprints/Structs/FMatchSettings` (`self.CurrentMatchSettings`)))))
    (:`then`
      (bind _returnvalue_3 (`|GetDataTableRow` "/Game/MLK/Blueprints/Data/DT_MapData.DT_MapData" (`KismetStringLibrary.Conv_StringToName` (`.NextMap_18_5D862F524A41C8398926368742F5047C` (break `/Game/MLK/Blueprints/Structs/FMatchSettings` _currentmatchsettings))))
        (:`then`
          (`KismetSystemLibrary.ExecuteConsoleCommand` (`KismetStringLibrary.Concat_StrStr` "ServerTravel " (`.AssetName_5_F28B2DC249049ECAC01B02B4BCA5758E` (break `/Game/MLK/Blueprints/Structs/FMapData` _returnvalue_3)) "?GameMode=" _gamemode "?MatchTime=" (`KismetStringLibrary.Conv_IntToString` _matchtime) "?game=" (`.GameModeShortCode_9_BBFE5B0C491E1670E892B38DD11F79E9` (break `/Game/MLK/Blueprints/Structs/FGameModeData` _returnvalue_2)) "?MaxPlayers=" (`KismetStringLibrary.Conv_IntToString` _returnvalue) "?Map=" (`.NextMap_18_5D862F524A41C8398926368742F5047C` (break `/Game/MLK/Blueprints/Structs/FMatchSettings` (`self.CurrentMatchSettings`)))) null))))))

(fn `SetFindMatchSettings`
  (params (FindMatchSettings :type "/Game/MLK/Blueprints/Structs/FFindMatchSettings Structure"))
  (set `self.CurrentFindMatchSettings` FindMatchSettings))

(fn `SetHostMatchSettings`
  (params (HostMatchSettings :type "/Game/MLK/Blueprints/Structs/FMatchSettings Structure"))
  (set `self.CurrentMatchSettings` HostMatchSettings))