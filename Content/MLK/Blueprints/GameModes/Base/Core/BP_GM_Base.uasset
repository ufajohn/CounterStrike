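; Base GameMode that carries match settings between levels and assigns players to teams.
; On BeginPlay it parses match time, mode and map from the options string, looks up team-based status in DT_GameModeData, and mirrors all to BP_GS_Base for replication.
; New logins join the smaller team, or team 0 in free-for-all.
; Seamless travel copies TeamID and cosmetic selections from old to new PlayerController.
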(event `self.ReceiveBeginPlay`
  ;[1 1 1] BEGIN PLAY | Receive all passed Options from the previous Level and initialize the GameState.
  (`self.ReceiveOptions`)
  (`self.SetupGameState`))

(event `self.K2_OnSwapPlayerControllers`
  (params (OldPC :type "PlayerController Object Reference") (NewPC :type "PlayerController Object Reference"))
  ;[1 1 1] ON SWAP PLAYERCONTROLLERS | Called after a Seamless Travel to swap from old to new PC.
  ; This allows moving data from old to new PC.
  (`self.HandleSeamlessPlayer` OldPC NewPC))

(event `self.K2_PostLogin`
  (params (NewPlayer :type "PlayerController Object Reference"))
  ;[1 1 1] ON POST LOGIN | Called when a new Player joins (non-seamless).
  ; This allows for the first connection to be handled.
  (`self.HandleNewPlayer` NewPlayer))

(fn `AssignTeamToPlayer`
  (params (Player :type "/Game/MLK/Blueprints/GameModes/Base/Player/BP_PC_Base Object Reference"))
  ;[1 1 1] Get the best team for the passed player and set the TeamID to the PlayerController.
  (`/Engine/EditorBlueprintResources/StandardMacros.IsValid` Player
    (:`Is Valid`
      (bind _asbp_ps_base (cast `/Game/MLK/Blueprints/GameModes/Base/Player/BP_PS_Base` (`Controller.PlayerState` Player)))
      (bind _teamid (`self.GetAppropriateTeam` _asbp_ps_base))
      (`/Game/MLK/Blueprints/GameModes/Base/Player/BP_PC_Base.SetTeamID` (`local.Player`) _teamid))))

(fn `GetAppropriateTeam`
  (params (Player :type "/Game/MLK/Blueprints/GameModes/Base/Player/BP_PS_Base Object Reference"))
  (returns (TeamID :type Byte))
  (bind _player (`local.Player`))
  (bind _teamid (`/Game/MLK/Blueprints/GameModes/Base/Player/BP_PS_Base.TeamID` _player))
  ;[1 1 1] Check if this GameMode is a TeamBased one. If not, we just return the FFA Team.
  (if (`self.bTeamBased`)
    ;[1 1 1] Check if the Player already has a team. This happens when moving back and forth between Lobby and Gameplay Levels. 0 = FFA = NO TEAM. In case they do have a team, just return that.
    (`/Engine/EditorBlueprintResources/StandardMacros.IsValid` _player
      (:`Is Valid`
        (if (== 0 _teamid)
          ;[1 1 1] Once we reach this point, we want to find a team. We ask the GameState for the TeamBalance and check which team has less players.
          (bind _asbp_gs_base (cast `/Game/MLK/Blueprints/GameModes/Base/Core/BP_GS_Base` (`GameplayStatics.GetGameState`))
            (:`then`
              (bind _teambalance (`/Game/MLK/Blueprints/GameModes/Base/Core/BP_GS_Base.GetTeamBalance` _asbp_gs_base))
              (return (select `bool` (> (`BlueprintMapLibrary.Map_Find` _teambalance 1) (`BlueprintMapLibrary.Map_Find` _teambalance 2)) :`false` 1 :`true` 2 :!type "Byte")))
            (:`CastFailed`
              (return 0)))
          (else
            (return _teamid))))
      (:`Is Not Valid`
        _)))
  ;[1 1 1] 0 = FFA or No Team
  (return 0))

(fn `HandleNewPlayer`
  (params (NewPlayer :type "PlayerController Object Reference"))
  ;[1 1 1] Assign a Team to the new Player.
  (bind _asbp_pc_base (cast `/Game/MLK/Blueprints/GameModes/Base/Player/BP_PC_Base` NewPlayer))
  (`self.AssignTeamToPlayer` _asbp_pc_base))

(fn `HandleSeamlessPlayer`
  (params (OldPC :type "PlayerController Object Reference") (NewPC :type "PlayerController Object Reference"))
  (locals (LocalNewPC :type "/Game/MLK/Blueprints/GameModes/Base/Player/BP_PC_Base Object Reference") (LocalOldPC :type "/Game/MLK/Blueprints/GameModes/Base/Player/BP_PC_Base Object Reference"))
  (`|ExecutionSequence`
    (:`then_0`
      (bind _asbp_pc_base (cast `/Game/MLK/Blueprints/GameModes/Base/Player/BP_PC_Base` (`local.NewPC`)))
      (set `local.LocalNewPC` _asbp_pc_base))
    (:`then_1`
      (bind _asbp_pc_base_2 (cast `/Game/MLK/Blueprints/GameModes/Base/Player/BP_PC_Base` (`local.OldPC`)))
      (set `local.LocalOldPC` _asbp_pc_base_2))
    (:`then_2`
      ;[1 1 1] Take all the selections over to the next GameMode.
      (set `/Game/MLK/Blueprints/GameModes/Base/Player/BP_PC_Base.SelectedPawn` (`/Game/MLK/Blueprints/GameModes/Base/Player/BP_PC_Base.SelectedPawn` (`local.LocalOldPC`)) (`local.LocalNewPC`))
      (set `/Game/MLK/Blueprints/GameModes/Base/Player/BP_PC_Base.SelectedHat` (`/Game/MLK/Blueprints/GameModes/Base/Player/BP_PC_Base.SelectedHat` (`local.LocalOldPC`)) (`local.LocalNewPC`))
      (set `/Game/MLK/Blueprints/GameModes/Base/Player/BP_PC_Base.SelectedBodyColor` (`/Game/MLK/Blueprints/GameModes/Base/Player/BP_PC_Base.SelectedBodyColor` (`local.LocalOldPC`)) (`local.LocalNewPC`))
      (set `/Game/MLK/Blueprints/GameModes/Base/Player/BP_PC_Base.SelectedLogoColor` (`/Game/MLK/Blueprints/GameModes/Base/Player/BP_PC_Base.SelectedLogoColor` (`local.LocalOldPC`)) (`local.LocalNewPC`))
      (set `/Game/MLK/Blueprints/GameModes/Base/Player/BP_PC_Base.SelectedHatColor` (`/Game/MLK/Blueprints/GameModes/Base/Player/BP_PC_Base.SelectedHatColor` (`local.LocalOldPC`)) (`local.LocalNewPC`)))
    (:`then_3`
      ;[1 1 1] Transfer the TeamID from old to new PC.
      (`/Game/MLK/Blueprints/GameModes/Base/Player/BP_PC_Base.SetTeamID` (`local.LocalNewPC`) (`/Game/MLK/Blueprints/GameModes/Base/Player/BP_PC_Base.TeamID` (`local.LocalOldPC`))))))

(fn `IsGameModeTeamBased`
  (params (GameMode :type String))
  (returns (bTeamBased :type Boolean))
  (bind _returnvalue (`|GetDataTableRow` "/Game/MLK/Blueprints/Data/DT_GameModeData.DT_GameModeData" (`KismetStringLibrary.Conv_StringToName` GameMode))
    (:`then`
      (return (`.bTeamBased_15_7588C7BD426AE88F59B32AA91C3ADC13` (break `/Game/MLK/Blueprints/Structs/FGameModeData` _returnvalue))))
    (:`RowNotFound`
      (return false))))

(fn `ReceiveOptions`
  ;[1 1 1] Retrieves all required information from the OptionsString, which where passed from the previous level on levelchange.
  (`self.SetMatchTime` (`GameplayStatics.GetIntOption` (`self.OptionsString`) "MatchTime"))
  (bind _output_get (set `self.GameMode` (`GameplayStatics.ParseOption` (`self.OptionsString`) "GameMode")))
  (`self.SetTeamBased` (`self.IsGameModeTeamBased` _output_get))
  (set `self.Map` (`GameplayStatics.ParseOption` (`self.OptionsString`) "Map")))

(fn `SetGameMode`
  (params (InGameMode :type String))
  (set `self.GameMode` InGameMode))

(fn `SetMap`
  (params (InMap :type String))
  (set `self.Map` InMap))

(fn `SetMatchTime`
  (params (MatchTime :type Integer))
  (set `self.MatchTime` MatchTime))

(fn `SetTeamBased`
  (params (bTeamBased :type Boolean))
  ;[1 1 1] Update the TeamBased variable and inform the GameState about the change.
  (set `self.bTeamBased` bTeamBased)
  (bind _asbp_gs_base (cast `/Game/MLK/Blueprints/GameModes/Base/Core/BP_GS_Base` (`GameplayStatics.GetGameState`)))
  (set `/Game/MLK/Blueprints/GameModes/Base/Core/BP_GS_Base.bTeamBased` (`self.bTeamBased`) _asbp_gs_base))

(fn `SetupGameState`
  ;[1 1 1] This informs the GameState about variables which it needs to replicate, since the GameMode can't do this.
  ; You usually do this with all settings that the Player needs to know about. E.g. TeamBased drives the lobby UI.
  (`|ExecutionSequence`
    (:`then_0`
      (bind _asbp_gs_base (cast `/Game/MLK/Blueprints/GameModes/Base/Core/BP_GS_Base` (`GameplayStatics.GetGameState`)))
      (set `/Game/MLK/Blueprints/GameModes/Base/Core/BP_GS_Base.bTeamBased` (`self.bTeamBased`) _asbp_gs_base)
      (set `/Game/MLK/Blueprints/GameModes/Base/Core/BP_GS_Base.MatchTime` (`self.MatchTime`) _asbp_gs_base))
    (:`then_1`
      (bind _asbp_gs_base_2 (cast `/Game/MLK/Blueprints/GameModes/Base/Core/BP_GS_Base` (`GameplayStatics.GetGameState`)))
      (set `/Game/MLK/Blueprints/GameModes/Base/Core/BP_GS_Base.GameMode` (`self.GameMode`) _asbp_gs_base_2))
    (:`then_2`
      (bind _asbp_gs_base_3 (cast `/Game/MLK/Blueprints/GameModes/Base/Core/BP_GS_Base` (`GameplayStatics.GetGameState`)))
      (set `/Game/MLK/Blueprints/GameModes/Base/Core/BP_GS_Base.Map` (`self.Map`) _asbp_gs_base_3))))

(fn `UpdateGameMode`
  (params (InGameMode :type String))
  ;[1 1 1] Updates the GameMode and passes the information to the GameState, so everyone can see it. In addition also determines the new TeamBased state.
  (`self.SetGameMode` InGameMode)
  (bind _asbp_gs_base (cast `/Game/MLK/Blueprints/GameModes/Base/Core/BP_GS_Base` (`GameplayStatics.GetGameState`)))
  (set `/Game/MLK/Blueprints/GameModes/Base/Core/BP_GS_Base.GameMode` (`self.GameMode`) _asbp_gs_base)
  (`self.SetTeamBased` (`self.IsGameModeTeamBased` (`self.GameMode`))))

(fn `UpdateMap`
  (params (InMap :type String))
  (`self.SetMap` InMap)
  (bind _asbp_gs_base (cast `/Game/MLK/Blueprints/GameModes/Base/Core/BP_GS_Base` (`GameplayStatics.GetGameState`)))
  (set `/Game/MLK/Blueprints/GameModes/Base/Core/BP_GS_Base.Map` (`self.Map`) _asbp_gs_base))

(fn `UpdateMatchTime`
  (params (MatchTime :type Integer))
  ;[1 1 1] Set the new MatchTime and inform the GameState about the change.
  (`self.SetMatchTime` MatchTime)
  (bind _asbp_gs_base (cast `/Game/MLK/Blueprints/GameModes/Base/Core/BP_GS_Base` (`GameplayStatics.GetGameState`)))
  (set `/Game/MLK/Blueprints/GameModes/Base/Core/BP_GS_Base.MatchTime` (`self.MatchTime`) _asbp_gs_base))

(fn `UserConstructionScript`)