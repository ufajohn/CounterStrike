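; Base GameState Blueprint that provides shared match state and hooks for child game states.
; A travel multicast has the local player controller clean up its UI before a map change.
; GetTeamBalance tallies players per TeamID from PlayerArray into a map.
; MatchTime and GameMode OnRep functions forward to empty Impl functions, working around a bug that prevents overriding OnReps in children.
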(event `Multicast_OnTravel`
  ;[1 1 1] MULTICAST ON TRAVEL | Inform everyone that we are about the travel, so they can cleanup their UI
  (bind _asbp_pc_base (cast `/Game/MLK/Blueprints/GameModes/Base/Player/BP_PC_Base` (`GameplayStatics.GetPlayerController` 0)))
  (`/Game/MLK/Blueprints/GameModes/Base/Player/BP_PC_Base.CleanUpUI` _asbp_pc_base))

(fn `GetTeamBalance`
  (returns (TeamBalance :type "Map of Byte to Integer"))
  (locals (CurrentTeamBalance :type "Map of Byte to Object Object Reference") (CurrentTeamID :type Byte :default 0))
  (bind (_value _returnvalue) (`BlueprintMapLibrary.Map_Find` (`local.CurrentTeamBalance`) (`local.CurrentTeamID`)))
  ;[1 1 1] Create a Map of Teams and the amount of players per team.
  (for _array_element (`self.PlayerArray`)
    (bind _asbp_ps_base (cast `/Game/MLK/Blueprints/GameModes/Base/Player/BP_PS_Base` _array_element))
    (set `local.CurrentTeamID` (`/Game/MLK/Blueprints/GameModes/Base/Player/BP_PS_Base.TeamID` _asbp_ps_base))
    (`BlueprintMapLibrary.Map_Add` (`local.CurrentTeamBalance`) (`local.CurrentTeamID`) (select `bool` _returnvalue :`false` 1 :`true` (+ _value 1))))
  (return (`local.CurrentTeamBalance`)))

(fn `OnRep_GameMode`
  (`self.OnRep_GameMode_Impl`))

(fn `OnRep_GameMode_Impl`)

(fn `OnRep_MatchTime`
  ;[1 1 1] Workaround of the "Can't override OnRep functions" - Bug
  (`self.OnRep_MatchTime_Impl`))

(fn `OnRep_MatchTime_Impl`)

(fn `UserConstructionScript`)