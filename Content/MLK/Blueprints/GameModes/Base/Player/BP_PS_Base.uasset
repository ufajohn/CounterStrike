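; Base PlayerState that holds a player's selected pawn class and team ID, sharing what other clients cannot read from the PlayerController.
; On BeginPlay the server copies the pawn class from BP_PC_Base, and TeamID carries over through seamless travel and reconnects.
; SwitchTeam flips between teams 1 and 2, updates the controller and forwards client calls to the server.
; The pawn-class OnRep delegates to an empty Impl function, working around children being unable to override OnReps.
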(event `self.ReceiveBeginPlay`
  (`/Engine/EditorBlueprintResources/ActorMacros.Switch Has Authority`
    (:`Authority`
      ;[1 1 1] PlayerState should get created in the PlayerController. So we can already access it and retrieve the PawnClass.
      ; Reason to do this is, that the PlayerController doesn't exist on other Players, so we use the PlayerState to share the information.
      (bind _asbp_pc_base (cast `/Game/MLK/Blueprints/GameModes/Base/Player/BP_PC_Base` (`self.GetOwner`)))
      (set `self.SelectedPawn` (`/Game/MLK/Blueprints/GameModes/Base/Player/BP_PC_Base.SelectedPawn` _asbp_pc_base)))))

(event `self.ReceiveCopyProperties`
  (params (NewPlayerState :type "PlayerState Object Reference"))
  ;[1 1 1] COPY PROPERTIES | In case we Seamless ServerTravel or reconnect, retrieve the previous TeamID.
  (bind _asbp_ps_base (cast `/Game/MLK/Blueprints/GameModes/Base/Player/BP_PS_Base` NewPlayerState))
  (set `/Game/MLK/Blueprints/GameModes/Base/Player/BP_PS_Base.TeamID` (`self.TeamID`) _asbp_ps_base))

(event `self.ReceiveOverrideWith`
  (params (OldPlayerState :type "PlayerState Object Reference"))
  ;[1 1 1] COPY PROPERTIES | In case we Seamless ServerTravel or reconnect, retrieve the previous TeamID.
  (bind _asbp_ps_base (cast `/Game/MLK/Blueprints/GameModes/Base/Player/BP_PS_Base` OldPlayerState))
  (set `self.TeamID` (`/Game/MLK/Blueprints/GameModes/Base/Player/BP_PS_Base.TeamID` _asbp_ps_base)))

(event `SwitchTeam`
  ;[1 1 1] SWITCH TEAM | Updates the TeamID.
  (set `self.TeamID` (- 3 (`self.TeamID`)))
  (bind _asbp_pc_base (cast `/Game/MLK/Blueprints/GameModes/Base/Player/BP_PC_Base` (`self.GetOwner`)))
  (`/Game/MLK/Blueprints/GameModes/Base/Player/BP_PC_Base.SetTeamID` _asbp_pc_base (`self.TeamID`))
  (`/Engine/EditorBlueprintResources/ActorMacros.Switch Has Authority`
    (:`Remote`
      (`self.Server_SwitchTeam`))))

(event `Server_SwitchTeam`
  ;[1 1 1] SWITCH TEAM | Updates the TeamID.
  (`self.SwitchTeam`))

(fn `OnRep_PawnClass`
  ;[1 1 1] We can't override OnRep functions in children. So we have to workaround this bug.
  ;
  ; https://issues.unrealengine.com/issue/UE-55600
  (`self.OnRep_PawnClass_Impl`))

(fn `OnRep_PawnClass_Impl`)

(fn `SetTeamID`
  (params (TeamID :type Byte))
  (set `self.TeamID` TeamID))

(fn `UserConstructionScript`)