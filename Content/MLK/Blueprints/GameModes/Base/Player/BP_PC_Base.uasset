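; Base player controller that holds each player's team and character customization (pawn, hat, colors) and provides overridable UI setup and cleanup hooks.
; Customization setters apply values locally, then send them through Server events to set the RepNotify variables for replication.
; OnReps forward to empty Impl functions so children can override them, working around an engine bug.
; SetTeamID copies the team to the PlayerState and forces a net update.
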(event `self.ReceiveBeginPlay`
  ;[1 1 1] BEGIN PLAY | Setup the UI for the Local Player.
  (if (`self.IsLocalPlayerController`)
    (`self.SetupUI`)))

(event `Server_SetSelectedPawn`
  (params (SelectedPawn :type Name))
  ;[1 1 1] SERVER CALLS FOR CUSTOMIZATION.
  ; Sets all RepNotify variables on the Server for replication.
  (set `self.SelectedPawn` SelectedPawn))

(event `Server_SetSelectedHat`
  (params (SelectedHat :type Name))
  ;[1 1 1] SERVER CALLS FOR CUSTOMIZATION.
  ; Sets all RepNotify variables on the Server for replication.
  (set `self.SelectedHat` SelectedHat))

(event `Server_SetSelectedBodyColor`
  (params (SelectedBodyColor :type Name))
  ;[1 1 1] SERVER CALLS FOR CUSTOMIZATION.
  ; Sets all RepNotify variables on the Server for replication.
  (set `self.SelectedBodyColor` SelectedBodyColor))

(event `Server_SetSelectedLogoColor`
  (params (SelectedLogoColor :type Name))
  ;[1 1 1] SERVER CALLS FOR CUSTOMIZATION.
  ; Sets all RepNotify variables on the Server for replication.
  (set `self.SelectedLogoColor` SelectedLogoColor))

(event `Server_SetSelectedHatColor`
  (params (SelectedHatColor :type Name))
  ;[1 1 1] SERVER CALLS FOR CUSTOMIZATION.
  ; Sets all RepNotify variables on the Server for replication.
  (set `self.SelectedHatColor` SelectedHatColor))

(fn `CleanUpUI`
  ;[1 1 1] Allows us to CleanUp the UI if needed.
)

(fn `OnRep_SelectedBodyColor`
  ;[1 1 1] Workaround of the "Can't override OnRep functions" - Bug
  (`self.OnRep_SelectedBodyColor_Impl`))

(fn `OnRep_SelectedBodyColor_Impl`)

(fn `OnRep_SelectedHat`
  ;[1 1 1] Workaround of the "Can't override OnRep functions" - Bug
  (`self.OnRep_SelectedHat_Impl`))

(fn `OnRep_SelectedHat_Impl`)

(fn `OnRep_SelectedHatColor`
  ;[1 1 1] Workaround of the "Can't override OnRep functions" - Bug
  (`self.OnRep_SelectedHatColor_Impl`))

(fn `OnRep_SelectedHatColor_Impl`)

(fn `OnRep_SelectedLogoColor`
  ;[1 1 1] Workaround of the "Can't override OnRep functions" - Bug
  (`self.OnRep_SelectedLogoColor_Impl`))

(fn `OnRep_SelectedLogoColor_Impl`)

(fn `OnRep_SelectedPawn`
  ;[1 1 1] Workaround of the "Can't override OnRep functions" - Bug
  (`self.OnRep_SelectedPawn_Impl`))

(fn `OnRep_SelectedPawn_Impl`)

(fn `SetSelectedBodyColor`
  (params (SelectedBodyColor :type Name))
  (`|ExecutionSequence`
    (:`then_0`
      (set `self.SelectedBodyColor` SelectedBodyColor))
    (:`then_1`
      (`self.Server_SetSelectedBodyColor` (`self.SelectedBodyColor`)))))

(fn `SetSelectedHat`
  (params (SelectedHat :type Name))
  (`|ExecutionSequence`
    (:`then_0`
      (set `self.SelectedHat` SelectedHat))
    (:`then_1`
      (`self.Server_SetSelectedHat` (`self.SelectedHat`)))))

(fn `SetSelectedHatColor`
  (params (SelectedHatColor :type Name))
  (`|ExecutionSequence`
    (:`then_0`
      (set `self.SelectedHatColor` SelectedHatColor))
    (:`then_1`
      (`self.Server_SetSelectedHatColor` (`self.SelectedHatColor`)))))

(fn `SetSelectedLogoColor`
  (params (SelectedLogoColor :type Name))
  (`|ExecutionSequence`
    (:`then_0`
      (set `self.SelectedLogoColor` SelectedLogoColor))
    (:`then_1`
      (`self.Server_SetSelectedLogoColor` (`self.SelectedLogoColor`)))))

(fn `SetSelectedPawn`
  (params (SelectedPawn :type Name))
  (`|ExecutionSequence`
    (:`then_0`
      (set `self.SelectedPawn` SelectedPawn))
    (:`then_1`
      (`self.Server_SetSelectedPawn` (`self.SelectedPawn`)))))

(fn `SetTeamID`
  (params (TeamID :type Byte))
  (bind _playerstate (`self.PlayerState`))
  ;[1 1 1] Update the TeamID and forward the new value to the PlayerState.
  (set `self.TeamID` TeamID)
  (bind _asbp_ps_base (cast `/Game/MLK/Blueprints/GameModes/Base/Player/BP_PS_Base` _playerstate))
  (set `/Game/MLK/Blueprints/GameModes/Base/Player/BP_PS_Base.TeamID` (`self.TeamID`) _asbp_ps_base)
  (`self.ForceNetUpdate` _playerstate))

(fn `SetupUI`
  ;[1 1 1] Used to setup the UI.
)

(fn `UserConstructionScript`)