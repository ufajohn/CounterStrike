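; BPC_Chat is a PlayerController component that gives each player text chat.
; On BeginPlay, if chat is enabled, it creates the chat widget for the local controller, removing it on EndPlay.
; Outgoing messages are routed to the server, which adds the player's name and hands them to the GameState's chat manager for distribution.
; Received messages are passed to the widget for display.
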(event `self.ReceiveBeginPlay`
  ;[1 1 1] BEGIN PLAY | Component should be attached to the PlayerController. If the PlayerController enables the Chat, spawn a ChatWidget for the Player.
  (if (`self.bEnableChat`)
    (bind _asplayer_controller (cast `PlayerController` (`self.GetOwner`)))
    (if (`Controller.IsLocalPlayerController` _asplayer_controller)
      (bind _returnvalue (`|CreateWidget` (`self.ChatWidgetClass`)))
      (bind _output_get (set `self.ChatWidget` _returnvalue))
      (`UserWidget.AddToViewport` _output_get 10))))

(event `ReceiveChatMessage`
  (params (Sender :type String) (Message :type String))
  ;[1 1 1] RECEIVE CHAT MESSAGE | When receiving a ChatMessage, tell the ChatWidget to add a new Message to the UI.
  (bind _aswb_chat (cast `/Game/MLK/Widgets/Chat/WB_Chat` (`self.ChatWidget`)))
  (`/Game/MLK/Widgets/Chat/WB_Chat.AddChatMessage` _aswb_chat Sender Message))

(event `SendChatMessage`
  (params (Message :type String))
  ;[1 1 1] SEND CHAT MESSAGE | When sending a ChatMessage, we need to move the Information to the Server. He then grabs the PlayerName and the passed Message and tells the GameState's ChatManager to send the Message to everyone else.
  (if (`Actor.HasAuthority` (`self.GetOwner`))
    (bind _asbp_gs_base (cast `/Game/MLK/Blueprints/GameModes/Base/Core/BP_GS_Base` (`GameplayStatics.GetGameState`)))
    (`/Game/MLK/Blueprints/GameModes/Base/Chat/BPC_Chat_Manager.SendChatMessage` (`/Game/MLK/Blueprints/GameModes/Base/Core/BP_GS_Base.BPC_Chat_Manager` _asbp_gs_base) (`PlayerState.GetPlayerName` (`Controller.PlayerState` (cast `PlayerController` (`self.GetOwner`) :!pure true))) Message)
    (else
      (`self.Server_SendChatMessage` Message))))

(event `Server_SendChatMessage`
  (params (Message :type String))
  ;[1 1 1] SEND CHAT MESSAGE | When sending a ChatMessage, we need to move the Information to the Server. He then grabs the PlayerName and the passed Message and tells the GameState's ChatManager to send the Message to everyone else.
  (`self.SendChatMessage` Message))

(event `self.ReceiveEndPlay`
  (params (EndPlayReason :type "EEndPlayReason Enum" :default "Destroyed"))
  (bind _chatwidget (`self.ChatWidget`))
  (`/Engine/EditorBlueprintResources/StandardMacros.IsValid` _chatwidget
    (:`Is Valid`
      (`Widget.RemoveFromParent` _chatwidget))))