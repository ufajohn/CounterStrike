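; Lobby PlayerController that shows the lobby UI and drives the character customization preview.
; On BeginPlay the local player spawns a BP_Pawn_Preview with the selected pawn, hat and colors and makes it the view target.
; Customization setters call the parent, then their OnRep handlers forward the value to the preview through the current view target.
; InitCustomizations takes defaults from the first row of the pawn, hat and color DataTables.
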(event `self.SetupUI`
  ;[1 1 1] SETUP UI | Add the Lobby UI to the viewport.
  (bind _returnvalue (`|CreateWidget` "/Game/MLK/Widgets/Lobby/WB_Lobby.WB_Lobby_C" self))
  (bind _output_get (set `self.WB_Lobby` _returnvalue))
  (`UserWidget.AddToViewport` _output_get 0)
  (`WidgetBlueprintLibrary.SetInputMode_UIOnlyEx` self (`self.WB_Lobby`))
  (set `self.bShowMouseCursor` true))

(event `self.CleanUpUI`
  (bind _wb_lobby (`self.WB_Lobby`))
  ;[1 1 1] CLEAN UP UI | Remove the Lobby UI from the Viewport.
  (`/Engine/EditorBlueprintResources/StandardMacros.IsValid` _wb_lobby
    (:`Is Valid`
      (`Widget.RemoveFromParent` _wb_lobby))))

(event `self.ReceiveBeginPlay`
  ;[1 1 1] BEGIN PLAY | Spawn a Preview Pawn for the Customization Screen of the Lobby for the Player and change the ViewTarget (camera) to it.
  (`|ExecutionSequence`
    (:`then_0`
      (if (`self.IsLocalPlayerController`)
        (bind _returnvalue (`|SpawnActorFromClass` "/Game/MLK/Blueprints/GameModes/Lobby/BP_Pawn_Preview.BP_Pawn_Preview_C" (`KismetMathLibrary.MakeTransform` (0.0 0.0 0.0)) "AlwaysSpawn" "OverrideRootScale" self (`self.SelectedPawn`) (`self.SelectedHat`) (`self.SelectedBodyColor`) (`self.SelectedLogoColor`) (`self.SelectedHatColor`) null))
        (bind _output_get (set `self.PawnPreview` _returnvalue))
        (`self.SetViewTargetWithBlend` _output_get)))
    (:`then_1`
      (`parent.ReceiveBeginPlay`))))

(event `self.SetSelectedPawn`
  (params (SelectedPawn :type Name))
  ;[1 1 1] CUSTOMIZATIONS | Events to update each Customizations and forwarding the call to the Preview Pawn.
  (`parent.SetSelectedPawn` SelectedPawn)
  (`self.OnRep_SelectedPawn_Impl`))

(event `self.OnRep_SelectedPawn_Impl`
  ;[1 1 1] CUSTOMIZATIONS | Events to update each Customizations and forwarding the call to the Preview Pawn.
  (bind _asbp_pawn_preview (cast `/Game/MLK/Blueprints/GameModes/Lobby/BP_Pawn_Preview` (`self.GetViewTarget`)))
  (`/Game/MLK/Blueprints/GameModes/Lobby/BP_Pawn_Preview.UpdatePawn` _asbp_pawn_preview (`self.SelectedPawn`)))

(event `self.SetSelectedHat`
  (params (SelectedHat :type Name))
  ;[1 1 1] CUSTOMIZATIONS | Events to update each Customizations and forwarding the call to the Preview Pawn.
  (`parent.SetSelectedHat` SelectedHat)
  (`self.OnRep_SelectedHat_Impl`))

(event `self.OnRep_SelectedHat_Impl`
  ;[1 1 1] CUSTOMIZATIONS | Events to update each Customizations and forwarding the call to the Preview Pawn.
  (bind _asbp_pawn_preview (cast `/Game/MLK/Blueprints/GameModes/Lobby/BP_Pawn_Preview` (`self.GetViewTarget`)))
  (`/Game/MLK/Blueprints/GameModes/Lobby/BP_Pawn_Preview.UpdateHat` _asbp_pawn_preview (`self.SelectedHat`)))

(event `self.SetSelectedBodyColor`
  (params (SelectedBodyColor :type Name))
  ;[1 1 1] CUSTOMIZATIONS | Events to update each Customizations and forwarding the call to the Preview Pawn.
  (`parent.SetSelectedBodyColor` SelectedBodyColor)
  (`self.OnRep_SelectedBodyColor_Impl`))

(event `self.OnRep_SelectedBodyColor_Impl`
  ;[1 1 1] CUSTOMIZATIONS | Events to update each Customizations and forwarding the call to the Preview Pawn.
  (bind _asbp_pawn_preview (cast `/Game/MLK/Blueprints/GameModes/Lobby/BP_Pawn_Preview` (`self.GetViewTarget`)))
  (`/Game/MLK/Blueprints/GameModes/Lobby/BP_Pawn_Preview.UpdateBodyColor` _asbp_pawn_preview (`self.SelectedBodyColor`)))

(event `self.SetSelectedLogoColor`
  (params (SelectedLogoColor :type Name))
  ;[1 1 1] CUSTOMIZATIONS | Events to update each Customizations and forwarding the call to the Preview Pawn.
  (`parent.SetSelectedLogoColor` SelectedLogoColor)
  (`self.OnRep_SelectedLogoColor_Impl`))

(event `self.OnRep_SelectedLogoColor_Impl`
  ;[1 1 1] CUSTOMIZATIONS | Events to update each Customizations and forwarding the call to the Preview Pawn.
  (bind _asbp_pawn_preview (cast `/Game/MLK/Blueprints/GameModes/Lobby/BP_Pawn_Preview` (`self.GetViewTarget`)))
  (`/Game/MLK/Blueprints/GameModes/Lobby/BP_Pawn_Preview.UpdateLogoColor` _asbp_pawn_preview (`self.SelectedLogoColor`)))

(event `self.SetSelectedHatColor`
  (params (SelectedHatColor :type Name))
  ;[1 1 1] CUSTOMIZATIONS | Events to update each Customizations and forwarding the call to the Preview Pawn.
  (`parent.SetSelectedHatColor` SelectedHatColor)
  (`self.OnRep_SelectedHatColor_Impl`))

(event `self.OnRep_SelectedHatColor_Impl`
  ;[1 1 1] CUSTOMIZATIONS | Events to update each Customizations and forwarding the call to the Preview Pawn.
  (bind _asbp_pawn_preview (cast `/Game/MLK/Blueprints/GameModes/Lobby/BP_Pawn_Preview` (`self.GetViewTarget`)))
  (`/Game/MLK/Blueprints/GameModes/Lobby/BP_Pawn_Preview.UpdateHatColor` _asbp_pawn_preview (`self.SelectedHatColor`)))

(event `InitCustomizations`
  ;[1 1 1] INIT CUSTOMIZATIONS | Retrieves the first entry of each DataTable as the Default Value for the customizations.
  (`|ExecutionSequence`
    (:`then_0`
      (bind _outrownames (`DataTableFunctionLibrary.GetDataTableRowNames` "/Game/MLK/Blueprints/Data/Customizations/DT_PawnData.DT_PawnData"))
      (set `self.SelectedPawn` (`|GetArrayItem` _outrownames)))
    (:`then_1`
      (bind _outrownames_2 (`DataTableFunctionLibrary.GetDataTableRowNames` "/Game/MLK/Blueprints/Data/Customizations/DT_HatData.DT_HatData"))
      (set `self.SelectedHat` (`|GetArrayItem` _outrownames_2)))
    (:`then_2`
      (bind _outrownames_3 (`DataTableFunctionLibrary.GetDataTableRowNames` "/Game/MLK/Blueprints/Data/Customizations/DT_ColorData.DT_ColorData"))
      (bind _output_get (set `self.SelectedBodyColor` (`|GetArrayItem` _outrownames_3)))
      (bind _output_get_2 (set `self.SelectedLogoColor` _output_get))
      (set `self.SelectedHatColor` _output_get_2))))

(fn `UserConstructionScript`
  (`parent.UserConstructionScript`))