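; BP_PS_Lobby is the lobby player state that tracks whether a player is ready.
; ToggleReady flips the flag through SetReady, which sets it locally at once and forwards it to the server.
; The server event stores the value and tells BP_GM_Lobby that the ready state changed.
; The rep notify for the flag is empty.
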(event `SetReady`
  (params (bReady :type Boolean))
  ;[1 1 1] Adjust ReadyState on Client and Server
  (bind _output_get (set `self.bReady` bReady))
  (`self.Server_SetReady` _output_get))

(event `Server_SetReady`
  (params (bReady :type Boolean))
  ;[1 1 1] Adjust ReadyState on Client and Server
  (set `self.bReady` bReady)
  (bind _asbp_gm_lobby (cast `/Game/MLK/Blueprints/GameModes/Lobby/Core/BP_GM_Lobby` (`GameplayStatics.GetGameMode`)))
  (`/Game/MLK/Blueprints/GameModes/Lobby/Core/BP_GM_Lobby.OnReadyStateChanged` _asbp_gm_lobby))

(event `ToggleReady`
  ;[1 1 1] Adjust ReadyState on Client and Server
  (`self.SetReady` (not (`self.bReady`))))

(fn `OnRep_bReady`)

(fn `UserConstructionScript`
  (`parent.UserConstructionScript`))