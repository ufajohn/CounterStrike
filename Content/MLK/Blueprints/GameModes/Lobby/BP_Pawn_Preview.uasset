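; Lobby preview actor that displays a customizable pawn with hat, body, logo and hat colors, hidden on BeginPlay until made visible.
; Update events store the selected row name, look it up in the pawn, hat or color DataTable, and fall back to a default row if missing.
; Colors are applied through dynamic material instances.
; Mesh swaps reapply the matching colors, with pawn swaps first restoring the new mesh's own materials.
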(event `self.ReceiveBeginPlay`
  (`self.HidePreview`)
  (`self.InitPreview`))

(event `InitPreview`
  (`self.ReapplyPawn`)
  (`self.ReapplyHat`)
  (`self.ReapplyBodyAndLogoColor`)
  (`self.ReapplyHatColor`))

(event `SetPreviewVisibility`
  (params (bNewVisible :type Boolean))
  ;[1 1 1] Hide and Show the Preview Mesh
  (if bNewVisible
    (`self.ShowPreview`)
    (else
      (`self.HidePreview`))))

(event `ShowPreview`
  ;[1 1 1] Hide and Show the Preview Mesh
  (`SceneComponent.SetVisibility` (`self.SkeletalMesh`) true true))

(event `HidePreview`
  ;[1 1 1] Hide and Show the Preview Mesh
  (`SceneComponent.SetVisibility` (`self.SkeletalMesh`) false true))

(event `UpdatePawn`
  (params (PawnRow :type Name))
  (bind ((`UISkeletalMesh_9_29BBB31C43582F8FA722A4B65034F524` _uiskeletalmesh)) (break `/Game/MLK/Blueprints/Structs/Customizations/FPawnData` (`self.PawnData`)))
  (bind _materials (`SkeletalMesh.Materials` _uiskeletalmesh))
  ;[1 1 1] Mesh Updates
  (bind _output_get (set `self.CurrentPawn` PawnRow))
  (bind _returnvalue (`|GetDataTableRow` "/Game/MLK/Blueprints/Data/Customizations/DT_PawnData.DT_PawnData" _output_get)
    (:`then`
      (set `self.PawnData` _returnvalue))
    (:`RowNotFound`
      (bind _returnvalue_2 (`|GetDataTableRow` "/Game/MLK/Blueprints/Data/Customizations/DT_PawnData.DT_PawnData" "BasePawn")
        (:`then`
          (set `self.PawnData` _returnvalue_2)))))
  (`SkinnedMeshComponent.SetSkinnedAssetAndUpdate` (`self.SkeletalMesh`) _uiskeletalmesh false)
  (`PrimitiveComponent.SetMaterial` (`self.SkeletalMesh`) 0 (`.MaterialInterface` (break `SkeletalMaterial` (`|GetArrayItem` _materials))))
  (`PrimitiveComponent.SetMaterial` (`self.SkeletalMesh`) 1 (`.MaterialInterface` (break `SkeletalMaterial` (`|GetArrayItem` _materials 1))))
  (`self.ReapplyBodyAndLogoColor`))

(event `UpdateHat`
  (params (HatRow :type Name))
  ;[1 1 1] Mesh Updates
  (bind _output_get (set `self.CurrentHat` HatRow))
  (bind _returnvalue (`|GetDataTableRow` "/Game/MLK/Blueprints/Data/Customizations/DT_HatData.DT_HatData" _output_get)
    (:`then`
      (set `self.HatData` _returnvalue))
    (:`RowNotFound`
      (bind _returnvalue_2 (`|GetDataTableRow` "/Game/MLK/Blueprints/Data/Customizations/DT_HatData.DT_HatData" "Cylinder")
        (:`then`
          (set `self.HatData` _returnvalue_2)))))
  (`StaticMeshComponent.SetStaticMesh` (`self.SM_Hat_Cylinder`) (`.StaticMesh_9_F397C86A4F3C93FFC455FCAFE92C5C0C` (break `/Game/MLK/Blueprints/Structs/Customizations/FHatData` (`self.HatData`))))
  (`self.ReapplyHatColor`))

(event `ReapplyPawn`
  ;[1 1 1] Mesh Updates
  (`self.UpdatePawn` (`self.CurrentPawn`)))

(event `ReapplyHat`
  ;[1 1 1] Mesh Updates
  (`self.UpdateHat` (`self.CurrentHat`)))

(event `UpdateBodyColor`
  (params (ColorRow :type Name))
  ;[1 1 1] Color Updates
  (bind _output_get (set `self.CurrentBodyColor` ColorRow))
  (bind _returnvalue (`|GetDataTableRow` "/Game/MLK/Blueprints/Data/Customizations/DT_ColorData.DT_ColorData" _output_get)
    (:`then`
      (set `self.BodyColorData` _returnvalue))
    (:`RowNotFound`
      (bind _returnvalue_2 (`|GetDataTableRow` "/Game/MLK/Blueprints/Data/Customizations/DT_ColorData.DT_ColorData" "White")
        (:`then`
          (set `self.BodyColorData` _returnvalue_2)))))
  (bind _returnvalue_3 (`PrimitiveComponent.CreateDynamicMaterialInstance` (`self.SkeletalMesh`) 0 null))
  (`MaterialInstanceDynamic.SetVectorParameterValue` _returnvalue_3 "BodyColor" (`.Color_2_FB8F2A4247D69DDA6A961F87DAC736B3` (break `/Game/MLK/Blueprints/Structs/Customizations/FColorData` (`self.BodyColorData`)))))

(event `UpdateLogoColor`
  (params (ColorRow :type Name))
  ;[1 1 1] Color Updates
  (bind _output_get (set `self.CurrentLogoColor` ColorRow))
  (bind _returnvalue (`|GetDataTableRow` "/Game/MLK/Blueprints/Data/Customizations/DT_ColorData.DT_ColorData" _output_get)
    (:`then`
      (set `self.LogoColorData` _returnvalue))
    (:`RowNotFound`
      (bind _returnvalue_2 (`|GetDataTableRow` "/Game/MLK/Blueprints/Data/Customizations/DT_ColorData.DT_ColorData" "White")
        (:`then`
          (set `self.LogoColorData` _returnvalue_2)))))
  (bind _returnvalue_3 (`PrimitiveComponent.CreateDynamicMaterialInstance` (`self.SkeletalMesh`) 1 null))
  (`MaterialInstanceDynamic.SetVectorParameterValue` _returnvalue_3 "LogoColor" (`.Color_2_FB8F2A4247D69DDA6A961F87DAC736B3` (break `/Game/MLK/Blueprints/Structs/Customizations/FColorData` (`self.LogoColorData`)))))

(event `UpdateHatColor`
  (params (ColorRow :type Name))
  ;[1 1 1] Color Updates
  (bind _output_get (set `self.CurrentHatColor` ColorRow))
  (bind _returnvalue (`|GetDataTableRow` "/Game/MLK/Blueprints/Data/Customizations/DT_ColorData.DT_ColorData" _output_get)
    (:`then`
      (set `self.HatColorData` _returnvalue))
    (:`RowNotFound`
      (bind _returnvalue_2 (`|GetDataTableRow` "/Game/MLK/Blueprints/Data/Customizations/DT_ColorData.DT_ColorData" "White")
        (:`then`
          (set `self.HatColorData` _returnvalue_2)))))
  (bind _returnvalue_3 (`PrimitiveComponent.CreateDynamicMaterialInstance` (`self.SM_Hat_Cylinder`) 0 null))
  (`MaterialInstanceDynamic.SetVectorParameterValue` _returnvalue_3 "Color" (`.Color_2_FB8F2A4247D69DDA6A961F87DAC736B3` (break `/Game/MLK/Blueprints/Structs/Customizations/FColorData` (`self.HatColorData`)))))

(event `ReapplyBodyAndLogoColor`
  ;[1 1 1] Color Updates
  (`self.UpdateBodyColor` (`self.CurrentBodyColor`))
  (`self.UpdateLogoColor` (`self.CurrentLogoColor`)))

(event `ReapplyHatColor`
  ;[1 1 1] Color Updates
  (`self.UpdateHatColor` (`self.CurrentHatColor`)))

(fn `UserConstructionScript`)