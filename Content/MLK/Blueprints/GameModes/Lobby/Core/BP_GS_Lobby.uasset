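; Lobby game state that holds match settings and passes their changes on to the lobby UI.
; On BeginPlay, a dedicated server copies game mode, next map and match time from the game instance's current match settings.
; RepNotify handlers reach the lobby widgets through the first player controller, forwarding round-start changes on non-dedicated instances and game mode changes to the match settings widget.
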(event `self.ReceiveBeginPlay`
  (if (`KismetSystemLibrary.IsDedicatedServer`)
    (bind _asbp_gi (cast `/Game/MLK/Blueprints/Core/BP_GI` (`GameplayStatics.GetGameInstance`)))
    (bind ((`GameMode_23_0FC75F574F0BB05B36C23997982B5EF0` _gamemode) (`NextMap_18_5D862F524A41C8398926368742F5047C` _nextmap) (`MatchTime_24_19A1859244E7184C85868DB74EC103FD` _matchtime)) (break `/Game/MLK/Blueprints/Structs/FMatchSettings` (`/Game/MLK/Blueprints/Core/BP_GI.CurrentMatchSettings` _asbp_gi)))
    (set `self.GameMode` _gamemode)
    (set `self.Map` _nextmap)
    (set `self.MatchTime` _matchtime)))

(fn `OnRep_bStartingRound`
  ;[1 1 1] When receiving a new value for bStartingRound, tell the PlayerController.
  (if (not (`KismetSystemLibrary.IsDedicatedServer`))
    (bind _asbp_pc_lobby (cast `/Game/MLK/Blueprints/GameModes/Lobby/Player/BP_PC_Lobby` (`GameplayStatics.GetPlayerController` 0)))
    (`/Game/MLK/Widgets/Lobby/WB_Lobby.OnStartStateChanged` (`/Game/MLK/Blueprints/GameModes/Lobby/Player/BP_PC_Lobby.WB_Lobby` _asbp_pc_lobby) (`self.bStartingRound`))))

(fn `OnRep_GameMode_Impl`
  (`parent.OnRep_GameMode_Impl`)
  (bind _asbp_pc_lobby (cast `/Game/MLK/Blueprints/GameModes/Lobby/Player/BP_PC_Lobby` (`GameplayStatics.GetPlayerController` 0)))
  (bind _wb_lobby (`/Game/MLK/Blueprints/GameModes/Lobby/Player/BP_PC_Lobby.WB_Lobby` _asbp_pc_lobby))
  (`/Engine/EditorBlueprintResources/StandardMacros.IsValid` _wb_lobby
    (:`Is Valid`
      (bind _wb_matchsettings (`/Game/MLK/Widgets/Lobby/WB_Lobby.WB_MatchSettings` _wb_lobby))
      (`/Engine/EditorBlueprintResources/StandardMacros.IsValid` _wb_matchsettings
        (:`Is Valid`
          (bind _wb_lobby_settings_match (`/Game/MLK/Widgets/Lobby/WB_Lobby_Settings.WB_Lobby_Settings_Match` _wb_matchsettings))
          (`/Engine/EditorBlueprintResources/StandardMacros.IsValid` _wb_lobby_settings_match
            (:`Is Valid`
              (`/Game/MLK/Widgets/Lobby/WB_Lobby_Settings_Match.SetGameMode` _wb_lobby_settings_match (`self.GameMode`)))))))))

(fn `UserConstructionScript`
  (`parent.UserConstructionScript`))