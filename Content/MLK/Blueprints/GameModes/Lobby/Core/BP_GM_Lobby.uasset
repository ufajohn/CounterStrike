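; Lobby game mode that starts the next round via server travel through the game instance once all players are ready.
; Ready-state changes start or cancel a countdown timer, mirroring the starting-round flag to the lobby GameState to inform players.
; New joiners get their customizations initialized and cancel any running countdown.
; Changing the team-based setting reassigns teams to everyone already in the lobby.
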(event `self.SetTeamBased`
  (params (bTeamBased :type Boolean))
  ;[1 1 1] When TeamBased is updated, we want to make sure that teams are properly updated.
  (`parent.SetTeamBased` bTeamBased)
  (`self.AssignTeams`))

(event `self.HandleNewPlayer`
  (params (NewPlayer :type "PlayerController Object Reference"))
  ;[1 1 1] Inits the customizations for a new joining player. Also make sure to cancel the round start if one is ongoing.
  (`parent.HandleNewPlayer` NewPlayer)
  (bind _asbp_pc_lobby (cast `/Game/MLK/Blueprints/GameModes/Lobby/Player/BP_PC_Lobby` NewPlayer))
  (`/Game/MLK/Blueprints/GameModes/Lobby/Player/BP_PC_Lobby.InitCustomizations` _asbp_pc_lobby)
  (`self.CancelRoundStart`))

(fn `AreAllPlayersReady`
  (returns (bAllReady :type Boolean))
  (locals (bLocalAllPlayersReady :type Boolean))
  ;[1 1 1] Check each PlayerState for being ready or not.
  (set `local.bLocalAllPlayersReady` true)
  (bind _asbp_gs_base (cast `/Game/MLK/Blueprints/GameModes/Base/Core/BP_GS_Base` (`GameplayStatics.GetGameState`)))
  (for _array_element (`GameStateBase.PlayerArray` _asbp_gs_base)
    (bind _asbp_ps_lobby (cast `/Game/MLK/Blueprints/GameModes/Lobby/Player/BP_PS_Lobby` _array_element))
    (if (not (`/Game/MLK/Blueprints/GameModes/Lobby/Player/BP_PS_Lobby.bReady` _asbp_ps_lobby))
      (set `local.bLocalAllPlayersReady` false)
      (break)))
  (return (`local.bLocalAllPlayersReady`)))

(fn `AssignTeams`
  ;[1 1 1] Assigns a Team to all Players. Used when the GameMode is changed during already being in the Lobby.
  (for _array_element (`GameStateBase.PlayerArray` (`GameplayStatics.GetGameState`))
    (bind _asbp_pc_base (cast `/Game/MLK/Blueprints/GameModes/Base/Player/BP_PC_Base` (`self.GetOwner` _array_element)))
    (`self.AssignTeamToPlayer` _asbp_pc_base)))

(fn `CancelRoundStart`
  ;[1 1 1] Cancels the Round Start Countdown and informs all Players.
  (if (`self.bStartingRound`)
    (set `self.bStartingRound` false)
    (`|ExecutionSequence`
      (:`then_0`
        (`KismetSystemLibrary.K2_ClearAndInvalidateTimerHandle` (`self.TimerHandle_StartRound`)))
      (:`then_1`
        (bind _asbp_gs_lobby (cast `/Game/MLK/Blueprints/GameModes/Lobby/Core/BP_GS_Lobby` (`GameplayStatics.GetGameState`)))
        (set `/Game/MLK/Blueprints/GameModes/Lobby/Core/BP_GS_Lobby.bStartingRound` (`self.bStartingRound`) _asbp_gs_lobby)))))

(fn `InitRoundStart`
  ;[1 1 1] Check if we aren't already starting the next round. If not, then set a timer and notify all players via the GameState.
  (if (not (`self.bStartingRound`))
    (set `self.bStartingRound` true)
    (`|ExecutionSequence`
      (:`then_0`
        (bind _asbp_gs_lobby (cast `/Game/MLK/Blueprints/GameModes/Lobby/Core/BP_GS_Lobby` (`GameplayStatics.GetGameState`)))
        (set `/Game/MLK/Blueprints/GameModes/Lobby/Core/BP_GS_Lobby.bStartingRound` (`self.bStartingRound`) _asbp_gs_lobby))
      (:`then_1`
        (bind _returnvalue (`KismetSystemLibrary.K2_SetTimer` null "StartRound" (`self.RoundStartTime`)))
        (set `self.TimerHandle_StartRound` _returnvalue)))))

(fn `OnReadyStateChanged`
  ;[1 1 1] When the ReadyState Changes, we want to either init the round start countdown or stop it.
  (if (`self.AreAllPlayersReady`)
    (`self.InitRoundStart`)
    (else
      (`self.CancelRoundStart`))))

(fn `StartRound`
  ;[1 1 1] ServerTravel to next Map. Update MaxPlayers Option to stop players from joining who weren't in the lobby.
  (bind _asbp_gi (cast `/Game/MLK/Blueprints/Core/BP_GI` (`GameplayStatics.GetGameInstance`)))
  (`/Game/MLK/Blueprints/Core/BP_GI.ServerTravelToNextMap` _asbp_gi))

(fn `UserConstructionScript`
  (`parent.UserConstructionScript`))