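; Gameplay player pawn that shows the player's chosen body, hat, colors and team during a match.
; On possession it copies TeamID and the saved lobby customizations from BP_PC_Gameplay.
; RepNotify functions look up data tables to swap skeletal and hat meshes and tint them through dynamic material instances.
; Mesh swaps reapply colors so they are not reset, and team changes update a debug text label.
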(event `self.ReceivePossessed`
  (params (NewController :type "Controller Object Reference"))
  ;[1 1 1] Retrieve the TeamID from the PlayerController and the Customizations when being possessed.
  (`self.RetrieveCustomizations`)
  (bind _asbp_pc_gameplay (cast `/Game/MLK/Blueprints/GameModes/Gameplay/Player/BP_PC_GamePlay` NewController))
  (set `self.TeamID` (`/Game/MLK/Blueprints/GameModes/Base/Player/BP_PC_Base.TeamID` _asbp_pc_gameplay)))

(fn `OnRep_SelectedBodyColor`
  (`self.RetrieveBodyColor`))

(fn `OnRep_SelectedHat`
  ;[1 1 1] When updating the Hat Mesh, make sure to reapply the color. Otherwise the hat has the default color.
  (bind _returnvalue (`|GetDataTableRow` "/Game/MLK/Blueprints/Data/Customizations/DT_HatData.DT_HatData" (`self.SelectedHat`))
    (:`then`
      (`StaticMeshComponent.SetStaticMesh` (`self.HatMesh`) (`.StaticMesh_9_F397C86A4F3C93FFC455FCAFE92C5C0C` (break `/Game/MLK/Blueprints/Structs/Customizations/FHatData` _returnvalue)))
      (`self.RetrieveHatColor`))))

(fn `OnRep_SelectedHatColor`
  (`self.RetrieveHatColor`))

(fn `OnRep_SelectedLogoColor`
  (`self.RetrieveLogoColor`))

(fn `OnRep_SelectedPawn`
  ;[1 1 1] When the SkeletalMesh is updated, make sure to also reapply the Color changes to the Mesh. Otherwise they are resetted and the Mesh has the default color.
  (bind _returnvalue (`|GetDataTableRow` "/Game/MLK/Blueprints/Data/Customizations/DT_PawnData.DT_PawnData" (`self.SelectedPawn`))
    (:`then`
      (bind ((`UISkeletalMesh_9_29BBB31C43582F8FA722A4B65034F524` _uiskeletalmesh)) (break `/Game/MLK/Blueprints/Structs/Customizations/FPawnData` _returnvalue))
      (`SkinnedMeshComponent.SetSkinnedAssetAndUpdate` (`self.SkeletalMesh`) _uiskeletalmesh false)
      (bind _materials (`SkeletalMesh.Materials` _uiskeletalmesh))
      (`PrimitiveComponent.SetMaterial` (`self.SkeletalMesh`) 0 (`.MaterialInterface` (break `SkeletalMaterial` (`|GetArrayItem` _materials))))
      (`PrimitiveComponent.SetMaterial` (`self.SkeletalMesh`) 1 (`.MaterialInterface` (break `SkeletalMaterial` (`|GetArrayItem` _materials 1))))
      (`self.RetrieveBodyColor`)
      (`self.RetrieveLogoColor`))))

(fn `OnRep_TeamID`
  ;[1 1 1] Just some simple debug. Change the Text and TextColor of the TextRenderer.
  ; You can do all kinds of adjustments here, like MeshColor and such.
  (`TextRenderComponent.K2_SetText` (`self.Team_Text`) (select `byte` (`self.TeamID`) :`0` "FFA" :`1` "ORANGE TEAM" :`2` "BLUE TEAM"))
  (`TextRenderComponent.SetTextRenderColor` (`self.Team_Text`) (select `byte` (`self.TeamID`) :`0` (`KismetMathLibrary.Conv_LinearColorToColor` (struct :`A` 1.0)) :`1` (`KismetMathLibrary.Conv_LinearColorToColor` (struct :`R` 0.955974 :`G` 0.223228 :`B` 0.030713 :`A` 1.0)) :`2` (`KismetMathLibrary.Conv_LinearColorToColor` (struct :`R` 0.039546 :`G` 0.135633 :`B` 0.672443 :`A` 1.0)))))

(fn `RetrieveBodyColor`
  ;[1 1 1] Override the Color on the SkeletalMesh Material.
  (bind _returnvalue (`|GetDataTableRow` "/Game/MLK/Blueprints/Data/Customizations/DT_ColorData.DT_ColorData" (`self.SelectedBodyColor`))
    (:`then`
      (bind _returnvalue_2 (`PrimitiveComponent.CreateDynamicMaterialInstance` (`self.SkeletalMesh`) 0 null "None"))
      (`MaterialInstanceDynamic.SetVectorParameterValue` _returnvalue_2 "BodyColor" (`.Color_2_FB8F2A4247D69DDA6A961F87DAC736B3` (break `/Game/MLK/Blueprints/Structs/Customizations/FColorData` _returnvalue))))))

(fn `RetrieveCustomizations`
  (locals (GameplayController :type "/Game/MLK/Blueprints/GameModes/Gameplay/Player/BP_PC_GamePlay Object Reference"))
  ;[1 1 1] Get all saved customization data from the PlayerController. This is passed when moving from Lobby to Gameplay level.
  (bind _asbp_pc_gameplay (cast `/Game/MLK/Blueprints/GameModes/Gameplay/Player/BP_PC_GamePlay` (`self.GetController`)))
  (set `local.GameplayController` _asbp_pc_gameplay)
  (`|ExecutionSequence`
    (:`then_0`
      (set `self.SelectedPawn` (`/Game/MLK/Blueprints/GameModes/Base/Player/BP_PC_Base.SelectedPawn` (`local.GameplayController`))))
    (:`then_1`
      (set `self.SelectedHat` (`/Game/MLK/Blueprints/GameModes/Base/Player/BP_PC_Base.SelectedHat` (`local.GameplayController`))))
    (:`then_2`
      (set `self.SelectedBodyColor` (`/Game/MLK/Blueprints/GameModes/Base/Player/BP_PC_Base.SelectedBodyColor` (`local.GameplayController`))))
    (:`then_3`
      (set `self.SelectedLogoColor` (`/Game/MLK/Blueprints/GameModes/Base/Player/BP_PC_Base.SelectedLogoColor` (`local.GameplayController`))))
    (:`then_4`
      (set `self.SelectedHatColor` (`/Game/MLK/Blueprints/GameModes/Base/Player/BP_PC_Base.SelectedHatColor` (`local.GameplayController`))))))

(fn `RetrieveHatColor`
  ;[1 1 1] Override the Color on the Hat Material.
  (bind _returnvalue (`|GetDataTableRow` "/Game/MLK/Blueprints/Data/Customizations/DT_ColorData.DT_ColorData" (`self.SelectedHatColor`))
    (:`then`
      (bind _returnvalue_2 (`PrimitiveComponent.CreateDynamicMaterialInstance` (`self.HatMesh`) 0 null "None"))
      (`MaterialInstanceDynamic.SetVectorParameterValue` _returnvalue_2 "Color" (`.Color_2_FB8F2A4247D69DDA6A961F87DAC736B3` (break `/Game/MLK/Blueprints/Structs/Customizations/FColorData` _returnvalue))))))

(fn `RetrieveLogoColor`
  ;[1 1 1] Override the Logo Color on the SkeletalMesh Material.
  (bind _returnvalue (`|GetDataTableRow` "/Game/MLK/Blueprints/Data/Customizations/DT_ColorData.DT_ColorData" (`self.SelectedLogoColor`))
    (:`then`
      (bind _returnvalue_2 (`PrimitiveComponent.CreateDynamicMaterialInstance` (`self.SkeletalMesh`) 1 null "None"))
      (`MaterialInstanceDynamic.SetVectorParameterValue` _returnvalue_2 "LogoColor" (`.Color_2_FB8F2A4247D69DDA6A961F87DAC736B3` (break `/Game/MLK/Blueprints/Structs/Customizations/FColorData` _returnvalue))))))

(fn `UserConstructionScript`
  (`parent.UserConstructionScript`))