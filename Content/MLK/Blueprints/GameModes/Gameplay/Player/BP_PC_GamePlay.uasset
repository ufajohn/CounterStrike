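; Base gameplay player controller that shows and removes an example game mode indicator on the player's screen.
; SetupUI creates a WB_GameModeIndicator widget with empty mode text, adds it to the viewport and switches input to game only.
; CleanUpUI removes that stored widget from its parent.
; It is meant as an inheritance example, where children for modes such as Deathmatch or Last Man Standing override the indicator text.
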(event `self.SetupUI`
  ;[1 1 1] Add the GameMode indicator Widget to the screen. This is a simple example on how inheritance here works. The specific Children of this class (e.g. Deathmatch, Last Man Standing, et.c) can override the GameModeText. You can of course to lots of things per different GameMode.
  (bind _returnvalue (`|CreateWidget` "/Game/MLK/Widgets/Examples/WB_GameModeIndicator.WB_GameModeIndicator_C" self))
  (bind _output_get (set `self.WB_GM_Indicator` _returnvalue))
  (`UserWidget.AddToViewport` _output_get 0)
  (`WidgetBlueprintLibrary.SetInputMode_GameOnly` self))

(event `self.CleanUpUI`
  ;[1 1 1] Removes the example GameMode indicator.
  (`Widget.RemoveFromParent` (`self.WB_GM_Indicator`)))

(fn `UserConstructionScript`
  (`parent.UserConstructionScript`))