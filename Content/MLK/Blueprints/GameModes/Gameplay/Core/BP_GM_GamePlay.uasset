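; BP_GM_GamePlay is the gameplay game mode, choosing each player's pawn class and handling the return to the lobby.
; It overrides GetDefaultPawnClassForController to look up the player controller's SelectedPawn row in DT_PawnData and return that row's PawnClass.
; ReturnToLobby uses a ReturningToLobby guard so it triggers only once, then calls ServerTravelToLobby on BP_GI.
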(fn `GetDefaultPawnClassForController`
  (params (InController :type "Controller Object Reference"))
  (returns (ReturnValue :type "Object Class Reference"))
  ;[1 1 1] Grab the saved pawn class from the player's playercontroller
  (bind _asbp_pc_base (cast `/Game/MLK/Blueprints/GameModes/Base/Player/BP_PC_Base` InController))
  (bind _returnvalue (`|GetDataTableRow` "/Game/MLK/Blueprints/Data/Customizations/DT_PawnData.DT_PawnData" (`/Game/MLK/Blueprints/GameModes/Base/Player/BP_PC_Base.SelectedPawn` _asbp_pc_base))
    (:`then`
      (return (`.PawnClass_3_B6B3A9B24D4A57F6E35CA4ACBC451ACE` (break `/Game/MLK/Blueprints/Structs/Customizations/FPawnData` _returnvalue))))))

(fn `ReturnToLobby`
  ;[1 1 1] Let's us return to the Lobby.
  (if (not (`self.bReturningToLobby`))
    (set `self.bReturningToLobby` true)
    (bind _asbp_gi (cast `/Game/MLK/Blueprints/Core/BP_GI` (`GameplayStatics.GetGameInstance`)))
    (`/Game/MLK/Blueprints/Core/BP_GI.ServerTravelToLobby` _asbp_gi)))

(fn `UserConstructionScript`
  (`parent.UserConstructionScript`))