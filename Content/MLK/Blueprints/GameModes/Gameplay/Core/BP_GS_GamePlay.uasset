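; Gameplay GameState that runs the match countdown and has the server return everyone to the lobby through BP_GM_Gameplay at zero.
; A looping one-second timer decrements RemainingMatchTime locally.
; Every ten seconds the server copies it to RemainingMatchTimeRep, whose OnRep overwrites the local value to correct drift.
; Setting MatchTime seeds the countdown, then resets to -1 so an identical value can retrigger the OnRep.
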(event `self.ReceiveTick`
  (params (DeltaSeconds :type "Float (single-precision)"))
  (set `self.DeltaSeconds` DeltaSeconds))

(event `self.ReceiveBeginPlay`
  ;[1 1 1] Start a timer that loops every second. Makes it easy to reduce our timers.
  (bind _returnvalue (`KismetSystemLibrary.K2_SetTimerDelegate` (`|CreateDelegate` :!event `DefaultTimer`) 1.0 true))
  (set `self.TimerHandle_DefaultTimer` _returnvalue))

(event `self.OnRep_MatchTime_Impl`
  ;[1 1 1] Initial setup
  (if (>= (`self.MatchTime`) 0)
    (bind _output_get (set `self.RemainingMatchTime` (`self.MatchTime`)))
    (set `self.RemainingMatchTimeRep` _output_get)
    ;[1 1 1] We can't force OnRep to call every time in BPs, so it wouldn't call if we set it to the same value again. That means if the time is 300 and we want to reset it to 300 again after some time, it wouldn't work. Thus we want to set the MatchTime to something "invalid" and filter this at the start of the OnRep.
    (set `self.MatchTime` -1)))

(event `DefaultTimer`
  ;[1 1 1] Check if we still have time
  (if (> (`self.RemainingMatchTime`) 0)
    ;[1 1 1] Reduce time on everyone
    (set `self.RemainingMatchTime` (- (`self.RemainingMatchTime`) 1))
    ;[1 1 1] If the time % 10 == 9, refresh the time everywhere with the server version to keep it in sync
    (`/Engine/EditorBlueprintResources/ActorMacros.Switch Has Authority`
      (:`Authority`
        (if (== (mod (`self.RemainingMatchTime`) 10) 9)
          (set `self.RemainingMatchTimeRep` (`self.RemainingMatchTime`)))))
    (else
      ;[1 1 1] RemainingTime <= 0, return to Lobby.
      (`/Engine/EditorBlueprintResources/ActorMacros.Switch Has Authority`
        (:`Authority`
          (bind _asbp_gm_gameplay (cast `/Game/MLK/Blueprints/GameModes/Gameplay/Core/BP_GM_GamePlay` (`GameplayStatics.GetGameMode`)))
          (`/Game/MLK/Blueprints/GameModes/Gameplay/Core/BP_GM_GamePlay.ReturnToLobby` _asbp_gm_gameplay))))))

(fn `OnRep_RemainingMatchTimeRep`
  ;[1 1 1] Override local time with replicated one
  (set `self.RemainingMatchTime` (`self.RemainingMatchTimeRep`)))

(fn `UserConstructionScript`
  (`parent.UserConstructionScript`))