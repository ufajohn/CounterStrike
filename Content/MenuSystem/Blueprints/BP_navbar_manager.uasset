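; Menu navbar manager that builds shortcut buttons for the active panel and routes key presses to that panel's commands.
; Panels supply their button list through a message, which is flattened into a cached command-per-key list that input handling scans.
; The navbar rebuilds when the panel changes or an update is forced, then broadcasts the change.
; It also holds the navigation manager and viewport navbar widget, clearing references for garbage collection.
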(fn `ClearForGC`
  (params (ActorBeingDestroyed :type "Actor Object Reference"))
  (`KismetArrayLibrary.Array_Clear` (`self.NavbarButtons`))
  (`KismetArrayLibrary.Array_Clear` (`self.NavbarButtonsReformattedForLoop`))
  (set `self.CurrentPanelToNavigate` null)
  (bind _navbarwidget (`self.NavbarWidget`)
    (:`then`
      (`Widget.RemoveFromParent` _navbarwidget))
    (:`else`)))

(fn `ClearNavbar`
  (`KismetArrayLibrary.Array_Clear` (`self.NavbarButtons`))
  (`KismetArrayLibrary.Array_Clear` (`self.NavbarButtonsReformattedForLoop`))
  (set `self.CurrentPanelToNavigate` null))

(fn `GetCurrentPanel`
  (returns (CurrentPanel :type "Widget Object Reference"))
  (bind _navmanager (`self.NavManager`)
    (:`then`
      (bind _widget (break `/Game/MenuSystem/Structs/FWidgetFix` (`/Game/MenuSystem/Blueprints/BP_NavigationManager.GetCurrentPanel` _navmanager)))
      (`/Engine/EditorBlueprintResources/StandardMacros.IsValid` _widget
        (:`Is Valid`
          (bind _output_get (set `self.CurrentPanelToNavigate` _widget))
          (return _output_get))))
    (:`else`)))

(fn `GetNavbarButtons`
  (returns (NavbarButtons :type "Array of /Game/MenuSystem/Structs/FNavbarButton Structure"))
  (return (`self.NavbarButtons`)))

(fn `GetNavbarWidget`
  (returns (NavbarWidget :type "/Game/MenuSystem/Widgets/Common/Overlay_and_popups/WBP_NavbarOverlay Object Reference"))
  (return (`self.NavbarWidget`)))

(fn `MakeNavbar`
  (params (PanelToNavigate :type "Widget Object Reference (by ref)"))
  (`/Engine/EditorBlueprintResources/StandardMacros.IsValid` PanelToNavigate
    (:`Is Valid`
      (`self.ClearNavbar`)
      (bind _output_get (set `self.CurrentPanelToNavigate` PanelToNavigate))
      (bind _navbarbuttons (message `/Game/MenuSystem/Interface/BPI_Navbar.MakeNavbar` _output_get))
      (`KismetArrayLibrary.Array_Clear` (`self.NavbarButtonsReformattedForLoop`))
      (bind _output_get_2 (set `self.NavbarButtons` _navbarbuttons))
      (for _array_element _output_get_2
        (bind ((`ShortcutKey_7_0D57367A412037EC46F8FD8A618CFCC6` _shortcutkey) (`Command_10_D91793D04C02FE872970599C28AE9D98` _command)) (break `/Game/MenuSystem/Structs/FNavbarButton` _array_element))
        (bind _values (`BlueprintMapLibrary.Map_Values` _shortcutkey))
        (for _array_element_2 _values
          (for _array_element_3 (`.keys_6_8AC0987F420A75699CE53D92195029D2` (break `/Game/MenuSystem/Structs/FShortcutKeyList` _array_element_2))
            (`KismetArrayLibrary.Array_Add` (`self.NavbarButtonsReformattedForLoop`) (make `/Game/MenuSystem/Structs/FNavbarButtonListCached` _command _array_element_3)))))
      (`self.NavbarUpdated` (make `/Game/MenuSystem/Structs/FWidgetFix` (`self.CurrentPanelToNavigate`))))))

(fn `OnInput`
  (params (Key :type "Key Structure" :default "None"))
  (returns (Handled :type Boolean))
  (locals (OwnerWidget :type "Widget Object Reference"))
  (for _array_element (`self.NavbarButtonsReformattedForLoop`)
    (bind (_command _key) (break `/Game/MenuSystem/Structs/FNavbarButtonListCached` _array_element))
    (if (== Key _key)
      (message `/Game/MenuSystem/Interface/BPI_Navbar.RunNavbarCommand` (`self.CurrentPanelToNavigate`) _command)
      (return true)))
  (return false))

(fn `SetNavbarWidget`
  (params (NavbarWidget :type "/Game/MenuSystem/Widgets/Common/Overlay_and_popups/WBP_NavbarOverlay Object Reference"))
  (bind _output_get (set `self.NavbarWidget` NavbarWidget))
  (`UserWidget.AddToViewport` _output_get 10))

(fn `SetNavigationManager`
  (params (NavigationManager :type "/Game/MenuSystem/Blueprints/BP_NavigationManager Object Reference (by ref)"))
  (set `self.NavManager` NavigationManager))

(fn `TryNavbarUpdate`
  (params (PanelToNavigate :type "/Game/MenuSystem/Structs/FWidgetFix Structure") (ForceUpdate :type Boolean))
  (if (or (!= PanelToNavigate_Widget_2_425509A44D85A122B67D7783D4133412 (`self.CurrentPanelToNavigate`)) ForceUpdate)
    (`self.MakeNavbar` PanelToNavigate_Widget_2_425509A44D85A122B67D7783D4133412)))