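; Blueprint function library of save system wrappers, used by the menu system as stand-ins for the AGS Basic Save Game plugin.
; Each wrapper covers one operation, such as saving, loading by ID or checkpoint, listing saves or savable actors, removing saves and fetching the save manager.
; All are stubs that do nothing or return false or empty values, except SaveGameWrapper, which prints that the plugin is not installed.
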(fn `GetSavableActorListWrapper`
  (returns (SavableActors :type "Array of Actor Object Reference"))
  (return))

(fn `GetSaveExistsWrapper`
  (returns (Exists :type Boolean))
  (return false))

(fn `GetSaveListWrapper`
  (returns (SaveData :type "Array of /Game/MenuSystem/Structs/FSaveDataWrapper Structure"))
  (locals (SaveDataArray :type "Array of /Game/MenuSystem/Structs/FSaveDataWrapper Structure"))
  (return))

(fn `GetSaveManager`
  (returns (IsValid :type Boolean) (SaveManager :type "/Game/MenuSystem/Blueprints/SaveSystem/BP_save_manager Object Reference"))
  (return false null))

(fn `IsLatestSaveIDWrapper`
  (params (SaveID :type String))
  (returns (ReturnValue :type Boolean))
  (return false))

(fn `LoadFromLastCheckpointWrapper`)

(fn `LoadFromSaveIDWrapper`
  (params (SaveID :type String)))

(fn `RemoveAllSavesWrapper`)

(fn `SaveGameWrapper`
  (`KismetSystemLibrary.PrintString` null "AGS Basic Save Game plugin is not installed! \nFor save system to work please follow the guide on the official docs." true true (struct :`R` 1.0 :`G` 0.229694 :`A` 1.0) 5.0))

(fn `SetSaveIDToLoadWrapper`
  (params (SaveID :type String)))