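; Menu spawner Blueprint that opens the startup media player ahead of the main menu and drives the menu background music.
; On BeginPlay it reads menu settings from the GameInstance through BPI_GI_AMS, creates and focuses the player widget, and applies saved settings.
; A GameInstance flag skips startup videos once played, with a force-skip override.
; Music fades in when the player closes and out on the menu's audio transition event.
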(event `fadeInBGMusic_event`
  ;[0.07221 0.5536 1] Play menu background music. This is only for demo purpose.
  ; Normally you want to do this sort of stuff in
  ; the "GameInstance" so music won't get interrupted when new level loads
  (bind _returnvalue (`GameplayStatics.CreateSound2D` "/Game/MenuSystem/Audio/Cues/A_menu_bg_music_Cue.A_menu_bg_music_Cue" 1.0 1.0 0.0 null))
  (bind _output_get (set `self.MenuBGMusic` _returnvalue))
  (`AudioComponent.FadeIn` _output_get 1.4 1.0 0.0 "Linear"))

(event `fadeOutBGMusic_event`
  ;[0.07221 0.5536 1] Play menu background music. This is only for demo purpose.
  ; Normally you want to do this sort of stuff in
  ; the "GameInstance" so music won't get interrupted when new level loads
  (`AudioComponent.FadeOut` (`self.MenuBGMusic`) 0.9 0.0 "Linear"))

(event `self.ReceiveBeginPlay`
  (bind _returnvalue (`GameplayStatics.GetPlayerController` 0))
  (if (`KismetSystemLibrary.DoesImplementInterface` (`GameplayStatics.GetGameInstance`) "/Game/MenuSystem/Interface/BPI_GI_AMS.BPI_GI_AMS_C")
    (bind _menusettings (message `/Game/MenuSystem/Interface/BPI_GI_AMS.GetMenuSettings` (`GameplayStatics.GetGameInstance`)))
    ;[0 0 0] Show Startup Media before the main menu
    (bind _canplayvideo (message `/Game/MenuSystem/Interface/BPI_GI_AMS.GetCanPlayVideo` (`GameplayStatics.GetGameInstance`)))
    (bind (_bismultiplayer _mainmenutoopen _pausemenutoopen _startupmediaoptions) (break `/Game/MenuSystem/Structs/FMenuSettings` _menusettings))
    (bind (_defaultskiptext _mediaplaylist _onmediaplaybackfinished _mediastretch) (break `/Game/MenuSystem/Structs/FStartupMediaSettings` _startupmediaoptions))
    (bind _returnvalue_2 (`|CreateWidget` "/Game/MenuSystem/Widgets/Common/WBP_StartupMediaPlayer.WBP_StartupMediaPlayer_C" null (select `bool` (`self.SkipVideos?`) :`false` (not _canplayvideo) :`true` true) _mainmenutoopen _defaultskiptext _mediaplaylist _onmediaplaybackfinished _mediastretch))
    (`UserWidget.AddToViewport` _returnvalue_2 0)
    (`Widget.SetKeyboardFocus` _returnvalue_2)
    (`WidgetBlueprintLibrary.SetInputMode_UIOnlyEx` _returnvalue _returnvalue_2)
    (set `PlayerController.bShowMouseCursor` true _returnvalue)
    (add `/Game/MenuSystem/Widgets/Common/WBP_StartupMediaPlayer.OnStartupPlayerClose` _returnvalue_2 (delegate `fadeInBGMusic_event`)) ; Only play main menu music when the startup player \ncloses
    (add `/Game/MenuSystem/Widgets/Common/WBP_Menu_Base.OnMenuAudioTransition` (`/Game/MenuSystem/Widgets/Common/WBP_StartupMediaPlayer.GetMainMenuWidgetRef` _returnvalue_2) (delegate `fadeOutBGMusic_event`)) ; Fadeout menu music when loading a new level \nor quiting the game
    (`/Game/MenuSystem/Blueprints/FunctionLibrary/BPFL_settings_lib.LoadSettingsOnStart`) ; Load and apply all the saved settings(if any) on start
    (message `/Game/MenuSystem/Interface/BPI_GI_AMS.SetCanPlayVideo` (`GameplayStatics.GetGameInstance`) false) ; Disable startup video once it is played already
    (else
      (`KismetSystemLibrary.PrintString` "ERROR: Game instance needs to implement BPI_GI_AMS interface" true true (struct :`R` 1.0 :`G` 0.090343 :`A` 1.0) 7.0))))

(fn `UserConstructionScript`)