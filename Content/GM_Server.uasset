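; GM_Server is a server game mode that appears to be an unfinished prototype for launching match servers once players join.
; Tick fires an event dispatcher every frame while at least two players are present.
; Its handler calls an empty LaunchServer event, and the binding to that handler is disconnected.
; Other disconnected fragments sketch launching the Covid19 map, creating a dedicated Advanced Session and traveling to a hardcoded IP with incremented ports.
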(event `self.ReceiveTick`
  (params (DeltaSeconds :type "Float (single-precision)"))
  (if (>= (`KismetArrayLibrary.Array_Length` (`GameStateBase.PlayerArray` (`GameplayStatics.GetGameState`))) 2)
    (`self.NewEventDispatcher_0`)))

(event `LaunchServer`)

(event `self.ReceiveBeginPlay`)

(event `NewEventDispatcher_0_Event`
  (`self.LaunchServer`))

(fn `UserConstructionScript`)